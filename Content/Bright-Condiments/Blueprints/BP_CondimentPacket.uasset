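; BP_CondimentPacket is an interactable condiment packet the player can carry, throw or jump on to spread sauce.
; While held, Tick positions it relative to the player and tilts it by charge, jittering at full power; release applies a camera-aimed impulse.
; Fully charged throws spawn puddles on impact through BPCPuddleSpawner.
; Hard landings spray a diamond of BP_CondimentSquirt out one end, occasionally both for middle hits, leaving a BP_CondimentOpen.
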(event `/Game/Blueprints/Interact/BPI_Interactable.Interact`
  ; Interact - Pick Up
  (bind _asbp_first_person_character_1 (cast `/Game/FirstPerson/Blueprints/BP_FirstPersonCharacter` (`GameplayStatics.GetPlayerCharacter` 0)))
  (`/Game/FirstPerson/Blueprints/BP_FirstPersonCharacter.PickupCondimentPacket` _asbp_first_person_character_1 self)
  (`CharacterMovementComponent.SetMovementMode` (`Character.CharacterMovement` (`GameplayStatics.GetPlayerCharacter` 0)) "MOVE_Flying" 0))

(event `self.ReceiveBeginPlay`
  ; Event BeginPlay
  (`/Game/Bright-Condiments/Blueprints/BPC_Condiments.SetType` (`self.BPC_Condiments`) (`self.Type`))
  (`PrimitiveComponent.SetMaterial` (`self.Sauce_packet_closed`) 0 (`/Game/Bright-Condiments/Blueprints/BPC_Condiments.Material` (`self.BPC_Condiments`))))

(event `self.ReceiveTick`
  (params (DeltaSeconds :type "Float (single-precision)"))
  (bind (_returnvalue_roll _returnvalue_pitch _returnvalue_yaw) (`KismetMathLibrary.BreakRotator` (`self.K2_GetActorRotation` (`GameplayStatics.GetPlayerCharacter` 0))))
  (bind _returnvalue (* (`self.LaunchStage`) 5.0))
  (bind _returnvalue_2 (+ (* (`self.LaunchPower`) 4.0) 400.0))
  ; Event Tick - Update if Picked Up
  (set `self.LaunchStage` (`KismetMathLibrary.Min` (/ (`self.LaunchPower`) 60) 3))
  (if (not (`self.PickedUp`))
    (if (`self.OldPickedUp`)
      (set `self.OldPickedUp` false)
      (`PrimitiveComponent.SetSimulatePhysics` (`self.Sauce_packet_closed`) true)
      (bind _asbp_first_person_character_1 (cast `/Game/FirstPerson/Blueprints/BP_FirstPersonCharacter` (`GameplayStatics.GetPlayerCharacter` 0)))
      (bind (_returnvalue_roll_2 _returnvalue_pitch_2) (`KismetMathLibrary.BreakRotator` (`SceneComponent.GetSocketRotation` (`/Game/FirstPerson/Blueprints/BP_FirstPersonCharacter.FirstPersonCamera` _asbp_first_person_character_1) "None")))
      (bind _returnvalue_3 (`KismetMathLibrary.FMax` _returnvalue_pitch_2))
      (bind _returnvalue_4 (* (`KismetMathLibrary.DegCos` _returnvalue_3) _returnvalue_2))
      (`PrimitiveComponent.AddImpulse` (`self.Sauce_packet_closed`) (`KismetMathLibrary.MakeVector` (* (`KismetMathLibrary.DegCos` _returnvalue_yaw) _returnvalue_4) (* (`KismetMathLibrary.DegSin` _returnvalue_yaw) _returnvalue_4) (* (`KismetMathLibrary.DegSin` _returnvalue_3) _returnvalue_2)) "None" true))
    (else
      (`SceneComponent.K2_SetWorldLocationAndRotation` (`self.Sauce_packet_closed`) (`KismetMathLibrary.TransformLocation` (`self.GetTransform` (`GameplayStatics.GetPlayerCharacter` 0)) (`KismetMathLibrary.MakeVector` (* (`KismetMathLibrary.DegSin` _returnvalue) -150.0) (select `bool` (== (`self.LaunchStage`) 3) :`true` (`KismetMathLibrary.RandomFloatInRange` -5.0 5.0)) (* (`KismetMathLibrary.DegCos` _returnvalue) 150.0))) (`KismetMathLibrary.MakeRotator` _returnvalue (.pitch (`self.K2_GetActorRotation` (`GameplayStatics.GetPlayerCharacter` 0))) (+ (.yaw (`self.K2_GetActorRotation` (`GameplayStatics.GetPlayerCharacter` 0))) 90.0)) false true)
      (`PrimitiveComponent.SetSimulatePhysics` (`self.Sauce_packet_closed`) false)
      (if (not (`self.OldPickedUp`))
        (set `self.OldPickedUp` true)
        (`CharacterMovementComponent.SetMovementMode` (`Character.CharacterMovement` (`GameplayStatics.GetPlayerCharacter` 0)) "MOVE_Falling" 0)))))

(event `self.Sauce_packet_closed.OnComponentHit`
  (params (HitComponent :type "PrimitiveComponent Object Reference") (OtherActor :type "Actor Object Reference") (OtherComp :type "PrimitiveComponent Object Reference") (NormalImpulse :type "Vector Structure") (Hit :type "HitResult Structure (by ref)"))
  ; On HitGround after thrown
  (if (and (== (`self.LaunchStage`) 3) (not (`GameplayStatics.ObjectIsA` OtherActor "/Game/FirstPerson/Blueprints/BP_FirstPersonCharacter.BP_FirstPersonCharacter_C")))
    (`/Game/Bright-Condiments/BPComponents/BPC_PuddleSpawner.Spawn Puddles` (`self.BPC_PuddleSpawner`) (`self.Splatter Life Span`) 2.0 (`self.Splatter Size`) (`.ImpactPoint` (`GameplayStatics.BreakHitResult` Hit)) (`self.Type`))
    (`self.K2_DestroyActor`)))

(event `self.ReceiveHit`
  (params (MyComp :type "PrimitiveComponent Object Reference") (Other :type "Actor Object Reference") (OtherComp :type "PrimitiveComponent Object Reference") (bSelfMoved :type Boolean) (HitLocation :type "Vector Structure") (HitNormal :type "Vector Structure") (NormalImpulse :type "Vector Structure") (Hit :type "HitResult Structure (by ref)"))
  ; Event Hit (by player)
  (`self.SpawnCondiment` (`/Game/Bright-Condiments/Blueprints/BPC_Condiments.Material` (`self.BPC_Condiments`)) Other))

(fn `GetPrompt`
  (returns (Prompt :type String))
  (return (`KismetStringLibrary.Concat_StrStr` "Pick Up " (`|GetEnumeratorNameAsString` (`self.Type`)) " Packet")))

(fn `IsInteractable`
  (returns (IsInteractable :type Boolean))
  (return (not (`self.PickedUp`))))

(fn `SpawnCondiment`
  (params (Material :type "MaterialInstance Object Reference") (HitOther :type "Actor Object Reference"))
  (locals (Condiment :type "/Game/Bright-Condiments/Blueprints/E_Condiments Enum") (CMaterial :type "MaterialInstance Object Reference"))
  (bind (_returnvalue_x _returnvalue_y _returnvalue_z) (`KismetMathLibrary.BreakVector` (`self.K2_GetActorLocation`)))
  (bind _splatter_size (`self.Splatter Size`))
  (bind (_returnvalue_location _returnvalue_rotation _returnvalue_scale) (`KismetMathLibrary.BreakTransform` (`SceneComponent.K2_GetComponentToWorld` (`self.Sauce_packet_closed`))))
  (bind _returnvalue (+ (`self.SizeY * 2`) 200.0))
  (set `local.CMaterial` Material)
  (set `self.HitOther` HitOther)
  (if (and (`GameplayStatics.ObjectIsA` HitOther "/Game/FirstPerson/Blueprints/BP_FirstPersonCharacter.BP_FirstPersonCharacter_C") (not (`self.PickedUp`)))
    ; Check If Enough Jump Force Was Applied
    (bind _asbp_first_person_character_1 (cast `/Game/FirstPerson/Blueprints/BP_FirstPersonCharacter` HitOther))
    (bind (_returnvalue_x_2 _returnvalue_y_2 _returnvalue_z_2) (`KismetMathLibrary.BreakVector` (`self.K2_GetActorLocation` _asbp_first_person_character_1)))
    (if (and (> (`/Game/Bright-Condiments/BPComponents/BPC_PlayerCondiments.JumpTime` (`/Game/FirstPerson/Blueprints/BP_FirstPersonCharacter.BPC_PlayerCondiments` _asbp_first_person_character_1)) 0.5) (> _returnvalue_z_2 _returnvalue_z))
      (set `self.SizeY * 2` (* (.y (`.BoxExtent` (`self.GetActorBounds` false))) 2.0))
      (set `self.OverlappingSouth` (`PrimitiveComponent.IsOverlappingActor` (`self.SouthHit`) (`self.HitOther`)))
      (for _index (range (- 0 _splatter_size) (+ _splatter_size 1)) :!label _label
        (bind _returnvalue_2 (- (`self.Splatter Size`) (`KismetMathLibrary.Abs_Int` _index)))
        ; Spawn Multiple Puddles of Condiment
        (for _index_2 (range (- 0 _returnvalue_2) (+ _returnvalue_2 1))
          (if (`self.OverlappingSouth`)
            (bind _returnvalue_3 (`self.OffsetKetchup` _index))
            (set `self.Location Y` (+ _returnvalue_3 _returnvalue))
            (else
              (set `self.Location Y` (- _returnvalue_3 _returnvalue))))
          (`|SpawnActorFromClass` "/Game/Bright-Condiments/Blueprints/BP_CondimentSquirt.BP_CondimentSquirt_C" (`KismetMathLibrary.MakeTransform` (`KismetMathLibrary.TransformLocation` (`SceneComponent.K2_GetComponentToWorld` (`self.Sauce_packet_closed`)) (`KismetMathLibrary.MakeVector` (`self.OffsetKetchup` _index_2) (`self.Location Y`)))) "Undefined" "MultiplyWithRoot" null (`self.Type`) (`self.Splatter Life Span`) 2.0 (- (`self.Splatter Size`) (+ (`KismetMathLibrary.Abs_Int` _index_2) (`KismetMathLibrary.Abs_Int` _index))) null)))
      (if (and (`PrimitiveComponent.IsOverlappingActor` (`self.MiddleHit`) (`self.HitOther`)) (not (`self.Doubled`)))
        (if (== (`KismetMathLibrary.RandomInteger` 3) 0)
          (set `self.Doubled` true)
          (set `self.OverlappingSouth` (not (`self.OverlappingSouth`)))
          (goto _label)
          (else
            (`KismetSystemLibrary.PrintString` "Hit Fail"))))
      (`|SpawnActorFromClass` "/Game/Bright-Condiments/Blueprints/BP_CondimentOpen.BP_CondimentOpen_C" (`KismetMathLibrary.MakeTransform` (+ _returnvalue_location (0.0 0.0 5.0)) _returnvalue_rotation _returnvalue_scale) "Undefined" "MultiplyWithRoot" null (`self.OverlappingSouth`) (`local.CMaterial`) 300 null)
      (`self.K2_DestroyActor`))))

(fn `UserConstructionScript`)