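; BP_CondimentOpen is a short-lived opened condiment packet that shows either a north-opened or south-opened mesh.
; BeginPlay uses the South flag to hide the unused mesh and applies Material to both, with SetDirection and SetMaterial repeating those steps as functions.
; Tick counts frames and destroys the actor once the count exceeds LifeSpan.
; An unconnected spin-and-shrink chain never runs.
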(event `self.ReceiveBeginPlay`
  (bind _material (`self.Material`))
  (if (`self.South`)
    (`SceneComponent.SetVisibility` (`self.Packet_openNorth`) false false)
    (else
      (`SceneComponent.SetVisibility` (`self.Packet_openSouth`) false false)))
  (`PrimitiveComponent.SetMaterial` (`self.Packet_openNorth`) 0 _material)
  (`PrimitiveComponent.SetMaterial` (`self.Packet_openSouth`) 0 _material))

(event `self.ReceiveTick`
  (params (DeltaSeconds :type "Float (single-precision)"))
  (bind _timer (`self.Timer`))
  (`/Engine/EditorBlueprintResources/StandardMacros.IncrementInt` _timer
    (:`  `
      (if (> _timer (`self.LifeSpan`))
        (`self.K2_DestroyActor`)))))

(fn `SetDirection`
  (params (South :type Boolean))
  (if South
    (`SceneComponent.SetVisibility` (`self.Packet_openNorth`) false false)
    (else
      (`SceneComponent.SetVisibility` (`self.Packet_openSouth`) false false))))

(fn `SetMaterial`
  (params (Material :type "MaterialInstance Object Reference"))
  (`PrimitiveComponent.SetMaterial` (`self.Packet_openNorth`) 0 Material)
  (`PrimitiveComponent.SetMaterial` (`self.Packet_openSouth`) 0 Material))

(fn `UserConstructionScript`)