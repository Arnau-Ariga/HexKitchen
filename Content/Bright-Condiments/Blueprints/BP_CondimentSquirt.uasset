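; Condiment puddle actor that takes its material from its condiment type, grows, then shrinks away.
; On BeginPlay a downward trace snaps it to the surface normal, ignoring same-type squirts, open condiments and packets.
; Tick scales the cylinder up to puddle size, then shrinks it and destroys the actor after its lifespan.
; Lifespan counts frames, converted at 60 per unit and staggered by circle index; negative values never expire.
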(event `self.ReceiveBeginPlay`
  (`/Game/Bright-Condiments/Blueprints/BPC_Condiments.SetType` (`self.BPC_Condiments`) (`self.Type`))
  (`PrimitiveComponent.SetMaterial` (`self.Cylinder1`) 0 (select `/Game/Bright-Condiments/Blueprints/E_Condiments` (`self.Type`) :`NewEnumerator0` "/Game/Bright-Condiments/Materials/MI_KetchupColorway.MI_KetchupColorway" :`NewEnumerator1` "/Game/Bright-Condiments/Materials/MI_HotSauceColorway.MI_HotSauceColorway" :`NewEnumerator2` "/Game/Bright-Condiments/Materials/MI_LemonColorway.MI_LemonColorway" :`NewEnumerator3` "/Game/Bright-Condiments/Materials/MI_MayoColorway.MI_MayoColorway" :`NewEnumerator4` "/Game/Bright-Condiments/Materials/MI_MustardColorway.MI_MustardColorway" :!type "MaterialInterface Object Reference"))
  (`self.Ray Trace`))

(event `self.ReceiveTick`
  (params (DeltaSeconds :type "Float (single-precision)"))
  (bind _lifespan (`self.LifeSpan`))
  (bind _cylinder1 (`self.Cylinder1`))
  (bind _cylinder1_2 (`self.Cylinder1`))
  (bind _cylinder1_3 (`self.Cylinder1`))
  (bind (_returnvalue_x _returnvalue_y _returnvalue_z) (`KismetMathLibrary.BreakVector` (`SceneComponent.K2_GetComponentScale` _cylinder1_2)))
  (bind (_returnvalue_x_2 _returnvalue_y_2 _returnvalue_z_2) (`KismetMathLibrary.BreakVector` (`SceneComponent.K2_GetComponentScale` _cylinder1_3)))
  (bind (_returnvalue_x_3 _returnvalue_y_3 _returnvalue_z_3) (`KismetMathLibrary.BreakVector` (`SceneComponent.K2_GetComponentScale` _cylinder1)))
  (bind _returnvalue (* _returnvalue_x_3 1.05))
  (bind _returnvalue_2 (- _returnvalue_x 0.02))
  (bind _returnvalue_3 (- _returnvalue_x_2 0.005))
  (bind _result (`/Engine/EditorBlueprintResources/StandardMacros.IncrementFloat` (`self.Timer`))
    (:`  `
      (if (or (< _result _lifespan) (< _lifespan 0.0))
        (if (< _returnvalue_x_3 (`self.PuddleSize`))
          (`SceneComponent.SetWorldScale3D` _cylinder1 (`KismetMathLibrary.MakeVector` _returnvalue _returnvalue _returnvalue_z_3)))
        (elif (>= _returnvalue_x_2 0.5)
          (`SceneComponent.SetWorldScale3D` _cylinder1_3 (`KismetMathLibrary.MakeVector` _returnvalue_3 _returnvalue_3 _returnvalue_z_2))
          (elif (>= _returnvalue_x 0.0)
            (`SceneComponent.SetWorldScale3D` _cylinder1_2 (`KismetMathLibrary.MakeVector` _returnvalue_2 _returnvalue_2 _returnvalue_z))
            (else
              (`self.K2_DestroyActor`))))))))

(fn `Ray Trace`
  (bind _returnvalue (`self.K2_GetActorLocation`))
  (bind _lifespan (`self.LifeSpan`))
  (bind _returnvalue_2 (+ _returnvalue (0.0 0.0 100.0)))
  (`self.AddToActorToIgnore` "BP_CondimentSquirt_C"
    (:`Out`
      (`self.AddToActorToIgnore` "/Game/Bright-Condiments/Blueprints/BP_CondimentOpen.BP_CondimentOpen_C"
        (:`Out`
          (`self.AddToActorToIgnore` "/Game/Bright-Condiments/Blueprints/BP_CondimentPacket.BP_CondimentPacket_C"
            (:`Out`
              (bind _outhit (`KismetSystemLibrary.LineTraceSingle` _returnvalue_2 (- _returnvalue (0.0 0.0 500.0)) "TraceTypeQuery1" false (`self.ActorsToIgnore`)))
              (bind (_bblockinghit _binitialoverlap _time _distance _location _impactpoint _normal _impactnormal) (`GameplayStatics.BreakHitResult` _outhit))
              (if (!= _location _returnvalue_2)
                (`self.K2_SetActorLocationAndRotation` _location (`KismetMathLibrary.MakeRotFromZ` _impactnormal))
                (if (>= _lifespan 0.0)
                  (set `self.LifeSpan` (+ (* _lifespan 60.0) (`KismetMathLibrary.Abs_Int` (* (`self.CircleIDX`) 150)))))))))))))

(fn `UserConstructionScript`)