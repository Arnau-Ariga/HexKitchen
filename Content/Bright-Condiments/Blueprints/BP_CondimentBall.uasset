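; BP_CondimentBall is a condiment projectile that either affects the player it hits or splatters into a puddle.
; Hitting BP_FirstPersonCharacter calls ApplyEffect, which is empty here, and destroys the ball.
; Other hits spawn a roughly diamond-shaped, randomly jittered grid of the Condiment class at the impact's XY and ball's height, then destroy it.
; Each piece receives an index that decreases with grid distance from the center.
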(event `self.ReceiveHit`
  (params (MyComp :type "PrimitiveComponent Object Reference") (Other :type "Actor Object Reference") (OtherComp :type "PrimitiveComponent Object Reference") (bSelfMoved :type Boolean) (HitLocation :type "Vector Structure") (HitNormal :type "Vector Structure") (NormalImpulse :type "Vector Structure") (Hit :type "HitResult Structure (by ref)"))
  (bind _puddlesplat (`self.PuddleSplat`))
  (if (`GameplayStatics.ObjectIsA` Other "/Game/FirstPerson/Blueprints/BP_FirstPersonCharacter.BP_FirstPersonCharacter_C")
    (`self.ApplyEffect` Other)
    (`self.K2_DestroyActor`)
    (else
      (for _index (range (- 0 _puddlesplat) (+ _puddlesplat 1))
        (bind _returnvalue (- (`self.PuddleSplat`) (`KismetMathLibrary.Abs_Int` _index)))
        (for _index_2 (range (- 0 _returnvalue) (+ _returnvalue 1))
          (`|SpawnActorFromClass` (`self.Condiment`) (`KismetMathLibrary.MakeTransform` (`KismetMathLibrary.TransformLocation` (`KismetMathLibrary.MakeTransform` (`KismetMathLibrary.MakeVector` HitLocation_X HitLocation_Y (.z (.location (`self.GetTransform`))))) (`KismetMathLibrary.MakeVector` (`self.OffsetKetchup` _index_2) (`self.OffsetKetchup` _index)))) "Undefined" "MultiplyWithRoot" null -1.0 2.0 (- _puddlesplat (+ (`KismetMathLibrary.Abs_Int` _index_2) (`KismetMathLibrary.Abs_Int` _index))) null)))
      (`self.K2_DestroyActor`))))

(fn `ApplyEffect`
  (params (Player :type "Actor Object Reference")))

(fn `SetCondiment`
  (params (Condiment :type "/Game/Bright-Condiments/Blueprints/BP_CondimentSquirt Class Reference"))
  (set `self.Condiment` Condiment))

(fn `UserConstructionScript`)