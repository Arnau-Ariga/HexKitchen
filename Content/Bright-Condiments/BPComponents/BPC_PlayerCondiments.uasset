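; Player component that handles carrying and throwing condiment packets, plus the lemon blind and ketchup slow effects on the player.
; Holding left mouse charges the held sauce's launch power, and releasing throws it with that power capped.
; Carrying, charging and the slow effect feed speed overrides into the character's BPCOverrideMvtSpeed.
; Per-tick counters drive slow recovery, fade the lemon and ketchup screen widgets, and track airborne time.
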(event `self.ReceiveBeginPlay`
  (bind _returnvalue (`GameplayStatics.GetPlayerCharacter` 0))
  (bind _returnvalue_2 (`|CreateWidget` "/Game/Bright-Condiments/UI/W_Lemon.W_Lemon_C"))
  (bind _output_get (set `self.WLemon` _returnvalue_2))
  (`UserWidget.AddToViewport` _output_get 0)
  (`Widget.SetRenderOpacity` _output_get 0.0)
  (bind _returnvalue_3 (`|CreateWidget` "/Game/Bright-Condiments/UI/W_KetchupBall.W_KetchupBall_C"))
  (bind _output_get_2 (set `self.WKetchupBall` _returnvalue_3))
  (`Widget.SetRenderOpacity` _output_get_2 0.0)
  (`UserWidget.AddToViewport` _output_get_2 0)
  (set `self.CharacterMovement` (`Character.CharacterMovement` _returnvalue))
  (bind _asbp_first_person_character (cast `/Game/FirstPerson/Blueprints/BP_FirstPersonCharacter` _returnvalue))
  (set `self.BPC_OverrideMvtSpeed` (`/Game/FirstPerson/Blueprints/BP_FirstPersonCharacter.BPC_OverrideMvtSpeed` _asbp_first_person_character)))

(event `self.ReceiveTick`
  (params (DeltaSeconds :type "Float (single-precision)"))
  (bind _effectblindtime (`self.EffectBlindTime`))
  (bind _wlemon (`self.WLemon`))
  (bind (_returnvalue_x _returnvalue_y _returnvalue_z) (`KismetMathLibrary.BreakVector` (`CharacterMovementComponent.GetLastUpdateVelocity` (`self.CharacterMovement`))))
  (bind _renderopacity (`Widget.RenderOpacity` (`self.WLemon`)))
  (bind _output_get (set `self.IsOnGround` (== _returnvalue_z 0.0)))
  (if _output_get
    (set `self.JumpTime` 0.0)
    (else
      (set `self.JumpTime` (+ (`self.JumpTime`) 0.01))))
  (`/Engine/EditorBlueprintResources/StandardMacros.IncrementFloat` _effectblindtime
    (:`  `
      (if (and (<= _effectblindtime 180.0) (>= _effectblindtime 30.0))
        (`Widget.SetRenderOpacity` _wlemon (- _renderopacity 0.001))
        (if (`KismetSystemLibrary.IsValid` (`self.Holding Sauce`)) :!label _label
          (`/Game/Bright-Condiments/BPComponents/BPC_OverrideMvtSpeed.AddOverride` (`self.BPC_OverrideMvtSpeed`) (select `bool` (`self.MouseDown`) :`false` 400 :`true` 100)))
        (`self.SlownessEffect`)
        (if (`self.MouseDown`)
          (bind _result (`/Engine/EditorBlueprintResources/StandardMacros.IncrementInt` (`self.MouseDownTime`))
            (:`  `
              (set `/Game/Bright-Condiments/Blueprints/BP_CondimentPacket.LaunchPower` _result (`self.Holding Sauce`)))))
        (elif (>= (`self.EffectBlindTime`) 240.0)
          (`Widget.SetRenderOpacity` _wlemon (- _renderopacity 0.005))
          (goto _label))))))

(event `Key|LeftMouseButton` :consume false :overrideparent false
  (params (Key :type "Key Structure"))
  ; Throwing Condiment Packet
  (:`Pressed`
    (if (`KismetSystemLibrary.IsValid` (`self.Holding Sauce`))
      (set `self.MouseDown` true)))
  (:`Released`
    (`self.ThrowPacket`)))

(fn `SlownessEffect`
  (bind _effectslowspeed (`self.EffectSlowSpeed`))
  (if (<= (`self.EffectSlowSpeed`) 600)
    (bind _result (`/Engine/EditorBlueprintResources/StandardMacros.IncrementInt` _effectslowspeed)
      (:`  `
        (`/Game/Bright-Condiments/BPComponents/BPC_OverrideMvtSpeed.AddOverride` (`self.BPC_OverrideMvtSpeed`) _result)
        (set `Widget.RenderOpacity` (- 1.0 (/ (`KismetMathLibrary.Conv_IntToDouble` _effectslowspeed) 600.0)) (`self.WKetchupBall`))))
    (else
      (set `Widget.RenderOpacity` 0.0 (`self.WKetchupBall`)))))