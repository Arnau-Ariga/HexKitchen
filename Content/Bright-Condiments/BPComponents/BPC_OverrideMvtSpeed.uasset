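; Actor component that arbitrates a Character's max walk speed from override requests and a stun flag.
; BeginPlay caches the movement component and default speed; AddOverride queues target speeds, which Tick resolves and clears, so overrides must be resubmitted continuously.
; Same-direction overrides apply the one furthest from default, while mixed ones average their extremes.
; Stunned forces zero speed; an empty queue restores the default.
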(event `self.ReceiveBeginPlay`
  (bind _ascharacter (cast `Character` (`self.GetOwner`)))
  (bind _output_get (set `self.Character Movement` (`Character.CharacterMovement` _ascharacter)))
  (bind _output_get_2 (set `self.DefaultSpeed` (`KismetMathLibrary.FTrunc` (`CharacterMovementComponent.MaxWalkSpeed` _output_get))))
  (set `self.WalkSpeed` _output_get_2))

(event `self.ReceiveTick`
  (params (DeltaSeconds :type "Float (single-precision)"))
  (bind _defaultspeed (`self.DefaultSpeed`))
  (bind _overridewalkspeed (`self.OverrideWalkSpeed`))
  (bind _minvalue (`self.MinValue`))
  (bind _maxvalue (`self.MaxValue`))
  (bind _character_movement (`self.Character Movement`))
  (if (`self.Stunned`)
    (set `CharacterMovementComponent.MaxWalkSpeed` 0.0 (`self.Character Movement`))
    (elif (`KismetArrayLibrary.Array_IsEmpty` (`self.OverrideWalkSpeed`))
      (set `CharacterMovementComponent.MaxWalkSpeed` (`KismetMathLibrary.Conv_IntToDouble` (`self.DefaultSpeed`)) (`self.Character Movement`))
      (else
        (set `self.MinValue` (- (`.MinValue` (`KismetMathLibrary.MinOfIntArray` _overridewalkspeed)) _defaultspeed))
        (set `self.MaxValue` (- (`.MaxValue` (`KismetMathLibrary.MaxOfIntArray` _overridewalkspeed)) _defaultspeed))
        (`KismetArrayLibrary.Array_Clear` (`self.OverrideWalkSpeed`))
        (if (!= (`KismetMathLibrary.SignOfInteger` _minvalue) (`KismetMathLibrary.SignOfInteger` _maxvalue))
          (set `CharacterMovementComponent.MaxWalkSpeed` (`KismetMathLibrary.Conv_IntToDouble` (+ (/ (+ _minvalue _maxvalue) 2) (`self.DefaultSpeed`))) (`self.Character Movement`))
          (elif (<= (`self.MaxValue`) 0)
            (set `CharacterMovementComponent.MaxWalkSpeed` (`KismetMathLibrary.Conv_IntToDouble` (+ (`self.MinValue`) (`self.DefaultSpeed`))) _character_movement)
            (else
              (set `CharacterMovementComponent.MaxWalkSpeed` (`KismetMathLibrary.Conv_IntToDouble` (+ (`self.MaxValue`) (`self.DefaultSpeed`))) _character_movement))))))))

(fn `AddOverride`
  (params (Override :type Integer))
  (`KismetArrayLibrary.Array_Add` (`self.OverrideWalkSpeed`) Override))