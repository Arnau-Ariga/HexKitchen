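; Character component that applies ketchup, hot sauce and mayo effects while the owning player or enemy overlaps those condiment actors.
; Each tick, a shared macro compares overlap with the previous state to fire start, continue and end branches.
; Ketchup slows walking and jumping, hot sauce deals periodic damage with brief stops (sparing grilled cheese), and mayo makes movement slippery.
; Speed and damage route through override-speed and health components; players also get screen widgets.
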(event `self.ReceiveBeginPlay`
  (bind _ascharacter (cast `Character` (`self.GetOwner`)))
  (bind _output_get (set `self.Character` _ascharacter))
  (set `self.CharacterMovement` (`Character.CharacterMovement` _output_get))
  (bind _asbp_first_person_character (cast `/Game/FirstPerson/Blueprints/BP_FirstPersonCharacter` _output_get)
    (:`then`
      (bind _output_get_2 (set `self.Player` _asbp_first_person_character))
      (set `self.BPC OverrideMvt` (`/Game/FirstPerson/Blueprints/BP_FirstPersonCharacter.BPC_OverrideMvtSpeed` _output_get_2))
      (set `self.BPC Health` (`/Game/FirstPerson/Blueprints/BP_FirstPersonCharacter.BPC_Health` _output_get_2))
      (set `self.isPlayer` true)
      (bind _returnvalue (`|CreateWidget` "/Game/Bright-Condiments/UI/W_Ketchup.W_Ketchup_C"))
      (bind _output_get_3 (set `self.WKetchup` _returnvalue))
      (`UserWidget.AddToViewport` _output_get_3 0))
    (:`CastFailed`
      (bind _asbp_enemy_base (cast `/Game/Enemies/AI_bases/BP_enemy_base` _output_get))
      (set `self.BPC OverrideMvt` (`/Game/Enemies/AI_bases/BP_enemy_base.BPC_OverrideMvtSpeed` _asbp_enemy_base))
      (set `self.BPC Health` (`/Game/Enemies/AI_bases/BP_enemy_base.BPC_Health` _asbp_enemy_base)))))

(event `self.ReceiveTick`
  (params (DeltaSeconds :type "Float (single-precision)"))
  (set `self.CurrWasOverlapping` (`self.WasKetchup`))
  (`self.Ketchup Effect`)
  (set `self.WasKetchup` (`self.CurrWasOverlapping`))
  (set `self.CurrWasOverlapping` (`self.WasHotSauce`))
  (`self.Hot Sauce Effect`)
  (set `self.WasHotSauce` (`self.CurrWasOverlapping`))
  (set `self.CurrWasOverlapping` (`self.WasMayo`))
  (`self.Mayo Effect`)
  (set `self.WasMayo` (`self.CurrWasOverlapping`)))

(fn `CheckOverlap`
  (params (`Actor Class` :type "Actor Class Reference"))
  (returns (Intersects :type Boolean))
  (bind _outactors (`GameplayStatics.GetAllActorsOfClass` `Actor Class`))
  (for _array_element _outactors
    (if (`Actor.IsOverlappingActor` (`self.GetOwner`) _array_element)
      (return true)))
  (return false))

(fn `Hot Sauce Effect`
  (bind _ignorearray (`self.IgnoreArray`))
  (`KismetArrayLibrary.Array_Add` _ignorearray "/Game/Enemies/BP_grilledCheese.BP_grilledCheese_C")
  (for _array_element _ignorearray
    (if (`GameplayStatics.ObjectIsA` (`self.GetOwner`) _array_element)
      (return)))
  (`self.EffectUpdated` "/Game/Bright-Condiments/Blueprints/BP_CHotSauce.BP_CHotSauce_C"
    (:`Continue inEffect`
      (bind _result (`/Engine/EditorBlueprintResources/StandardMacros.DecrementInt` (`self.HotSauceCooldown`))
        (:`  `
          (if (<= _result 0)
            (`/Game/Blueprints/BPC_Health.TakeDamage` (`self.BPC Health`) null 5.0 null null null)
            (set `self.HotSauceCooldown` 60)
            (`/Game/Bright-Condiments/BPComponents/BPC_OverrideMvtSpeed.AddOverride` (`self.BPC OverrideMvt`) 0)
            (if (`self.isPlayer`)
              (bind _returnvalue (`|CreateWidget` "/Game/Bright-Condiments/UI/W_HotSauce.W_HotSauce_C"))
              (`UserWidget.AddToViewport` _returnvalue 0))
            (elif (>= (`self.HotSauceCooldown`) 40)
              (`/Game/Bright-Condiments/BPComponents/BPC_OverrideMvtSpeed.AddOverride` (`self.BPC OverrideMvt`) 0))))))
    (:`StartEffect`
      (set `self.HotSauceCooldown` 0))))

(fn `Ketchup Effect`
  (bind _charactermovement (`self.CharacterMovement`))
  (bind _ketchupoverride (`self.KetchupOverride`))
  (bind _bpc_overridemvt (`self.BPC OverrideMvt`))
  (bind _defaultwalkspeed (`/Game/Bright-Condiments/BPComponents/BPC_OverrideMvtSpeed.DefaultWalkSpeed` (`self.BPC OverrideMvt`)))
  (`self.EffectUpdated` "/Game/Bright-Condiments/Blueprints/BP_CKetchup.BP_CKetchup_C"
    (:`Continue inEffect`
      (bind _output_get (set `self.KetchupOverride` (/ _defaultwalkspeed 2)))
      (`/Game/Bright-Condiments/BPComponents/BPC_OverrideMvtSpeed.AddOverride` _bpc_overridemvt _output_get))
    (:`Continue OutEffect`
      (if (< _ketchupoverride _defaultwalkspeed)
        (bind _result (`/Engine/EditorBlueprintResources/StandardMacros.IncrementInt` _ketchupoverride)
          (:`  `
            (`/Game/Bright-Condiments/BPComponents/BPC_OverrideMvtSpeed.AddOverride` _bpc_overridemvt _result)
            (if (`self.isPlayer`)
              (`Widget.SetRenderOpacity` (`self.WKetchup`) (- 1.0 (/ (`KismetMathLibrary.Conv_IntToDouble` (`self.KetchupOverride`)) (`/Game/Bright-Condiments/BPComponents/BPC_OverrideMvtSpeed.DefaultWalkSpeed` (`self.BPC OverrideMvt`)))))
              (set `/Game/Bright-Condiments/UI/W_Ketchup.FadeIn` false (`self.WKetchup`)))))))
    (:`StartEffect`
      (set `CharacterMovementComponent.JumpZVelocity` 200.0 _charactermovement)
      (if (`self.isPlayer`)
        (set `/Game/Bright-Condiments/UI/W_Ketchup.FadeIn` true (`self.WKetchup`))))
    (:`EndEffect`
      (set `CharacterMovementComponent.JumpZVelocity` 420.0 _charactermovement))))

(fn `Mayo Effect`
  (bind _charactermovement (`Character.CharacterMovement` (`self.Character`)))
  (`self.EffectUpdated` "/Game/Bright-Condiments/Blueprints/BP_CMayo.BP_CMayo_C"
    (:`StartEffect`
      (set `CharacterMovementComponent.GroundFriction` 0.5 _charactermovement)
      (set `CharacterMovementComponent.BrakingDecelerationWalking` 0.0 _charactermovement)
      (set `CharacterMovementComponent.MaxAcceleration` 1000.0 _charactermovement))
    (:`EndEffect`
      (set `CharacterMovementComponent.GroundFriction` 8.0 _charactermovement)
      (set `CharacterMovementComponent.BrakingDecelerationWalking` 2048.0 _charactermovement)
      (set `CharacterMovementComponent.MaxAcceleration` 2048.0 _charactermovement))))