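; BPC_PuddleSpawner is a component that spawns a splatter of condiment puddle actors around a center point.
; SpawnPuddles runs nested grid loops, with Form a Circle_2 bounding each row to approximate a circle by a diamond sized by SplatterSize.
; OffsetKetchup converts grid indices into randomly jittered offsets.
; Each puddle receives lifespan, size and a CircleIDX that falls from the center outward by Manhattan distance.
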(fn `Spawn Puddles`
  (params (`Life Span` :type "Float (double-precision)") (`Puddle Size` :type "Float (double-precision)") (Condiment :type "/Game/Bright-Condiments/Blueprints/BP_CondimentSquirt Class Reference") (`Splatter Size` :type Integer) (Center :type "Vector Structure"))
  (locals (LifeSpan :type "Float (double-precision)") (PuddleSize :type "Float (double-precision)"))
  (set `local.LifeSpan` `Life Span`)
  (set `local.PuddleSize` `Puddle Size`)
  (for _index (range (- 0 `Splatter Size`) (+ `Splatter Size` 1))
    (bind _returnvalue (- `Splatter Size` (`KismetMathLibrary.Abs_Int` _index)))
    (for _index_2 (range (- 0 _returnvalue) (+ _returnvalue 1))
      (`|SpawnActorFromClass` Condiment (`KismetMathLibrary.MakeTransform` (`KismetMathLibrary.TransformLocation` (`KismetMathLibrary.MakeTransform` Center) (`KismetMathLibrary.MakeVector` (`self.OffsetKetchup` _index_2) (`self.OffsetKetchup` _index)))) "Undefined" "MultiplyWithRoot" null (`local.LifeSpan`) (`local.PuddleSize`) (- `Splatter Size` (+ (`KismetMathLibrary.Abs_Int` _index_2) (`KismetMathLibrary.Abs_Int` _index))) null))))