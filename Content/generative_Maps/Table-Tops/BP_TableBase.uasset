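; Table base Blueprint for generative maps that dresses a table top with a random small decorator mesh on BeginPlay.
; It expands each SmallDecorators entry's weight into an index map, then rolls a random integer to make a weighted pick.
; The mesh attaches to the Cube's "Small" socket, with an optional random yaw and an offset by its own negated "Small" socket location.
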(event `self.ReceiveBeginPlay`
  (bind _small_decorator (`self.Small Decorator`))
  (bind _smalldecoratortotal (`self.SmallDecoratorTotal`))
  (bind _output_mesh (break `/Game/generative_Maps/Table-Tops/Decorator` (`|GetArrayItem` (`self.SmallDecorators`) (`self.SmallDecoratorIndex`))))
  (`|ExecutionSequence`
    (:`then_0`
      ; Random Small Decorator Calculation
      (for (_array_element _array_index) (`self.SmallDecorators`)
        (for _index (range _smalldecoratortotal (+ _smalldecoratortotal (`.Weight_5_73C8B2134BF239BB02BB91A4CCA16CD4` (break `/Game/generative_Maps/Table-Tops/Decorator` _array_element))))
          (`BlueprintMapLibrary.Map_Add` (`self.SmallDecoratorMap`) _index _array_index))
        (set `self.SmallDecoratorTotal` (+ (`.Weight_5_73C8B2134BF239BB02BB91A4CCA16CD4` (break `/Game/generative_Maps/Table-Tops/Decorator` _array_element)) (`self.SmallDecoratorTotal`))))
      (set `self.SmallDecoratorIndex` (`BlueprintMapLibrary.Map_Find` (`self.SmallDecoratorMap`) (`KismetMathLibrary.RandomInteger` (`self.SmallDecoratorTotal`))))
      (`StaticMeshComponent.SetStaticMesh` (`self.Small Decorator`) _output_mesh)
      (`SceneComponent.K2_AttachToComponent` (`self.Small Decorator`) (`self.Cube`) "Small" "KeepRelative" "KeepRelative" "KeepRelative" true)
      (if (`.RandomRotation_7_5AC7C2784788BD87B8B9159F2AC6201B` (break `/Game/generative_Maps/Table-Tops/Decorator` _array_element))
        (bind (_x _y) (`KismetMathLibrary.BreakVector2D` (`.RotationAmount_12_6BFB1002497401AB464256B6638FA0DC` (break `/Game/generative_Maps/Table-Tops/Decorator` _array_element))))
        (`SceneComponent.K2_SetRelativeLocationAndRotation` _small_decorator (`KismetMathLibrary.NegateVector` (`SceneComponent.GetSocketLocation` _small_decorator "Small")) (`KismetMathLibrary.MakeRotator` 0.0 0.0 (`KismetMathLibrary.RandomFloatInRange` _x _y)) false false)))
    (:`then_1`)
    (:`then_2`)))

(fn `UserConstructionScript`)