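; Parent room Blueprint for grid-based map generation that opens paths between neighbouring rooms.
; BeginPlay records XY coordinates; CreatePaths runs once, matching RoomConnections by grid offset to map eight neighbours.
; Qualifying orthogonal neighbours hide walls and disable their collision, updating wall count; certain room levels also hide open pieces and increment table count.
; For one rotation type, update events cast self to BP_Table or BP_Island to rotate tables or generate interior walls.
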(event `Update Walls`
  (if (`|EnumEquality` (`self.RotationType`) "NewEnumerator2")
    (bind _asbp_table (cast `/Game/generative_Maps/Room-Generation/TableRooms/BP_Table` self))
    (bind _asbp_island (cast `/Game/generative_Maps/Room-Generation/TableRooms/BP_Island` _asbp_table))
    (`/Game/generative_Maps/Room-Generation/TableRooms/BP_Island.GenerateInteriorWall` _asbp_island)))

(event `Update Tables`
  (if (`|EnumEquality` (`self.RotationType`) "NewEnumerator2")
    (`TextRenderComponent.K2_SetText` (`self.Debug Walls`) (`KismetTextLibrary.Conv_StringToText` (`KismetStringLibrary.BuildString_Int` "walls: " "" (`self.Walls`))))
    (`TextRenderComponent.K2_SetText` (`self.Debug Tables`) (`KismetTextLibrary.Conv_StringToText` (`KismetStringLibrary.BuildString_Int` "tables:" "" (`self.Tables`))))
    (if (`|EnumEquality` (`self.RotationType`) "NewEnumerator2")
      (bind _asbp_table (cast `/Game/generative_Maps/Room-Generation/TableRooms/BP_Table` self))
      (`/Game/generative_Maps/Room-Generation/TableRooms/BP_Table.UpdateTableRotation` _asbp_table))))

(event `self.ReceiveBeginPlay`
  (bind (_returnvalue_x _returnvalue_y) (`KismetMathLibrary.BreakVector` (`self.K2_GetActorLocation`)))
  (set `self.Coordinates` (`KismetMathLibrary.MakeVector2D` _returnvalue_x _returnvalue_y))
  (set `self.Walls` 4))

(event `Create Paths`
  (params (`Grid Size` :type "Vector2D Structure"))
  (bind (_x _y) (`KismetMathLibrary.BreakVector2D` `Grid Size`))
  (bind _front (`self.Front`))
  (bind _back (`self.Back`))
  (bind _left (`self.Left`))
  (bind _right (`self.Right`))
  (bind (_coordinates_x _coordinates_y) (`KismetMathLibrary.BreakVector2D` (`self.Coordinates`)))
  (bind (_coordinates_x_2 _coordinates_y_2) (`KismetMathLibrary.BreakVector2D` (`self.Coordinates`)))
  (bind _coordinates_x_3 (`KismetMathLibrary.BreakVector2D` (`self.Coordinates`)))
  (if (not (`self.Paths Done`))
    (for _array_element (`self.Room Connections`)
      (if (!= self _array_element)
        (`|ExecutionSequence`
          (:`then_0`
            (bind (_coordinates_x_4 _coordinates_y_3) (`KismetMathLibrary.BreakVector2D` (`/Game/generative_Maps/Room-Generation/EmptyRooms/BP_RoomParent.Coordinates` _array_element)))
            (bind _returnvalue (== _coordinates_x_4 (+ _coordinates_x _x)))
            (bind _returnvalue_2 (== _coordinates_y_3 _coordinates_y_2))
            (if (and _returnvalue _returnvalue_2)
              (bind _returnvalue_3 (`|EnumInequality` (`/Game/generative_Maps/Room-Generation/EmptyRooms/BP_RoomParent.RotationType` _array_element) "NewEnumerator0"))
              (if _returnvalue_3
                (`SceneComponent.SetVisibility` _front false true)
                (`PrimitiveComponent.SetCollisionEnabled` _front "NoCollision")
                (`/Engine/EditorBlueprintResources/StandardMacros.DecrementInt` (`self.Walls`)
                  (:`  `
                    (bind _room_level (`/Game/generative_Maps/Room-Generation/EmptyRooms/BP_RoomParent.Room Level` _array_element))
                    (if (or (`|EnumEquality` "NewEnumerator0" _room_level) (`|EnumEquality` _room_level "NewEnumerator2"))
                      (`/Engine/EditorBlueprintResources/StandardMacros.IncrementInt` (`self.Tables`)
                        (:`  `
                          (`SceneComponent.SetVisibility` (`self.FrontOpen`) false true)))))))
              (`BlueprintMapLibrary.Map_Add` (`self.Neighboor Rotation Types`) 0 (`/Game/generative_Maps/Room-Generation/EmptyRooms/BP_RoomParent.RotationType` _array_element))
              (`BlueprintMapLibrary.Map_Add` (`self.Neighboor Level Types`) 0 _array_element)))
          (:`then_1`
            (bind _returnvalue_4 (== _coordinates_x_4 (- _coordinates_x _x)))
            (if (and _returnvalue_2 _returnvalue_4)
              (if _returnvalue_3
                (`SceneComponent.SetVisibility` _back false true)
                (`PrimitiveComponent.SetCollisionEnabled` _back "NoCollision")
                (`/Engine/EditorBlueprintResources/StandardMacros.DecrementInt` (`self.Walls`)
                  (:`  `
                    (bind _room_level_2 (`/Game/generative_Maps/Room-Generation/EmptyRooms/BP_RoomParent.Room Level` _array_element))
                    (if (or (`|EnumEquality` "NewEnumerator0" _room_level_2) (`|EnumEquality` _room_level_2 "NewEnumerator2"))
                      (`/Engine/EditorBlueprintResources/StandardMacros.IncrementInt` (`self.Tables`)
                        (:`  `
                          (`SceneComponent.SetVisibility` (`self.BackOpen`) false true)))))))
              (`BlueprintMapLibrary.Map_Add` (`self.Neighboor Rotation Types`) 1 (`/Game/generative_Maps/Room-Generation/EmptyRooms/BP_RoomParent.RotationType` _array_element))
              (`BlueprintMapLibrary.Map_Add` (`self.Neighboor Level Types`) 1 _array_element)))
          (:`then_2`
            (bind _returnvalue_5 (== _coordinates_y_3 (+ _coordinates_y _y)))
            (bind _returnvalue_6 (== _coordinates_x_4 _coordinates_x_3))
            (if (and _returnvalue_5 _returnvalue_6)
              (if _returnvalue_3
                (`SceneComponent.SetVisibility` _right false true)
                (`PrimitiveComponent.SetCollisionEnabled` _right "NoCollision")
                (`/Engine/EditorBlueprintResources/StandardMacros.DecrementInt` (`self.Walls`)
                  (:`  `
                    (bind _room_level_3 (`/Game/generative_Maps/Room-Generation/EmptyRooms/BP_RoomParent.Room Level` _array_element))
                    (if (or (`|EnumEquality` "NewEnumerator0" _room_level_3) (`|EnumEquality` _room_level_3 "NewEnumerator2"))
                      (`/Engine/EditorBlueprintResources/StandardMacros.IncrementInt` (`self.Tables`)
                        (:`  `
                          (`SceneComponent.SetVisibility` (`self.RightOpen`) false true)))))))
              (`BlueprintMapLibrary.Map_Add` (`self.Neighboor Rotation Types`) 2 (`/Game/generative_Maps/Room-Generation/EmptyRooms/BP_RoomParent.RotationType` _array_element))
              (`BlueprintMapLibrary.Map_Add` (`self.Neighboor Level Types`) 2 _array_element)))
          (:`then_3`
            (bind _returnvalue_7 (== _coordinates_y_3 (- _coordinates_y _y)))
            (if (and _returnvalue_6 _returnvalue_7)
              (if _returnvalue_3
                (`SceneComponent.SetVisibility` _left false true)
                (`PrimitiveComponent.SetCollisionEnabled` _left "NoCollision")
                (`/Engine/EditorBlueprintResources/StandardMacros.DecrementInt` (`self.Walls`)
                  (:`  `
                    (bind _room_level_4 (`/Game/generative_Maps/Room-Generation/EmptyRooms/BP_RoomParent.Room Level` _array_element))
                    (if (or (`|EnumEquality` "NewEnumerator0" _room_level_4) (`|EnumEquality` _room_level_4 "NewEnumerator2"))
                      (`/Engine/EditorBlueprintResources/StandardMacros.IncrementInt` (`self.Tables`)
                        (:`  `
                          (`SceneComponent.SetVisibility` (`self.LeftOpen`) false true)))))))
              (`BlueprintMapLibrary.Map_Add` (`self.Neighboor Rotation Types`) 3 (`/Game/generative_Maps/Room-Generation/EmptyRooms/BP_RoomParent.RotationType` _array_element))
              (`BlueprintMapLibrary.Map_Add` (`self.Neighboor Level Types`) 3 _array_element)))
          (:`then_4`
            (if (and _returnvalue _returnvalue_5)
              (`BlueprintMapLibrary.Map_Add` (`self.Neighboor Level Types`) 4 _array_element)))
          (:`then_5`
            (if (and _returnvalue _returnvalue_7)
              (`BlueprintMapLibrary.Map_Add` (`self.Neighboor Level Types`) 5 _array_element)))
          (:`then_6`
            (if (and _returnvalue_4 _returnvalue_5)
              (`BlueprintMapLibrary.Map_Add` (`self.Neighboor Level Types`) 6 _array_element)))
          (:`then_7`
            (if (and _returnvalue_4 _returnvalue_7)
              (`BlueprintMapLibrary.Map_Add` (`self.Neighboor Level Types`) 7 _array_element)))
          (:`then_8`
            (set `self.Paths Done` true)))))))

(event `Destroy Light`
  (`ActorComponent.K2_DestroyComponent` (`self.PointLight`)))

(fn `UserConstructionScript`)