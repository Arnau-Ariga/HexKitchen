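; Procedural room generator that builds a grid map of room actors on BeginPlay, tracked in an actor-to-position map.
; A cardinal random walk from the start room lays empty rooms, then neighbour passes add padding and wall tables.
; It trims bounding-box edges, swaps eligible rooms for islands, replaces lonely tables, adds an outer ring, and has rooms build paths, tables and walls.
; The interior-room pass is disconnected and never runs.
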(event `self.ReceiveBeginPlay`
  (bind (_max_cords_x _max_cords_y) (`KismetMathLibrary.BreakVector2D` (`self.Max Cords`)))
  (bind (_min_cords_x _min_cords_y) (`KismetMathLibrary.BreakVector2D` (`self.Min Cords`)))
  (bind (_max_cords_x_2 _max_cords_y_2) (`KismetMathLibrary.BreakVector2D` (`self.Max Cords`)))
  (bind (_min_cords_x_2 _min_cords_y_2) (`KismetMathLibrary.BreakVector2D` (`self.Min Cords`)))
  (bind (_max_cords_x_3 _max_cords_y_3) (`KismetMathLibrary.BreakVector2D` (`self.Max Cords`)))
  (bind (_min_cords_x_3 _min_cords_y_3) (`KismetMathLibrary.BreakVector2D` (`self.Min Cords`)))
  (set `self.Rooms Left` (`self.Room Amount`))
  (bind _returnvalue (`|SpawnActorFromClass` "/Game/generative_Maps/Room-Generation/EmptyRooms/BP_StartRoom.BP_StartRoom_C" (`KismetMathLibrary.MakeTransform` (0.0 0.0 0.0)) "Undefined" "MultiplyWithRoot" null null))
  (bind _output_get (set `self.Start Room` _returnvalue))
  (bind (_returnvalue_x _returnvalue_y) (`KismetMathLibrary.BreakVector` (`self.K2_GetActorLocation` _returnvalue)))
  (`BlueprintMapLibrary.Map_Add` (`self.Rooms`) _output_get (`KismetMathLibrary.MakeVector2D` _returnvalue_x _returnvalue_y))
  (set `self.Last Room` (`self.Start Room`))
  (bind _result (`/Engine/EditorBlueprintResources/StandardMacros.DecrementInt` (`self.Rooms Left`))
    (:`  `
      (bind _output_get_2 (set `self.Rooms Left` _result))
      (if (> _output_get_2 0) :!label _label
        (`self.Spawn Random Rooms`)
        (goto _label)
        (else
          (`KismetSystemLibrary.Delay` 0.0)
          (bind _keys (`BlueprintMapLibrary.Map_Keys` (`self.Rooms`)))
          (for _array_element _keys
            (`self.Spawn Inside Outside Rooms` _array_element))
          (bind _keys_2 (`BlueprintMapLibrary.Map_Keys` (`self.Rooms`)))
          (for _array_element_2 _keys_2
            (`self.Spawn Outside Rooms` _array_element_2))
          (bind _keys_3 (`BlueprintMapLibrary.Map_Keys` (`self.Rooms`)))
          (for _array_element_3 _keys_3
            (`|ExecutionSequence`
              (:`then_0`
                (bind (_coordinates_x _coordinates_y) (`KismetMathLibrary.BreakVector2D` (`/Game/generative_Maps/Room-Generation/EmptyRooms/BP_RoomParent.Coordinates` _array_element_3)))
                (if (> _coordinates_x _max_cords_x_2)
                  (set `self.Max Cords` (`KismetMathLibrary.MakeVector2D` _coordinates_x _max_cords_y_3))))
              (:`then_1`
                (if (< _coordinates_x _min_cords_x_2)
                  (set `self.Min Cords` (`KismetMathLibrary.MakeVector2D` _coordinates_x _min_cords_y_3))))
              (:`then_2`
                (if (> _coordinates_y _max_cords_y_2)
                  (set `self.Max Cords` (`KismetMathLibrary.MakeVector2D` _max_cords_x_3 _coordinates_y))))
              (:`then_3`
                (if (< _coordinates_y _min_cords_y_2)
                  (set `self.Min Cords` (`KismetMathLibrary.MakeVector2D` _min_cords_x_3 _coordinates_y))))))
          (bind _keys_4 (`BlueprintMapLibrary.Map_Keys` (`self.Rooms`)))
          (for _array_element_4 _keys_4
            (bind (_coordinates_x_2 _coordinates_y_2) (`KismetMathLibrary.BreakVector2D` (`/Game/generative_Maps/Room-Generation/EmptyRooms/BP_RoomParent.Coordinates` _array_element_4)))
            (if (or (== _coordinates_x_2 _max_cords_x) (== _max_cords_y _coordinates_y_2) (== _coordinates_x_2 _min_cords_x) (== _min_cords_y _coordinates_y_2))
              (`BlueprintMapLibrary.Map_Remove` (`self.Rooms`) _array_element_4)
              (`self.K2_DestroyActor` _array_element_4)))
          (bind _keys_5 (`BlueprintMapLibrary.Map_Keys` (`self.Rooms`)))
          (for _array_element_5 _keys_5
            (if (`|EnumEquality` (`/Game/generative_Maps/Room-Generation/EmptyRooms/BP_RoomParent.Room Level` _array_element_5) "NewEnumerator1")
              (`self.Spawn Inside Rooms` _array_element_5)))
          (bind _keys_6 (`BlueprintMapLibrary.Map_Keys` (`self.Rooms`)))
          (for _array_element_6 _keys_6
            (bind _keys_7 (`BlueprintMapLibrary.Map_Keys` (`self.Rooms`)))
            (set `/Game/generative_Maps/Room-Generation/EmptyRooms/BP_RoomParent.Room Connections` _keys_7 _array_element_6)
            (`/Game/generative_Maps/Room-Generation/EmptyRooms/BP_RoomParent.Create Paths` _array_element_6 (`self.Grid Size`)))
          (bind _keys_8 (`BlueprintMapLibrary.Map_Keys` (`self.Rooms`)))
          (for _array_element_7 _keys_8
            (`self.Remove Lonely Tables` _array_element_7))
          (bind _keys_9 (`BlueprintMapLibrary.Map_Keys` (`self.Rooms`)))
          (for _array_element_8 _keys_9
            (`self.Spawn Outside Dead Rooms` _array_element_8))
          (bind _keys_10 (`BlueprintMapLibrary.Map_Keys` (`self.Rooms`)))
          (for _array_element_9 _keys_10
            (bind _keys_11 (`BlueprintMapLibrary.Map_Keys` (`self.Rooms`)))
            (set `/Game/generative_Maps/Room-Generation/EmptyRooms/BP_RoomParent.Room Connections` _keys_11 _array_element_9)
            (`/Game/generative_Maps/Room-Generation/EmptyRooms/BP_RoomParent.Create Paths` _array_element_9 (`self.Grid Size`))
            (`/Game/generative_Maps/Room-Generation/EmptyRooms/BP_RoomParent.Update Tables` _array_element_9)
            (`/Game/generative_Maps/Room-Generation/EmptyRooms/BP_RoomParent.Update Walls` _array_element_9))
          (bind _keys_12 (`BlueprintMapLibrary.Map_Keys` (`self.Rooms`)))
          (for _array_element_10 _keys_12
            (bind _keys_13 (`BlueprintMapLibrary.Map_Keys` (`self.Rooms`)))
            (set `/Game/generative_Maps/Room-Generation/EmptyRooms/BP_RoomParent.Room Connections` _keys_13 _array_element_10)
            (`/Game/generative_Maps/Room-Generation/EmptyRooms/BP_RoomParent.Create Paths` _array_element_10 (`self.Grid Size`))
            (`/Game/generative_Maps/Room-Generation/EmptyRooms/BP_RoomParent.Update Tables` _array_element_10)
            (`/Game/generative_Maps/Room-Generation/EmptyRooms/BP_RoomParent.Update Walls` _array_element_10)))))))

(fn `Remove Lonely Tables`
  (params (`Current Room` :type "/Game/generative_Maps/Room-Generation/EmptyRooms/BP_RoomParent Object Reference"))
  (locals (RoomCords :type "Vector2D Structure"))
  (bind (_roomcords_x _roomcords_y) (`KismetMathLibrary.BreakVector2D` (`local.RoomCords`)))
  (if (and (`|EnumInequality` "NewEnumerator1" (`/Game/generative_Maps/Room-Generation/EmptyRooms/BP_RoomParent.Room Level` `Current Room`)) (== 0 (`/Game/generative_Maps/Room-Generation/EmptyRooms/BP_RoomParent.Tables` `Current Room`)))
    (set `local.RoomCords` (`/Game/generative_Maps/Room-Generation/EmptyRooms/BP_RoomParent.Coordinates` `Current Room`))
    (`BlueprintMapLibrary.Map_Remove` (`self.Rooms`) `Current Room`)
    (`self.K2_DestroyActor` `Current Room`)
    (bind _returnvalue (`|SpawnActorFromClass` "/Game/generative_Maps/Room-Generation/EmptyRooms/BP_EmptyRoom.BP_EmptyRoom_C" (`KismetMathLibrary.MakeTransform` (`KismetMathLibrary.MakeVector` _roomcords_x _roomcords_y)) "Undefined" "MultiplyWithRoot" null null))
    (set `/Game/generative_Maps/Room-Generation/EmptyRooms/BP_RoomParent.Room Level` "NewEnumerator1" _returnvalue)
    (set `/Game/generative_Maps/Room-Generation/EmptyRooms/BP_RoomParent.RotationType` "NewEnumerator1" _returnvalue)
    (bind (_returnvalue_x _returnvalue_y) (`KismetMathLibrary.BreakVector` (`self.K2_GetActorLocation` _returnvalue)))
    (`BlueprintMapLibrary.Map_Add` (`self.Rooms`) _returnvalue (`KismetMathLibrary.MakeVector2D` _returnvalue_x _returnvalue_y))))

(fn `Spawn Inside Outside Rooms`
  (params (CurrentRoom :type "/Game/generative_Maps/Room-Generation/EmptyRooms/BP_RoomParent Object Reference"))
  (locals (`Potential Loc` :type "Vector2D Structure") (`Current Room` :type "/Game/generative_Maps/Room-Generation/EmptyRooms/BP_RoomParent Object Reference"))
  (bind _grid_size_x (`KismetMathLibrary.BreakVector2D` (`self.Grid Size`)))
  (bind (_grid_size_x_2 _grid_size_y) (`KismetMathLibrary.BreakVector2D` (`self.Grid Size`)))
  (bind _grid_size_x_3 (`KismetMathLibrary.BreakVector2D` (`self.Grid Size`)))
  (bind (_grid_size_x_4 _grid_size_y_2) (`KismetMathLibrary.BreakVector2D` (`self.Grid Size`)))
  (bind (_grid_size_x_5 _grid_size_y_3) (`KismetMathLibrary.BreakVector2D` (`self.Grid Size`)))
  (bind (_grid_size_x_6 _grid_size_y_4) (`KismetMathLibrary.BreakVector2D` (`self.Grid Size`)))
  (bind (_grid_size_x_7 _grid_size_y_5) (`KismetMathLibrary.BreakVector2D` (`self.Grid Size`)))
  (bind (_grid_size_x_8 _grid_size_y_6) (`KismetMathLibrary.BreakVector2D` (`self.Grid Size`)))
  (bind (_potential_loc_x _potential_loc_y) (`KismetMathLibrary.BreakVector2D` (`local.Potential Loc`)))
  (bind _value (`BlueprintMapLibrary.Map_Find` (`self.Rooms`) CurrentRoom))
  (bind (_x _y) (`KismetMathLibrary.BreakVector2D` _value))
  (bind (_x_2 _y_2) (`KismetMathLibrary.BreakVector2D` _value))
  (bind (_x_3 _y_3) (`KismetMathLibrary.BreakVector2D` _value))
  (bind (_x_4 _y_4) (`KismetMathLibrary.BreakVector2D` _value))
  (bind (_x_5 _y_5) (`KismetMathLibrary.BreakVector2D` _value))
  (bind (_x_6 _y_6) (`KismetMathLibrary.BreakVector2D` _value))
  (bind (_x_7 _y_7) (`KismetMathLibrary.BreakVector2D` _value))
  (bind (_x_8 _y_8) (`KismetMathLibrary.BreakVector2D` _value))
  (for _array_element (`|MakeArray` (`KismetMathLibrary.MakeVector2D` (+ _x_2 _grid_size_x) _y_2) (`KismetMathLibrary.MakeVector2D` _x_3 (+ _y_3 _grid_size_y)) (`KismetMathLibrary.MakeVector2D` (- _x_4 _grid_size_x_3) _y_4) (`KismetMathLibrary.MakeVector2D` _x_5 (- _y_5 _grid_size_y_2)) (`KismetMathLibrary.MakeVector2D` (+ _x_7 _grid_size_x_7) (+ _y_7 _grid_size_y_5)) (`KismetMathLibrary.MakeVector2D` (- _x_8 _grid_size_x_8) (+ _y_8 _grid_size_y_6)) (`KismetMathLibrary.MakeVector2D` (+ _x_6 _grid_size_x_6) (- _y_6 _grid_size_y_4)) (`KismetMathLibrary.MakeVector2D` (- _x _grid_size_x_5) (- _y _grid_size_y_3)))
    (bind _output_get (set `local.Potential Loc` _array_element))
    (bind _values (`BlueprintMapLibrary.Map_Values` (`self.Rooms`)))
    (if (not (`KismetArrayLibrary.Array_Contains` _values _output_get))
      (bind _returnvalue (`|SpawnActorFromClass` "/Game/generative_Maps/Room-Generation/EmptyRooms/BP_EmptyRoom.BP_EmptyRoom_C" (`KismetMathLibrary.MakeTransform` (`KismetMathLibrary.MakeVector` _potential_loc_x _potential_loc_y)) "Undefined" "MultiplyWithRoot" null null))
      (set `/Game/generative_Maps/Room-Generation/EmptyRooms/BP_RoomParent.Room Level` "NewEnumerator1" _returnvalue)
      (set `/Game/generative_Maps/Room-Generation/EmptyRooms/BP_RoomParent.RotationType` "NewEnumerator1" _returnvalue)
      (bind (_returnvalue_x _returnvalue_y) (`KismetMathLibrary.BreakVector` (`self.K2_GetActorLocation` _returnvalue)))
      (`BlueprintMapLibrary.Map_Add` (`self.Rooms`) _returnvalue (`KismetMathLibrary.MakeVector2D` _returnvalue_x _returnvalue_y))))
  (return))

(fn `Spawn Inside Rooms`
  (params (`Current Room` :type "/Game/generative_Maps/Room-Generation/EmptyRooms/BP_RoomParent Object Reference"))
  (locals (Offsets :type "Array of Vector2D Structure") (`Island Cords` :type "Vector2D Structure"))
  (bind (_island_cords_x _island_cords_y) (`KismetMathLibrary.BreakVector2D` (`local.Island Cords`)))
  (bind _rooms (`self.Rooms`))
  (for (_array_element _array_index) (`local.Offsets`)
    (`KismetArrayLibrary.Array_Set` (`local.Offsets`) _array_index (+ (`BlueprintMapLibrary.Map_Find` (`self.Rooms`) `Current Room`) (* _array_element (`self.Grid Size`)))))
  (for _array_element_2 (`local.Offsets`)
    (bind _values (`BlueprintMapLibrary.Map_Values` _rooms))
    (if (`|EnumEquality` (`/Game/generative_Maps/Room-Generation/EmptyRooms/BP_RoomParent.Room Level` (`BlueprintMapLibrary.Map_GetKeyValueByIndex` _rooms (`KismetArrayLibrary.Array_Find` _values _array_element_2))) "NewEnumerator0")
      (set `/Game/generative_Maps/Room-Generation/EmptyRooms/BP_RoomParent.Can Be Island` false `Current Room`)))
  (if (`/Game/generative_Maps/Room-Generation/EmptyRooms/BP_RoomParent.Can Be Island` `Current Room`)
    (set `local.Island Cords` (`/Game/generative_Maps/Room-Generation/EmptyRooms/BP_RoomParent.Coordinates` `Current Room`))
    (`BlueprintMapLibrary.Map_Remove` (`self.Rooms`) `Current Room`)
    (`self.K2_DestroyActor` `Current Room`)
    (bind _returnvalue (`|SpawnActorFromClass` "/Game/generative_Maps/Room-Generation/TableRooms/BP_Island.BP_Island_C" (`KismetMathLibrary.MakeTransform` (`KismetMathLibrary.MakeVector` _island_cords_x _island_cords_y)) "Undefined" "MultiplyWithRoot" null null))
    (set `/Game/generative_Maps/Room-Generation/EmptyRooms/BP_RoomParent.Room Level` "NewEnumerator2" _returnvalue)
    (set `/Game/generative_Maps/Room-Generation/EmptyRooms/BP_RoomParent.RotationType` "NewEnumerator2" _returnvalue)
    (bind (_returnvalue_x _returnvalue_y) (`KismetMathLibrary.BreakVector` (`self.K2_GetActorLocation` _returnvalue)))
    (`BlueprintMapLibrary.Map_Add` (`self.Rooms`) _returnvalue (`KismetMathLibrary.MakeVector2D` _returnvalue_x _returnvalue_y))))

(fn `Spawn Interior Rooms`
  (params (`Current Room` :type "/Game/generative_Maps/Room-Generation/EmptyRooms/BP_RoomParent Object Reference"))
  (locals (Offsets :type "Array of Vector2D Structure") (`Island Cords` :type "Vector2D Structure"))
  (bind (_island_cords_x _island_cords_y) (`KismetMathLibrary.BreakVector2D` (`local.Island Cords`)))
  (bind _rooms (`self.Rooms`))
  (if (`|EnumEquality` (`/Game/generative_Maps/Room-Generation/EmptyRooms/BP_RoomParent.Room Level` `Current Room`) "NewEnumerator4")
    (for (_array_element _array_index) (`local.Offsets`)
      (`KismetArrayLibrary.Array_Set` (`local.Offsets`) _array_index (+ (`BlueprintMapLibrary.Map_Find` (`self.Rooms`) `Current Room`) (* _array_element (`self.Grid Size`)))))
    (for _array_element_2 (`local.Offsets`)
      (bind _values (`BlueprintMapLibrary.Map_Values` _rooms))
      (if (not (`|EnumEquality` (`/Game/generative_Maps/Room-Generation/EmptyRooms/BP_RoomParent.Room Level` (`BlueprintMapLibrary.Map_GetKeyValueByIndex` _rooms (`KismetArrayLibrary.Array_Find` _values _array_element_2))) "NewEnumerator4"))
        (set `/Game/generative_Maps/Room-Generation/EmptyRooms/BP_RoomParent.Can Be Interior` true `Current Room`)))
    (if (`/Game/generative_Maps/Room-Generation/EmptyRooms/BP_RoomParent.Can Be Interior` `Current Room`)
      (set `local.Island Cords` (`/Game/generative_Maps/Room-Generation/EmptyRooms/BP_RoomParent.Coordinates` `Current Room`))
      (`BlueprintMapLibrary.Map_Remove` (`self.Rooms`) `Current Room`)
      (`self.K2_DestroyActor` `Current Room`)
      (bind _returnvalue (`|SpawnActorFromClass` "/Game/generative_Maps/Room-Generation/EmptyRooms/BP_InteriorRoom.BP_InteriorRoom_C" (`KismetMathLibrary.MakeTransform` (`KismetMathLibrary.MakeVector` _island_cords_x _island_cords_y)) "Undefined" "MultiplyWithRoot" null null))
      (set `/Game/generative_Maps/Room-Generation/EmptyRooms/BP_RoomParent.Room Level` "NewEnumerator4" _returnvalue)
      (set `/Game/generative_Maps/Room-Generation/EmptyRooms/BP_RoomParent.RotationType` "NewEnumerator1" _returnvalue)
      (bind (_returnvalue_x _returnvalue_y) (`KismetMathLibrary.BreakVector` (`self.K2_GetActorLocation` _returnvalue)))
      (`BlueprintMapLibrary.Map_Add` (`self.Rooms`) _returnvalue (`KismetMathLibrary.MakeVector2D` _returnvalue_x _returnvalue_y)))))

(fn `Spawn Outside Dead Rooms`
  (params (CurrentRoom :type "/Game/generative_Maps/Room-Generation/EmptyRooms/BP_RoomParent Object Reference"))
  (locals (`Potential Loc` :type "Vector2D Structure") (`Current Room` :type "/Game/generative_Maps/Room-Generation/EmptyRooms/BP_RoomParent Object Reference"))
  (bind _grid_size_x (`KismetMathLibrary.BreakVector2D` (`self.Grid Size`)))
  (bind (_grid_size_x_2 _grid_size_y) (`KismetMathLibrary.BreakVector2D` (`self.Grid Size`)))
  (bind _grid_size_x_3 (`KismetMathLibrary.BreakVector2D` (`self.Grid Size`)))
  (bind (_grid_size_x_4 _grid_size_y_2) (`KismetMathLibrary.BreakVector2D` (`self.Grid Size`)))
  (bind (_grid_size_x_5 _grid_size_y_3) (`KismetMathLibrary.BreakVector2D` (`self.Grid Size`)))
  (bind (_grid_size_x_6 _grid_size_y_4) (`KismetMathLibrary.BreakVector2D` (`self.Grid Size`)))
  (bind (_grid_size_x_7 _grid_size_y_5) (`KismetMathLibrary.BreakVector2D` (`self.Grid Size`)))
  (bind (_grid_size_x_8 _grid_size_y_6) (`KismetMathLibrary.BreakVector2D` (`self.Grid Size`)))
  (bind (_potential_loc_x _potential_loc_y) (`KismetMathLibrary.BreakVector2D` (`local.Potential Loc`)))
  (bind _value (`BlueprintMapLibrary.Map_Find` (`self.Rooms`) CurrentRoom))
  (bind (_x _y) (`KismetMathLibrary.BreakVector2D` _value))
  (bind (_x_2 _y_2) (`KismetMathLibrary.BreakVector2D` _value))
  (bind (_x_3 _y_3) (`KismetMathLibrary.BreakVector2D` _value))
  (bind (_x_4 _y_4) (`KismetMathLibrary.BreakVector2D` _value))
  (bind (_x_5 _y_5) (`KismetMathLibrary.BreakVector2D` _value))
  (bind (_x_6 _y_6) (`KismetMathLibrary.BreakVector2D` _value))
  (bind (_x_7 _y_7) (`KismetMathLibrary.BreakVector2D` _value))
  (bind (_x_8 _y_8) (`KismetMathLibrary.BreakVector2D` _value))
  (for _array_element (`|MakeArray` (`KismetMathLibrary.MakeVector2D` (+ _x_2 _grid_size_x) _y_2) (`KismetMathLibrary.MakeVector2D` _x_3 (+ _y_3 _grid_size_y)) (`KismetMathLibrary.MakeVector2D` (- _x_4 _grid_size_x_3) _y_4) (`KismetMathLibrary.MakeVector2D` _x_5 (- _y_5 _grid_size_y_2)) (`KismetMathLibrary.MakeVector2D` (+ _x_7 _grid_size_x_7) (+ _y_7 _grid_size_y_5)) (`KismetMathLibrary.MakeVector2D` (- _x_8 _grid_size_x_8) (+ _y_8 _grid_size_y_6)) (`KismetMathLibrary.MakeVector2D` (+ _x_6 _grid_size_x_6) (- _y_6 _grid_size_y_4)) (`KismetMathLibrary.MakeVector2D` (- _x _grid_size_x_5) (- _y _grid_size_y_3)))
    (bind _output_get (set `local.Potential Loc` _array_element))
    (bind _values (`BlueprintMapLibrary.Map_Values` (`self.Rooms`)))
    (if (not (`KismetArrayLibrary.Array_Contains` _values _output_get))
      (bind _returnvalue (`|SpawnActorFromClass` "/Game/generative_Maps/Room-Generation/EmptyRooms/BP_EmptyRoom.BP_EmptyRoom_C" (`KismetMathLibrary.MakeTransform` (`KismetMathLibrary.MakeVector` _potential_loc_x _potential_loc_y)) "Undefined" "MultiplyWithRoot" null null))
      (set `/Game/generative_Maps/Room-Generation/EmptyRooms/BP_RoomParent.Room Level` "NewEnumerator1" _returnvalue)
      (set `/Game/generative_Maps/Room-Generation/EmptyRooms/BP_RoomParent.RotationType` "NewEnumerator0" _returnvalue)
      (bind (_returnvalue_x _returnvalue_y) (`KismetMathLibrary.BreakVector` (`self.K2_GetActorLocation` _returnvalue)))
      (`BlueprintMapLibrary.Map_Add` (`self.Rooms`) _returnvalue (`KismetMathLibrary.MakeVector2D` _returnvalue_x _returnvalue_y))))
  (return))

(fn `Spawn Outside Rooms`
  (params (CurrentRoom :type "/Game/generative_Maps/Room-Generation/EmptyRooms/BP_RoomParent Object Reference"))
  (locals (`Potential Loc` :type "Vector2D Structure") (`Current Room` :type "/Game/generative_Maps/Room-Generation/EmptyRooms/BP_RoomParent Object Reference"))
  (bind _grid_size_x (`KismetMathLibrary.BreakVector2D` (`self.Grid Size`)))
  (bind (_grid_size_x_2 _grid_size_y) (`KismetMathLibrary.BreakVector2D` (`self.Grid Size`)))
  (bind _grid_size_x_3 (`KismetMathLibrary.BreakVector2D` (`self.Grid Size`)))
  (bind (_grid_size_x_4 _grid_size_y_2) (`KismetMathLibrary.BreakVector2D` (`self.Grid Size`)))
  (bind (_grid_size_x_5 _grid_size_y_3) (`KismetMathLibrary.BreakVector2D` (`self.Grid Size`)))
  (bind (_grid_size_x_6 _grid_size_y_4) (`KismetMathLibrary.BreakVector2D` (`self.Grid Size`)))
  (bind (_grid_size_x_7 _grid_size_y_5) (`KismetMathLibrary.BreakVector2D` (`self.Grid Size`)))
  (bind (_grid_size_x_8 _grid_size_y_6) (`KismetMathLibrary.BreakVector2D` (`self.Grid Size`)))
  (bind (_potential_loc_x _potential_loc_y) (`KismetMathLibrary.BreakVector2D` (`local.Potential Loc`)))
  (bind _value (`BlueprintMapLibrary.Map_Find` (`self.Rooms`) CurrentRoom))
  (bind (_x _y) (`KismetMathLibrary.BreakVector2D` _value))
  (bind (_x_2 _y_2) (`KismetMathLibrary.BreakVector2D` _value))
  (bind (_x_3 _y_3) (`KismetMathLibrary.BreakVector2D` _value))
  (bind (_x_4 _y_4) (`KismetMathLibrary.BreakVector2D` _value))
  (bind (_x_5 _y_5) (`KismetMathLibrary.BreakVector2D` _value))
  (bind (_x_6 _y_6) (`KismetMathLibrary.BreakVector2D` _value))
  (bind (_x_7 _y_7) (`KismetMathLibrary.BreakVector2D` _value))
  (bind (_x_8 _y_8) (`KismetMathLibrary.BreakVector2D` _value))
  (for _array_element (`|MakeArray` (`KismetMathLibrary.MakeVector2D` (+ _x_2 _grid_size_x) _y_2) (`KismetMathLibrary.MakeVector2D` _x_3 (+ _y_3 _grid_size_y)) (`KismetMathLibrary.MakeVector2D` (- _x_4 _grid_size_x_3) _y_4) (`KismetMathLibrary.MakeVector2D` _x_5 (- _y_5 _grid_size_y_2)) (`KismetMathLibrary.MakeVector2D` (+ _x_7 _grid_size_x_7) (+ _y_7 _grid_size_y_5)) (`KismetMathLibrary.MakeVector2D` (- _x_8 _grid_size_x_8) (+ _y_8 _grid_size_y_6)) (`KismetMathLibrary.MakeVector2D` (+ _x_6 _grid_size_x_6) (- _y_6 _grid_size_y_4)) (`KismetMathLibrary.MakeVector2D` (- _x _grid_size_x_5) (- _y _grid_size_y_3)))
    (bind _output_get (set `local.Potential Loc` _array_element))
    (bind _values (`BlueprintMapLibrary.Map_Values` (`self.Rooms`)))
    (if (not (`KismetArrayLibrary.Array_Contains` _values _output_get))
      (bind _returnvalue (`|SpawnActorFromClass` "/Game/generative_Maps/Room-Generation/TableRooms/BP_WallTable.BP_WallTable_C" (`KismetMathLibrary.MakeTransform` (`KismetMathLibrary.MakeVector` _potential_loc_x _potential_loc_y)) "Undefined" "MultiplyWithRoot" null null))
      (set `/Game/generative_Maps/Room-Generation/EmptyRooms/BP_RoomParent.Room Level` "NewEnumerator0" _returnvalue)
      (set `/Game/generative_Maps/Room-Generation/EmptyRooms/BP_RoomParent.RotationType` "NewEnumerator2" _returnvalue)
      (bind (_returnvalue_x _returnvalue_y) (`KismetMathLibrary.BreakVector` (`self.K2_GetActorLocation` _returnvalue)))
      (`BlueprintMapLibrary.Map_Add` (`self.Rooms`) _returnvalue (`KismetMathLibrary.MakeVector2D` _returnvalue_x _returnvalue_y))))
  (return))

(fn `Spawn Random Rooms`
  (locals (`Potential Loc` :type "Vector2D Structure") (`Current Room` :type "/Game/generative_Maps/Room-Generation/EmptyRooms/BP_RoomParent Object Reference"))
  (bind _rooms (`self.Rooms`))
  (bind _grid_size_x (`KismetMathLibrary.BreakVector2D` (`self.Grid Size`)))
  (bind (_grid_size_x_2 _grid_size_y) (`KismetMathLibrary.BreakVector2D` (`self.Grid Size`)))
  (bind _grid_size_x_3 (`KismetMathLibrary.BreakVector2D` (`self.Grid Size`)))
  (bind (_grid_size_x_4 _grid_size_y_2) (`KismetMathLibrary.BreakVector2D` (`self.Grid Size`)))
  (bind _current_room (`local.Current Room`))
  (bind (_grid_size_x_5 _grid_size_y_3) (`KismetMathLibrary.BreakVector2D` (`self.Grid Size`)))
  (bind (_grid_size_x_6 _grid_size_y_4) (`KismetMathLibrary.BreakVector2D` (`self.Grid Size`)))
  (bind (_grid_size_x_7 _grid_size_y_5) (`KismetMathLibrary.BreakVector2D` (`self.Grid Size`)))
  (bind (_grid_size_x_8 _grid_size_y_6) (`KismetMathLibrary.BreakVector2D` (`self.Grid Size`)))
  (bind (_potential_loc_x _potential_loc_y) (`KismetMathLibrary.BreakVector2D` (`local.Potential Loc`)))
  (bind _value (`BlueprintMapLibrary.Map_Find` (`self.Rooms`) (`self.Last Room`)))
  (bind (_x _y) (`KismetMathLibrary.BreakVector2D` _value))
  (bind (_x_2 _y_2) (`KismetMathLibrary.BreakVector2D` _value))
  (bind (_x_3 _y_3) (`KismetMathLibrary.BreakVector2D` _value))
  (bind (_x_4 _y_4) (`KismetMathLibrary.BreakVector2D` _value))
  (bind (_x_5 _y_5) (`KismetMathLibrary.BreakVector2D` _value))
  (bind (_x_6 _y_6) (`KismetMathLibrary.BreakVector2D` _value))
  (bind (_x_7 _y_7) (`KismetMathLibrary.BreakVector2D` _value))
  (bind (_x_8 _y_8) (`KismetMathLibrary.BreakVector2D` _value))
  (bind _output_get (set `local.Potential Loc` (select `int` (`KismetMathLibrary.RandomInteger` 4) :`0` (`KismetMathLibrary.MakeVector2D` (+ _x_2 _grid_size_x) _y_2) :`1` (`KismetMathLibrary.MakeVector2D` _x_3 (+ _y_3 _grid_size_y)) :`2` (`KismetMathLibrary.MakeVector2D` (- _x_4 _grid_size_x_3) _y_4) :`3` (`KismetMathLibrary.MakeVector2D` _x_5 (- _y_5 _grid_size_y_2)) :`4` (`KismetMathLibrary.MakeVector2D` (+ _x_7 _grid_size_x_7) (+ _y_7 _grid_size_y_5)) :`5` (`KismetMathLibrary.MakeVector2D` (- _x_8 _grid_size_x_8) (+ _y_8 _grid_size_y_6)) :`6` (`KismetMathLibrary.MakeVector2D` (+ _x_6 _grid_size_x_6) (- _y_6 _grid_size_y_4)) :`7` (`KismetMathLibrary.MakeVector2D` (- _x _grid_size_x_5) (- _y _grid_size_y_3)))))
  (bind _values (`BlueprintMapLibrary.Map_Values` (`self.Rooms`)))
  (if (`KismetArrayLibrary.Array_Contains` _values _output_get)
    (bind _values_2 (`BlueprintMapLibrary.Map_Values` _rooms))
    (`BlueprintMapLibrary.Map_Keys` _rooms)
    (set `self.Last Room` (`BlueprintMapLibrary.Map_GetKeyValueByIndex` _rooms (`KismetArrayLibrary.Array_Find` _values_2 (`local.Potential Loc`))))
    (return)
    (else
      (bind _returnvalue (`|SpawnActorFromClass` "/Game/generative_Maps/Room-Generation/EmptyRooms/BP_EmptyRoom.BP_EmptyRoom_C" (`KismetMathLibrary.MakeTransform` (`KismetMathLibrary.MakeVector` _potential_loc_x _potential_loc_y)) "Undefined" "MultiplyWithRoot" null null))
      (bind _output_get_2 (set `local.Current Room` _returnvalue))
      (bind (_returnvalue_x _returnvalue_y) (`KismetMathLibrary.BreakVector` (`self.K2_GetActorLocation` _returnvalue)))
      (`BlueprintMapLibrary.Map_Add` (`self.Rooms`) _output_get_2 (`KismetMathLibrary.MakeVector2D` _returnvalue_x _returnvalue_y))
      (bind _result (`/Engine/EditorBlueprintResources/StandardMacros.DecrementInt` (stale _output_get_3))
        (:`  `
          (bind _output_get_3 (set `self.Rooms Left` _result))
          (set `/Game/generative_Maps/Room-Generation/EmptyRooms/BP_RoomParent.Room Level` "NewEnumerator1" _current_room)
          (set `/Game/generative_Maps/Room-Generation/EmptyRooms/BP_RoomParent.RotationType` "NewEnumerator1" _current_room)
          (return))))))

(fn `UserConstructionScript`)