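; BP_Table is a table room piece for generative map generation that picks its table mesh and yaw from neighboring rooms.
; UpdateTableRotation scans DT_Rotations for rows whose Front, Back, Right and Left values match NeighboorRotationTypes.
; A match sets the intersection type, rotates the Table, shows the angle on debug text and swaps in the corresponding mesh.
; One intersection type also changes RoomLevel.
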(event `UpdateTableRotation`
  (bind _intersection (`self.Intersection`))
  (bind _table (`self.Table`))
  (bind _neighboor_rotation_types (`self.Neighboor Rotation Types`))
  (bind _outrownames (`DataTableFunctionLibrary.GetDataTableRowNames` "/Game/generative_Maps/Room-Generation/DataTables/Rotations/DT_Rotations.DT_Rotations"))
  (for _array_element _outrownames
    (bind _returnvalue (`|GetDataTableRow` "/Game/generative_Maps/Room-Generation/DataTables/Rotations/DT_Rotations.DT_Rotations" _array_element)
      (:`then`
        (if (and (`|EnumEquality` (`.Front_42_463A41BE4AC590697F36DB89707258B5` (break `/Game/generative_Maps/Room-Generation/DataTables/Rotations/RotationBase` _returnvalue)) (`BlueprintMapLibrary.Map_Find` _neighboor_rotation_types)) (`|EnumEquality` (`.Back_52_E1FDF1614F1EBFD40B6196B8B844E1C3` (break `/Game/generative_Maps/Room-Generation/DataTables/Rotations/RotationBase` _returnvalue)) (`BlueprintMapLibrary.Map_Find` _neighboor_rotation_types 1)) (`|EnumEquality` (`.Right_53_AAC2A6E4408E3A4C1BF9A091793C4DE2` (break `/Game/generative_Maps/Room-Generation/DataTables/Rotations/RotationBase` _returnvalue)) (`BlueprintMapLibrary.Map_Find` _neighboor_rotation_types 2)) (`|EnumEquality` (`.Left_51_C37BC59B412ABE698E29339F893B3A30` (break `/Game/generative_Maps/Room-Generation/DataTables/Rotations/RotationBase` _returnvalue)) (`BlueprintMapLibrary.Map_Find` _neighboor_rotation_types 3)))
          (set `self.Intersection` (break `/Game/generative_Maps/Room-Generation/DataTables/Rotations/RotationBase` _returnvalue))
          (bind _returnvalue_2 (`KismetMathLibrary.Conv_IntToDouble` (`.Rotation_57_71C512F8401ABE52AA763390923C0B80` (break `/Game/generative_Maps/Room-Generation/DataTables/Rotations/RotationBase` _returnvalue))))
          (`SceneComponent.K2_SetRelativeRotation` (`self.Table`) (`KismetMathLibrary.MakeRotator` 0.0 0.0 _returnvalue_2) false false)
          (`TextRenderComponent.K2_SetText` (`self.DebugIntersection Table`) (`KismetTextLibrary.Conv_DoubleToText` _returnvalue_2 "HalfToEven"))
          (`|ExecutionSequence`
            (:`then_0`
              (if (`|EnumEquality` _intersection "NewEnumerator2")
                (`StaticMeshComponent.SetStaticMesh` _table "/Game/generative_Maps/Table-Tops/Table/Billy.Billy")))
            (:`then_1`
              (if (`|EnumEquality` _intersection "NewEnumerator0")
                (`StaticMeshComponent.SetStaticMesh` _table "/Game/generative_Maps/Table-Tops/Table/Bob.Bob")))
            (:`then_2`
              (if (`|EnumEquality` _intersection "NewEnumerator1")
                (`StaticMeshComponent.SetStaticMesh` _table "/Game/generative_Maps/Table-Tops/Table/Joee.Joee")))
            (:`then_3`
              (if (`|EnumEquality` _intersection "NewEnumerator5")
                (`StaticMeshComponent.SetStaticMesh` _table "/Game/generative_Maps/Table-Tops/Table/Jimm.Jimm")))
            (:`then_4`
              (if (`|EnumEquality` _intersection "NewEnumerator3")
                (`StaticMeshComponent.SetStaticMesh` _table "/Game/generative_Maps/Table-Tops/Table/tom.tom")))
            (:`then_5`
              (if (`|EnumEquality` _intersection "NewEnumerator6")
                (`StaticMeshComponent.SetStaticMesh` _table "/Game/generative_Maps/Table-Tops/Table/kev.kev")
                (set `self.Room Level` "NewEnumerator4")))))))))

(fn `UserConstructionScript`
  (`parent.UserConstructionScript`))