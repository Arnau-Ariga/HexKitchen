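; BP_Island is a table-room Blueprint for procedural map generation that builds its interior walls from neighboring rooms' levels.
; For one Intersection type, GenerateInteriorWall checks all eight neighbors for a specific RoomLevel, sets straight or diagonal wall meshes to match, and flags HasWalls.
; For one RotationType, it also adds diagonal filler meshes where two adjacent straight-side neighbors share that level, regardless of intersection.
; Construction defers to the parent class.
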(event `GenerateInteriorWall`
  (if (`|EnumEquality` (`self.Intersection`) "NewEnumerator6")
    (`|ExecutionSequence`
      (:`then_0`
        (if (`|EnumEquality` (`/Game/generative_Maps/Room-Generation/EmptyRooms/BP_RoomParent.Room Level` (`BlueprintMapLibrary.Map_Find` (`self.Neighboor Level Types`))) "NewEnumerator4")
          (`StaticMeshComponent.SetStaticMesh` (`self.Wall Interior Front`) "/Game/generative_Maps/Table-Tops/Table/wallsUncrosspiece.wallsUncrosspiece")
          (set `self.HasWalls` true :!label _label)))
      (:`then_1`
        (if (`|EnumEquality` (`/Game/generative_Maps/Room-Generation/EmptyRooms/BP_RoomParent.Room Level` (`BlueprintMapLibrary.Map_Find` (`self.Neighboor Level Types`) 1)) "NewEnumerator4")
          (`StaticMeshComponent.SetStaticMesh` (`self.Wall Interior Back`) "/Game/generative_Maps/Table-Tops/Table/wallsUncrosspiece.wallsUncrosspiece")
          (goto _label)))
      (:`then_2`
        (if (`|EnumEquality` (`/Game/generative_Maps/Room-Generation/EmptyRooms/BP_RoomParent.Room Level` (`BlueprintMapLibrary.Map_Find` (`self.Neighboor Level Types`) 2)) "NewEnumerator4")
          (`StaticMeshComponent.SetStaticMesh` (`self.Wall Interior Right`) "/Game/generative_Maps/Table-Tops/Table/wallsUncrosspiece.wallsUncrosspiece")
          (goto _label)))
      (:`then_3`
        (if (`|EnumEquality` (`/Game/generative_Maps/Room-Generation/EmptyRooms/BP_RoomParent.Room Level` (`BlueprintMapLibrary.Map_Find` (`self.Neighboor Level Types`) 3)) "NewEnumerator4")
          (`StaticMeshComponent.SetStaticMesh` (`self.Wall Interior Left`) "/Game/generative_Maps/Table-Tops/Table/wallsUncrosspiece.wallsUncrosspiece")
          (goto _label)))
      (:`then_4`
        (if (`|EnumEquality` (`/Game/generative_Maps/Room-Generation/EmptyRooms/BP_RoomParent.Room Level` (`BlueprintMapLibrary.Map_Find` (`self.Neighboor Level Types`) 4)) "NewEnumerator4")
          (`StaticMeshComponent.SetStaticMesh` (`self.Wall Interior Front Angle`) "/Game/generative_Maps/Table-Tops/Table/wallsUncrossDiagonal.wallsUncrossDiagonal")
          (goto _label)))
      (:`then_5`
        (if (`|EnumEquality` (`/Game/generative_Maps/Room-Generation/EmptyRooms/BP_RoomParent.Room Level` (`BlueprintMapLibrary.Map_Find` (`self.Neighboor Level Types`) 5)) "NewEnumerator4")
          (`StaticMeshComponent.SetStaticMesh` (`self.Wall Interior Back Angle`) "/Game/generative_Maps/Table-Tops/Table/wallsUncrossDiagonal.wallsUncrossDiagonal")
          (goto _label)))
      (:`then_6`
        (if (`|EnumEquality` (`/Game/generative_Maps/Room-Generation/EmptyRooms/BP_RoomParent.Room Level` (`BlueprintMapLibrary.Map_Find` (`self.Neighboor Level Types`) 6)) "NewEnumerator4")
          (`StaticMeshComponent.SetStaticMesh` (`self.Wall Interior Right Angle`) "/Game/generative_Maps/Table-Tops/Table/wallsUncrossDiagonal.wallsUncrossDiagonal")
          (goto _label)))
      (:`then_7`
        (if (`|EnumEquality` (`/Game/generative_Maps/Room-Generation/EmptyRooms/BP_RoomParent.Room Level` (`BlueprintMapLibrary.Map_Find` (`self.Neighboor Level Types`) 7)) "NewEnumerator4")
          (`StaticMeshComponent.SetStaticMesh` (`self.Wall Interior Left Angle`) "/Game/generative_Maps/Table-Tops/Table/wallsUncrossDiagonal.wallsUncrossDiagonal")
          (goto _label)))
      (:`then_8`
        (if (`|EnumEquality` (`self.RotationType`) "NewEnumerator2") :!label _label_2
          (`|ExecutionSequence`
            (:`then_0`
              (if (and (`|EnumEquality` (`/Game/generative_Maps/Room-Generation/EmptyRooms/BP_RoomParent.Room Level` (`BlueprintMapLibrary.Map_Find` (`self.Neighboor Level Types`))) "NewEnumerator4") (`|EnumEquality` (`/Game/generative_Maps/Room-Generation/EmptyRooms/BP_RoomParent.Room Level` (`BlueprintMapLibrary.Map_Find` (`self.Neighboor Level Types`) 2)) "NewEnumerator4"))
                (`StaticMeshComponent.SetStaticMesh` (`self.Wall Interior Front Angle Filler`) "/Game/generative_Maps/Table-Tops/Table/wallsUncrossDiagFiller.wallsUncrossDiagFiller")))
            (:`then_1`
              (if (and (`|EnumEquality` (`/Game/generative_Maps/Room-Generation/EmptyRooms/BP_RoomParent.Room Level` (`BlueprintMapLibrary.Map_Find` (`self.Neighboor Level Types`))) "NewEnumerator4") (`|EnumEquality` (`/Game/generative_Maps/Room-Generation/EmptyRooms/BP_RoomParent.Room Level` (`BlueprintMapLibrary.Map_Find` (`self.Neighboor Level Types`) 3)) "NewEnumerator4"))
                (`StaticMeshComponent.SetStaticMesh` (`self.Wall Interior Back Angle Filler`) "/Game/generative_Maps/Table-Tops/Table/wallsUncrossDiagFiller.wallsUncrossDiagFiller")))
            (:`then_2`
              (if (and (`|EnumEquality` (`/Game/generative_Maps/Room-Generation/EmptyRooms/BP_RoomParent.Room Level` (`BlueprintMapLibrary.Map_Find` (`self.Neighboor Level Types`) 1)) "NewEnumerator4") (`|EnumEquality` (`/Game/generative_Maps/Room-Generation/EmptyRooms/BP_RoomParent.Room Level` (`BlueprintMapLibrary.Map_Find` (`self.Neighboor Level Types`) 3)) "NewEnumerator4"))
                (`StaticMeshComponent.SetStaticMesh` (`self.Wall Interior Left Angle Filler`) "/Game/generative_Maps/Table-Tops/Table/wallsUncrossDiagFiller.wallsUncrossDiagFiller")))
            (:`then_3`
              (if (and (`|EnumEquality` (`/Game/generative_Maps/Room-Generation/EmptyRooms/BP_RoomParent.Room Level` (`BlueprintMapLibrary.Map_Find` (`self.Neighboor Level Types`) 1)) "NewEnumerator4") (`|EnumEquality` (`/Game/generative_Maps/Room-Generation/EmptyRooms/BP_RoomParent.Room Level` (`BlueprintMapLibrary.Map_Find` (`self.Neighboor Level Types`) 2)) "NewEnumerator4"))
                (`StaticMeshComponent.SetStaticMesh` (`self.Wall Interior Right Angle Filler`) "/Game/generative_Maps/Table-Tops/Table/wallsUncrossDiagFiller.wallsUncrossDiagFiller")))))))
    (else
      (goto _label_2))))

(fn `UserConstructionScript`
  (`parent.UserConstructionScript`))