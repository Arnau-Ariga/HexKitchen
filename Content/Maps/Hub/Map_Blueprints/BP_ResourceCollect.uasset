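; Interactable resource pickup for the hub that represents Cheese, Rubber, Metal, Wood or Plastic, chosen by the ResourceType enum.
; Construction Script and BeginPlay run DisableOtherModels, which hides and disables collision on the four unused meshes.
; EnableCurrentModel turns on the chosen mesh's collision and nudges it out and back, without setting visibility.
; The prompt names the resource, and Interact only shows a pop-up, with no inventory change or removal.
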(event `self.ReceiveBeginPlay`
  (`self.Disable Other models`))

(event `/Game/Blueprints/Interact/BPI_Interactable.Interact`
  (`/Game/Blueprints/PopUp/FL_PopUpFunctions.SendPopUp` "/Engine/EngineResources/Development/ZenIcon.ZenIcon" (`KismetTextLibrary.Conv_StringToText` (`KismetStringLibrary.Concat_StrStr` "You got some " (`|GetEnumeratorNameAsString` (`self.Resource Type`)) "!"))))

(fn `GetPrompt`
  (returns (Prompt :type String))
  (return (`KismetStringLibrary.Concat_StrStr` "Acquire " (`|GetEnumeratorNameAsString` (`self.Resource Type`)))))

(fn `IsInteractable`
  (returns (IsInteractable :type Boolean))
  (return true))

(fn `UserConstructionScript`
  (if (`|EnumEquality` (`self.Resource Type`) "NewEnumerator0")
    (`KismetSystemLibrary.PrintString` "tset 3")
    (`self.Disable Other models`)
    (elif (`|EnumEquality` (`self.Resource Type`) "NewEnumerator1")
      (`self.Disable Other models`)
      (elif (`|EnumEquality` (`self.Resource Type`) "NewEnumerator2")
        (`self.Disable Other models`)
        (elif (`|EnumEquality` (`self.Resource Type`) "NewEnumerator3")
          (`self.Disable Other models`)
          (elif (`|EnumEquality` (`self.Resource Type`) "NewEnumerator4")
            (`self.Disable Other models`)))))))