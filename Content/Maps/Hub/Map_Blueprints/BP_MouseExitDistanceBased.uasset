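; Mouse hole exit actor that sends the player to Level2 when the first-person character walks into its trigger.
; The trigger overlap prints a debug message, fades the camera out, then opens the level after a matching delay.
; The construction script sets the hole's preview material from the PreviewTexture enum, though two options assign no material.
; Interaction functions are stubbed: Interact is empty and IsInteractable returns false.
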(event `self.Interact`)

(event `self.Trigger.OnComponentBeginOverlap`
  (params (OverlappedComponent :type "PrimitiveComponent Object Reference") (OtherActor :type "Actor Object Reference") (OtherComp :type "PrimitiveComponent Object Reference") (OtherBodyIndex :type Integer) (bFromSweep :type Boolean) (SweepResult :type "HitResult Structure (by ref)"))
  (`KismetSystemLibrary.PrintString` "Hello")
  (cast `/Game/FirstPerson/Blueprints/BP_FirstPersonCharacter` OtherActor)
  (`PlayerCameraManager.StartCameraFade` :`self` (`GameplayStatics.GetPlayerCameraManager` 0) :`ToAlpha` 1.0 :`Duration` 1.5)
  (`KismetSystemLibrary.Delay` 1.5)
  (`GameplayStatics.OpenLevel` "Level2"))

(fn `GetPrompt`
  (returns (Prompt :type String))
  (return "Exit"))

(fn `IsInteractable`
  (returns (IsInteractable :type Boolean))
  (return false))

(fn `UserConstructionScript`
  (if (`|EnumEquality` (`self.PreviewTexture`) "NewEnumerator1")
    (`PrimitiveComponent.SetMaterial` (`self.SM_MouseHole`) 0 null)
    (elif (`|EnumEquality` (`self.PreviewTexture`) "NewEnumerator2")
      (`PrimitiveComponent.SetMaterial` (`self.SM_MouseHole`) 0 null)
      (elif (`|EnumEquality` (`self.PreviewTexture`) "NewEnumerator3")
        (`PrimitiveComponent.SetMaterial` (`self.SM_MouseHole`) 0 "/Game/Maps/Hub/materials/Preview_Kitchen.Preview_Kitchen")
        (else
          (`PrimitiveComponent.SetMaterial` (`self.SM_MouseHole`) 0 "/Game/Maps/Hub/materials/Preview_Hub.Preview_Hub"))))))