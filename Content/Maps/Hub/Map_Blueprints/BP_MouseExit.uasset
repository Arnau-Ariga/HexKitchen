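; BP_MouseExit is an interactable mouse hole in the Hub map that serves as an exit to Level2.
; Its interaction functions always report it as usable with an "Exit" prompt.
; Interact fades the camera out, waits for the fade, then opens the hard-coded level by name.
; The construction script sets the mouse hole material from the PreviewTexture enum, with only the kitchen preview material assigned.
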(event `/Game/Blueprints/Interact/BPI_Interactable.Interact`
  (`PlayerCameraManager.StartCameraFade` :`self` (`GameplayStatics.GetPlayerCameraManager` 0) :`ToAlpha` 1.0 :`Duration` 1.5)
  (`KismetSystemLibrary.Delay` 1.5)
  (`GameplayStatics.OpenLevel` "Level2"))

(fn `GetPrompt`
  (returns (Prompt :type String))
  (return "Exit"))

(fn `IsInteractable`
  (returns (IsInteractable :type Boolean))
  (return true))

(fn `UserConstructionScript`
  (if (`|EnumEquality` (`self.PreviewTexture`) "NewEnumerator1")
    (`PrimitiveComponent.SetMaterial` (`self.SM_MouseHole`) 0 null)
    (elif (`|EnumEquality` (`self.PreviewTexture`) "NewEnumerator2")
      (`PrimitiveComponent.SetMaterial` (`self.SM_MouseHole`) 0 null)
      (elif (`|EnumEquality` (`self.PreviewTexture`) "NewEnumerator3")
        (`PrimitiveComponent.SetMaterial` (`self.SM_MouseHole`) 0 "/Game/Maps/Hub/materials/Preview_Kitchen.Preview_Kitchen")
        (else
          (`PrimitiveComponent.SetMaterial` (`self.SM_MouseHole`) 0 null))))))