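; BP_icyFloor is a Freezer level floor actor that makes the first-person player slide while inside its Box volume.
; BeginPlay caches the player's BP_FirstPersonCharacter.
; While the Icy flag is set, Box overlap begin zeroes that character's ground friction and walking braking deceleration.
; Overlap end restores fixed values rather than saved originals, and only if Icy is still true.
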(event `self.ReceiveBeginPlay`
  (bind _asbp_first_person_character (cast `/Game/FirstPerson/Blueprints/BP_FirstPersonCharacter` (`GameplayStatics.GetPlayerCharacter` 0)))
  (set `self.As BP First Person Character` _asbp_first_person_character))

(event `self.Box.OnComponentBeginOverlap`
  (params (OverlappedComponent :type "PrimitiveComponent Object Reference") (OtherActor :type "Actor Object Reference") (OtherComp :type "PrimitiveComponent Object Reference") (OtherBodyIndex :type Integer) (bFromSweep :type Boolean) (SweepResult :type "HitResult Structure (by ref)"))
  (bind _charactermovement (`Character.CharacterMovement` (`self.As BP First Person Character`)))
  (if (`self.Icy?`)
    (if (== OtherActor (`self.As BP First Person Character`))
      (set `CharacterMovementComponent.GroundFriction` 0.0 _charactermovement)
      (set `CharacterMovementComponent.BrakingDecelerationWalking` 0.0 _charactermovement))))

(event `self.Box.OnComponentEndOverlap`
  (params (OverlappedComponent :type "PrimitiveComponent Object Reference") (OtherActor :type "Actor Object Reference") (OtherComp :type "PrimitiveComponent Object Reference") (OtherBodyIndex :type Integer))
  (bind _charactermovement (`Character.CharacterMovement` (`self.As BP First Person Character`)))
  (if (`self.Icy?`)
    (if (== OtherActor (`self.As BP First Person Character`))
      (set `CharacterMovementComponent.GroundFriction` 2.0 _charactermovement)
      (set `CharacterMovementComponent.BrakingDecelerationWalking` 2048.0 _charactermovement))))

(fn `UserConstructionScript`)