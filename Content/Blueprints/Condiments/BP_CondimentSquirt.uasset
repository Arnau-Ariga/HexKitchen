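; BP_CondimentSquirt is a condiment splat actor that animates a cylinder mesh over its lifetime and then destroys itself.
; Each tick it spreads the cylinder wider and flatter up to a size cap, then after LifeSpan ticks shrinks its width until gone.
; A RayTrace function traces down past actors of ignored classes and snaps the splat to the hit surface, aligned to its normal.
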(event `self.ReceiveTick`
  (params (DeltaSeconds :type "Float (single-precision)"))
  (bind _cylinder1 (`self.Cylinder1`))
  (bind _cylinder1_2 (`self.Cylinder1`))
  (bind (_returnvalue_x _returnvalue_y _returnvalue_z) (`KismetMathLibrary.BreakVector` (`SceneComponent.K2_GetComponentScale` _cylinder1_2)))
  (bind (_returnvalue_x_2 _returnvalue_y_2 _returnvalue_z_2) (`KismetMathLibrary.BreakVector` (`SceneComponent.K2_GetComponentScale` _cylinder1)))
  (bind _returnvalue (* _returnvalue_x 1.05))
  (bind _returnvalue_2 (- _returnvalue_x_2 0.005))
  (bind _result (`/Engine/EditorBlueprintResources/StandardMacros.IncrementFloat` (`self.Timer`))
    (:`  `
      (if (< _result (`self.LifeSpan`))
        (if (< _returnvalue_x 2.0)
          (`SceneComponent.SetWorldScale3D` _cylinder1_2 (`KismetMathLibrary.MakeVector` _returnvalue _returnvalue (- _returnvalue_z 0.02))))
        (elif (>= _returnvalue_x_2 0.0)
          (`SceneComponent.SetWorldScale3D` _cylinder1 (`KismetMathLibrary.MakeVector` _returnvalue_2 _returnvalue_2 _returnvalue_z_2))
          (else
            (`self.K2_DestroyActor`)))))))

(fn `Ray Trace`
  (params (MyClass :type "Actor Class Reference"))
  (bind _returnvalue (`self.K2_GetActorLocation`))
  (bind _returnvalue_2 (+ _returnvalue (0.0 0.0 100.0)))
  (`self.AddToActorToIgnore` MyClass
    (:`Out`
      (`self.AddToActorToIgnore` null
        (:`Out`
          (`self.AddToActorToIgnore` null
            (:`Out`
              (bind _outhit (`KismetSystemLibrary.LineTraceSingle` _returnvalue_2 (- _returnvalue (0.0 0.0 500.0)) "TraceTypeQuery1" false (`self.ActorsToIgnore`)))
              (bind (_bblockinghit _binitialoverlap _time _distance _location _impactpoint _normal _impactnormal) (`GameplayStatics.BreakHitResult` _outhit))
              (if (!= _location _returnvalue_2)
                (`self.K2_SetActorLocationAndRotation` _location (`KismetMathLibrary.MakeRotFromZ` _impactnormal))))))))))

(fn `UserConstructionScript`)