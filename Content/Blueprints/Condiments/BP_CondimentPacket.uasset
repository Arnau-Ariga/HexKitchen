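; BP_CondimentPacket is a closed sauce packet that bursts into condiment puddles when the first-person character hits it after a long enough jump.
; SpawnCondiment checks the character's JumpTime, then uses the SouthHit overlap to choose which side to spray.
; Nested loops spawn the given condiment class in a randomly jittered, roughly circular grid beyond the packet.
; It then swaps itself for a BP_CondimentOpen, passing on direction and material.
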(event `self.ReceiveBeginPlay`)

(event `self.ReceiveActorBeginOverlap`
  (params (OtherActor :type "Actor Object Reference")))

(fn `SpawnCondiment`
  (params (CondimentClass :type "Actor Class Reference") (Material :type "MaterialInstance Object Reference") (HitOther :type "Actor Object Reference"))
  (locals (Condiment :type "Actor Class Reference") (CMaterial :type "MaterialInstance Object Reference"))
  (bind (_returnvalue_location _returnvalue_rotation _returnvalue_scale) (`KismetMathLibrary.BreakTransform` (`SceneComponent.K2_GetComponentToWorld` (`self.Sauce_packet_closed`))))
  (bind _returnvalue (+ (`self.SizeY * 2`) 200.0))
  (set `local.Condiment` CondimentClass)
  (set `local.CMaterial` Material)
  (set `self.HitOther` HitOther)
  ; Check If Enough Jump Force Was Applied
  (if (`GameplayStatics.ObjectIsA` HitOther "/Game/FirstPerson/Blueprints/BP_FirstPersonCharacter.BP_FirstPersonCharacter_C")
    (bind _asbp_first_person_character (cast `/Game/FirstPerson/Blueprints/BP_FirstPersonCharacter` HitOther))
    (if (> (`/Game/FirstPerson/Blueprints/BP_FirstPersonCharacter.JumpTime` _asbp_first_person_character) 0.6)
      (set `self.SizeY * 2` (* (.y (`.BoxExtent` (`self.GetActorBounds` false))) 2.0))
      (set `self.OverlappingSouth` (`PrimitiveComponent.IsOverlappingActor` (`self.SouthHit`) (`self.HitOther`)))
      (for _index (range -5 6)
        (bind _returnvalue_2 (- 4 (`KismetMathLibrary.Abs_Int` _index)))
        ; Spawn Multiple Puddles of Condiment
        (for _index_2 (range (- 0 _returnvalue_2) (+ _returnvalue_2 1))
          (if (`self.OverlappingSouth`)
            (bind _returnvalue_3 (`self.OffsetKetchup` _index))
            (set `self.Location Y` (+ _returnvalue_3 _returnvalue))
            (else
              (set `self.Location Y` (- _returnvalue_3 _returnvalue))))
          (`|SpawnActorFromClass` (`local.Condiment`) (`KismetMathLibrary.MakeTransform` (`KismetMathLibrary.TransformLocation` (`SceneComponent.K2_GetComponentToWorld` (`self.Sauce_packet_closed`)) (`KismetMathLibrary.MakeVector` (`self.OffsetKetchup` _index_2) (`self.Location Y`)))) "Undefined" "MultiplyWithRoot" null null)))
      (bind _returnvalue_4 (`|SpawnActorFromClass` "/Game/Blueprints/Condiments/BP_CondimentOpen.BP_CondimentOpen_C" (`KismetMathLibrary.MakeTransform` (+ _returnvalue_location (0.0 0.0 5.0)) _returnvalue_rotation _returnvalue_scale) "Undefined" "MultiplyWithRoot" null null))
      (`/Game/Blueprints/Condiments/BP_CondimentOpen.SetDirection` _returnvalue_4 (`self.OverlappingSouth`))
      (`/Game/Blueprints/Condiments/BP_CondimentOpen.SetMaterial` _returnvalue_4 (`local.CMaterial`))
      (`self.K2_DestroyActor`))))

(fn `UserConstructionScript`)