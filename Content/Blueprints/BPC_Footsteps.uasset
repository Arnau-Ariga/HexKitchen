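; Footstep component for the first-person player character that plays surface-based step and jump sounds.
; Raw WASD key events start a looping timer while walking on the ground, with Left Shift changing the step interval.
; Each step sphere-traces below the capsule and picks wood, tile or metal sound by surface type, defaulting to tile.
; Space triggers a similar trace for the jump-landing sound, and Tick watches the health component for death.
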(event `Key|W`
  (params (Key :type "Key Structure"))
  ; Checks if key is pressed to walk
  (:`Pressed`
    (set `self.WPressed` true)
    (`self.CheckWalk` :!label _label))
  (:`Released`
    (set `self.WPressed` false)
    (`KismetSystemLibrary.K2_ClearAndInvalidateTimerHandle` (`self.WalkTimer`) :!label _label_2)
    (goto _label)))

(event `Key|A`
  (params (Key :type "Key Structure"))
  ; Checks if key is pressed to walk
  (:`Pressed`
    (set `self.APressed` true)
    (goto _label))
  (:`Released`
    (set `self.APressed` false)
    (goto _label_2)))

(event `Key|S`
  (params (Key :type "Key Structure"))
  ; Checks if key is pressed to walk
  (:`Pressed`
    (set `self.SPressed` true)
    (goto _label))
  (:`Released`
    (set `self.SPressed` false)
    (goto _label_2)))

(event `Key|D`
  (params (Key :type "Key Structure"))
  ; Checks if key is pressed to walk
  (:`Pressed`
    (set `self.DPressed` true)
    (goto _label))
  (:`Released`
    (set `self.DPressed` false)
    (goto _label_2)))

(event `Key|LeftShift`
  (params (Key :type "Key Structure"))
  ; Checks if key is pressed to walk
  (:`Pressed`
    (set `self.RunSpeed` 0.25)
    (goto _label_2))
  (:`Released`
    (set `self.RunSpeed` 0.3)
    (goto _label_2)))

(event `CheckWalk`
  ; Checks is player is on ground before walking
  (bind _asbp_first_person_character (cast `/Game/FirstPerson/Blueprints/BP_FirstPersonCharacter` (`self.GetOwner`)))
  (bind _charactermovement (`Character.CharacterMovement` _asbp_first_person_character))
  (if (and (`NavMovementInterface.IsMovingOnGround` _charactermovement) (`CharacterMovementComponent.IsWalking` _charactermovement))
    (if (or (`self.WPressed`) (`self.APressed`) (`self.SPressed`) (`self.DPressed`))
      (`self.Walk`))))

(event `Walk`
  ; Plays walk sound if player is not dead
  (if (not (`self.IsPlayerDead`))
    (bind _returnvalue (`KismetSystemLibrary.K2_SetTimerDelegate` (delegate `FootTime`) (`self.RunSpeed`) true false -1.0))
    (set `self.WalkTimer` _returnvalue)))

(event `FootTime`
  ; Plays walk sound if player is not dead
  (`self.FootstepTrace`))

(event `Key|SpaceBar`
  (params (Key :type "Key Structure"))
  ; Checks is player trying to jump
  (:`Pressed`
    (bind _output_get (set `self.Cooldown` true))
    (if (or _output_get (`NavMovementComponent.IsMovingOnGround` (`Character.CharacterMovement` (`GameplayStatics.GetPlayerCharacter` 0))))
      (`self.JumpTrace`))))

(event `self.ReceiveTick`
  (params (DeltaSeconds :type "Float (single-precision)"))
  ; Checks is player dead (so walking doesn't keep playing)
  (bind _asbp_first_person_character (cast `/Game/FirstPerson/Blueprints/BP_FirstPersonCharacter` (`GameplayStatics.GetPlayerCharacter` 0)))
  (if (`/Game/UserInterface/Indicators/BPC_Health.IsDead` (`/Game/FirstPerson/Blueprints/BP_FirstPersonCharacter.BPC_Health` _asbp_first_person_character))
    (set `self.IsPlayerDead` true)))

(fn `FootstepTrace`
  (bind _returnvalue (`Actor.K2_GetActorLocation` (`self.GetOwner`)))
  (bind _capsulecomponent (`Character.CapsuleComponent` (`GameplayStatics.GetPlayerCharacter` 0)))
  (if (not (`self.Cooldown`))
    (bind (_outhit _returnvalue_2) (`KismetSystemLibrary.SphereTraceSingle` _returnvalue (`KismetMathLibrary.MakeVector` (.x _returnvalue) (.y _returnvalue) (- (.z _returnvalue) (`CapsuleComponent.GetScaledCapsuleHalfHeight` _capsulecomponent))) (`CapsuleComponent.GetScaledCapsuleRadius` _capsulecomponent) "TraceTypeQuery1"))
    (if _returnvalue_2
      (set `self.HitResultLocation` (`.Location` (`GameplayStatics.BreakHitResult` _outhit)))
      (switch `EPhysicalSurface` (`GameplayStatics.GetSurfaceType` _outhit)
        (:`SurfaceType_Default`
          (`GameplayStatics.PlaySoundAtLocation` "/Game/SFX/Cues/Footsteps/TileSteps_Cue.TileSteps_Cue" (`self.HitResultLocation`) (struct) 1.0 1.0 0.0 null null null null :!label _label))
        (:`SurfaceType1`
          (`GameplayStatics.PlaySoundAtLocation` "/Game/SFX/Cues/Footsteps/WoodSteps_Cue.WoodSteps_Cue" (`self.HitResultLocation`) (struct) 1.0 1.0 0.0 null null null null))
        (:`SurfaceType2`
          (goto _label))
        (:`SurfaceType3`
          (`GameplayStatics.PlaySoundAtLocation` "/Game/SFX/Cues/Footsteps/MetalSteps_Cue.MetalSteps_Cue" (`self.HitResultLocation`) (struct) 1.0 1.0 0.0 null null null null))))))

(fn `JumpTrace`
  (bind _returnvalue (`Actor.K2_GetActorLocation` (`self.GetOwner`)))
  (bind _capsulecomponent (`Character.CapsuleComponent` (`GameplayStatics.GetPlayerCharacter` 0)))
  (if (`self.Cooldown`)
    (bind (_outhit _returnvalue_2) (`KismetSystemLibrary.SphereTraceSingle` _returnvalue (`KismetMathLibrary.MakeVector` (.x _returnvalue) (.y _returnvalue) (- (.z _returnvalue) (`CapsuleComponent.GetScaledCapsuleHalfHeight` _capsulecomponent))) (`CapsuleComponent.GetScaledCapsuleRadius` _capsulecomponent) "TraceTypeQuery1"))
    (if _returnvalue_2
      (set `self.HitResultLocation` (`.Location` (`GameplayStatics.BreakHitResult` _outhit)))
      (`GameplayStatics.PlaySoundAtLocation` "/Game/SFX/Cues/JumpLand_Cue.JumpLand_Cue" (`self.HitResultLocation`) (struct) 1.0 1.0 0.0 null null null null)
      (set `self.Cooldown` false))))