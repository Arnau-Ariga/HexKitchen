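; Player stamina component that creates an on-screen stamina bar and updates it as stamina drains and regenerates.
; DecreaseStamina, meant to be bound to sprinting or jumping, drains stamina and turns any deficit into non-lethal damage through the owning BP_FirstPersonCharacter's health component.
; Tick regenerates stamina after a delay since the last drain, at a per-frame rate that rises with current health and ignores delta time.
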(event `self.ReceiveBeginPlay`
  (bind _returnvalue (`|CreateWidget` "/Game/Blueprints/W_StaminaBar.W_StaminaBar_C"))
  (bind _output_get (set `self.Widget` _returnvalue))
  (`UserWidget.AddToViewport` _output_get 0) ; Stamina Bar is viewable by Player.
  (bind _output_get_2 (set `self.MaxStamina` 100.0))
  (bind _output_get_3 (set `self.Stamina` _output_get_2))
  (`self.SetPercentBar` _output_get_3))

(event `DecreaseStamina`
  (params (StaminaDrainMult :type "Float (double-precision)"))
  (bind _bpc_health (`/Game/FirstPerson/Blueprints/BP_FirstPersonCharacter.BPC_Health` (cast `/Game/FirstPerson/Blueprints/BP_FirstPersonCharacter` (`self.GetOwner`) :!pure true)))
  ; USER NOTE: Bind this event to Player Sprinting/Jumping
  (bind _output_get (set `self.Stamina` (- (`self.Stamina`) (* StaminaDrainMult 0.04 1.0))))
  ; Drain Health if Stamina is Zero
  (bind _returnvalue (`KismetSystemLibrary.GetGameTimeInSeconds`))
  (set `self.Last Stamina Tick` _returnvalue)
  (bind _returnvalue_2 (* _output_get 0.25 -1.0))
  (if (and (<= _output_get 0.0) (< _returnvalue_2 (`/Game/Blueprints/BPC_Health.Health` _bpc_health)))
    (`/Game/Blueprints/BPC_Health.PlayerTakeDamage` _bpc_health null _returnvalue_2 null null null))
  (bind _output_get_2 (set `self.Stamina` (`KismetMathLibrary.FClamp` (`self.Stamina`) 0.0 (`self.MaxStamina`))))
  (`self.SetPercentBar` _output_get_2))

(event `self.ReceiveTick`
  (params (DeltaSeconds :type "Float (single-precision)"))
  ; Regenerate Stamina if player is not moving
  (bind _returnvalue (`KismetSystemLibrary.GetGameTimeInSeconds`))
  (if (>= (- _returnvalue (`self.Last Stamina Tick`)) 3.0)
    (bind _output_get (set `self.Stamina` (`KismetMathLibrary.FMin` (+ (`self.Stamina`) (* (+ (`/Game/Blueprints/BPC_Health.Health` (`/Game/FirstPerson/Blueprints/BP_FirstPersonCharacter.BPC_Health` (cast `/Game/FirstPerson/Blueprints/BP_FirstPersonCharacter` (`self.GetOwner`) :!pure true))) 20.0) 2.0 0.0015)) (`self.MaxStamina`))))
    (`self.SetPercentBar` _output_get)))

(fn `SetPercentBar`
  (params (InDouble :type "Float (double-precision)"))
  (`/Game/Blueprints/W_StaminaBar.SetPercentBar` (`self.Widget`) (`KismetStringLibrary.Conv_DoubleToString` (/ (`KismetMathLibrary.Conv_IntToDouble` (`KismetMathLibrary.Round` (* InDouble 100.0))) 100.0))))