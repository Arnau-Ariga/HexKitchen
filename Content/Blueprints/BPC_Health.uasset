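; Health component shared by the first-person player and enemies, binding a damage handler to whichever owner it has.
; Player damage is clamped, saved to the game instance and shown on a health bar widget, with a death menu at zero.
; Enemy damage is scaled when the attacker's damage type matches its weakness, triggering indicator particles and killing it at zero.
; Tick also calls Die on zero health or player falls; G applies test damage.
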(event `self.ReceiveBeginPlay`
  (bind _returnvalue (`self.GetOwner`))
  ; If player is damaged update health
  (bind _asbp_first_person_character (cast `/Game/FirstPerson/Blueprints/BP_FirstPersonCharacter` _returnvalue)
    (:`then`
      (set `self.IsPlayer` true)
      (add `Actor.OnTakeAnyDamage` _asbp_first_person_character (delegate `PlayerTakeDamage`))
      (bind _returnvalue_2 (`|CreateWidget` "/Game/UserInterface/Indicators/W_HealthBar.W_HealthBar_C"))
      (bind _output_get (set `self.WHealthBar` _returnvalue_2))
      (`UserWidget.AddToViewport` _output_get 0)
      (bind _output_get_2 (set `self.MaxHealth` (`/Game/FirstPerson/Blueprints/BP_FirstPersonCharacter.MaxHealth` _asbp_first_person_character)))
      (set `self.Health` _output_get_2)
      (bind _asw_health_bar (cast `/Game/Blueprints/W_HealthBar` (`self.WHealthBar`)))
      (bind _returnvalue_3 (`KismetStringLibrary.Conv_DoubleToString` _output_get_2))
      (`/Game/Blueprints/W_HealthBar.SetPercentBar` _asw_health_bar (`KismetStringLibrary.Concat_StrStr` _returnvalue_3 " / " _returnvalue_3)))
    (:`CastFailed`
      (cast `/Game/Enemies/AI_bases/BP_enemy_base` _returnvalue)
      (set `self.IsPlayer` false)
      (add `Actor.OnTakeAnyDamage` _returnvalue (delegate `EnemyTakeDamage`))
      (`self.SetMaxHealth` 40.0))))

(event `PlayerTakeDamage`
  (params (DamagedActor :type "Actor Object Reference") (Damage :type "Float (single-precision)") (DamageType :type "DamageType Object Reference") (InstigatedBy :type "Controller Object Reference") (DamageCauser :type "Actor Object Reference"))
  ; If player is damaged update health
  (set `self.Health` (`KismetMathLibrary.FClamp` (- (`self.Health`) Damage) 0.0 (`self.MaxHealth`)))
  (bind _asgame_instance_colson (cast `/Game/UserInterface/GameInstanceColson` (`GameplayStatics.GetGameInstance`)))
  (set `/Game/UserInterface/GameInstanceColson.health` (`self.Health`) _asgame_instance_colson)
  (if (`self.IsPlayer`)
    (bind _asw_health_bar (cast `/Game/Blueprints/W_HealthBar` (`self.WHealthBar`)))
    (`/Game/Blueprints/W_HealthBar.SetPercentBar` _asw_health_bar (`KismetStringLibrary.Concat_StrStr` (`KismetStringLibrary.Conv_DoubleToString` (`self.Health`)) " / " (`KismetStringLibrary.Conv_DoubleToString` (`self.MaxHealth`))))
    (`GameplayStatics.PlaySound2D` "/Game/SFX/Cues/Damage_Cue.Damage_Cue" 1.0 1.0 0.0 null null)
    (if (<= (`self.Health`) 0.0)
      (`self.Die`))))

(event `EnemyTakeDamage`
  (params (DamagedActor :type "Actor Object Reference") (Damage :type "Float (single-precision)") (DamageType :type "DamageType Object Reference") (InstigatedBy :type "Controller Object Reference") (DamageCauser :type "Actor Object Reference"))
  ; If player is damaged update health
  (bind _a (`self.Compare Damage Types` 2.0 DamageCauser))
  (bind _output_get (set `self.Health` (- (`self.Health`) (* _a Damage))))
  (bind _asbp_enemy_base (cast `/Game/Enemies/AI_bases/BP_enemy_base` (`self.GetOwner`)))
  (if (> _a 1.0)
    (`self.Activate` (`/Game/Enemies/AI_bases/BP_enemy_base.AttackIndicatorParticles` _asbp_enemy_base) true)
    (else
      (`self.Activate` (`/Game/Enemies/AI_bases/BP_enemy_base.CritAttackIndicator` _asbp_enemy_base) true)))
  (if (<= _output_get 0.0)
    (set `self.IsDead` true)
    (`/Game/Enemies/AI_bases/BP_enemy_base.kill` _asbp_enemy_base)))

(event `Die`
  (bind _returnvalue (`GameplayStatics.GetPlayerController` 0))
  ; If the player dies call this function
  (if (not (`self.IsDead`))
    (set `self.IsDead` true)
    (if (`self.IsPlayer`)
      (bind _returnvalue_2 (`|CreateWidget` "/Game/UserInterface/W_DeathMenu.W_DeathMenu_C"))
      (`UserWidget.AddToViewport` _returnvalue_2 0)
      (set `PlayerController.bShowMouseCursor` true _returnvalue)
      (`Actor.DisableInput` (`GameplayStatics.GetPlayerCharacter` 0) _returnvalue)
      (`GameplayStatics.PlaySound2D` "/Game/SFX/WompWomp.WompWomp" 1.0 1.0 0.0 null null)
      (else
        (`Actor.K2_DestroyActor` (`self.GetOwner`))))))

(event `self.ReceiveTick`
  (params (DeltaSeconds :type "Float (single-precision)"))
  ; Checks if player fell off map
  (if (or (> -100.0 (.z (`Actor.K2_GetActorLocation` (`GameplayStatics.GetPlayerCharacter` 0)))) (<= (`self.Health`) 0.0))
    (`self.Die`)))

(event `Key|G`
  (params (Key :type "Key Structure"))
  ; Test Damage
  (:`Pressed`
    (`GameplayStatics.ApplyDamage` (`self.GetOwner`) 10.0)))

(fn `Compare Damage Types`
  (params (`Matching Type Mult` :type "Float (double-precision)") (`Damage Causer` :type "Actor Object Reference"))
  (returns (A :type "Float (double-precision)"))
  (locals (Mult :type "Float (double-precision)"))
  (set `local.Mult` `Matching Type Mult`)
  (bind _asbp_first_person_character (cast `/Game/FirstPerson/Blueprints/BP_FirstPersonCharacter` `Damage Causer`)
    (:`then`
      (bind _damage_type (`/Game/FirstPerson/Blueprints/BP_FirstPersonCharacter.Damage Type` _asbp_first_person_character))
      (return (select `bool` (and (`|EnumInequality` _damage_type "NewEnumerator3") (`|EnumEquality` _damage_type (`self.Weakness`))) :`false` 1.0 :`true` (`local.Mult`))))
    (:`CastFailed`
      (return 1.0))))

(fn `DamageTypeFunction`
  (params (Object :type "Object Object Reference"))
  (returns (DamageType :type Byte))
  (if (`GameplayStatics.ObjectIsA` Object)
    (return 0)
    (elif (`GameplayStatics.ObjectIsA` Object)
      (return 0)
      (elif (`GameplayStatics.ObjectIsA` Object)
        (return 0)
        (else
          (return 0))))))

(fn `Initiate`
  (params (MaxHealth :type "Float (double-precision)") (Weakness :type "/Game/Items/Weapons/Enum_DamageType Enum" :default "NewEnumerator3"))
  (bind _output_get (set `self.MaxHealth` MaxHealth))
  (set `self.Health` _output_get)
  (set `self.Weakness` Weakness))

(fn `SetMaxHealth`
  (params (`Max Health` :type "Float (double-precision)"))
  (bind _output_get (set `self.MaxHealth` `Max Health`))
  (set `self.Health` _output_get))