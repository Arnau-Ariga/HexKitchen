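; BPC_CreepyAmbience is a component that plays a creepy ambience cue at the player's location at random intervals.
; CreepyEvent loops by calling itself after a random delay, skipping the sound and waiting longer while IsEnemyNear is set.
; Tick scans every BP_enemy_walker and sets that flag when one is over 50 units from the owner on all three axes, despite its name.
; The flag is never cleared.
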(event `self.ReceiveBeginPlay`
  (`self.CreepyEvent`))

(event `self.ReceiveTick`
  (params (DeltaSeconds :type "Float (single-precision)"))
  (bind _outactors (`GameplayStatics.GetAllActorsOfClass` "/Game/Enemies/AI_bases/BP_enemy_walker.BP_enemy_walker_C"))
  (for _array_element _outactors
    (if (not (or (<= (`KismetMathLibrary.Abs` (.x (- (`Actor.K2_GetActorLocation` _array_element) (`Actor.K2_GetActorLocation` (`self.GetOwner`))))) 50.0) (<= (`KismetMathLibrary.Abs` (.y (- (`Actor.K2_GetActorLocation` _array_element) (`Actor.K2_GetActorLocation` (`self.GetOwner`))))) 50.0) (<= (`KismetMathLibrary.Abs` (.z (- (`Actor.K2_GetActorLocation` _array_element) (`Actor.K2_GetActorLocation` (`self.GetOwner`))))) 50.0)))
      (set `self.IsEnemyNear` true))))

(event `CreepyEvent`
  (`KismetSystemLibrary.Delay` (* (`KismetMathLibrary.RandomFloat`) 50.0))
  (if (`self.IsEnemyNear`)
    (set `self.IsEnemyNear` true)
    (`KismetSystemLibrary.Delay` 5.0)
    (else
      (`GameplayStatics.PlaySoundAtLocation` "/Game/SFX/Cues/Ambience/CreepyAmbience_Cue.CreepyAmbience_Cue" (`Actor.K2_GetActorLocation` (`GameplayStatics.GetPlayerCharacter` 0)) (struct) 1.0 1.0 0.0 null null null null)))
  (`self.CreepyEvent`))