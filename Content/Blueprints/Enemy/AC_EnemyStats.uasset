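; AC_EnemyStats is an enemy stats component that tracks health and handles incoming typed damage.
; Health starts at MaxHealth on BeginPlay, and TakeDamage subtracts damage scaled by CompareDamageTypes.
; At zero health it flags death and destroys the owning actor, otherwise it prints a debug hit message.
; CompareDamageTypes holds weakness-based double-damage logic, but those nodes are left unused.
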(event `self.ReceiveBeginPlay`
  (set `self.Health` (`self.MaxHealth`)))

(event `Event Take Damage`
  (params (Damage :type "Float (double-precision)") (Type :type "/Game/Enemy/E_DamageType Enum" :default "NewEnumerator0"))
  (bind _output_get (set `self.Health` (- (`self.Health`) (* Damage (select `bool` (and (!= Type 0) (== Type (`KismetSystemLibrary.MakeLiteralByte` (`self.Weakness`)))) :`false` 1.0 :`true` 2.0)))))
  (if (<= _output_get 0.0)
    (set `self.Is Dead` true)
    (`Actor.K2_DestroyActor` (`self.GetOwner`)) ; If the enemy is dead then delete it from the world
    (else
      (`KismetSystemLibrary.PrintString` (`KismetStringLibrary.Concat_StrStr` "@AC_EnemyStats hit " (`|GetEnumeratorNameAsString` Type))))))

(fn `Get Health`
  (returns (Health :type "Float (double-precision)"))
  (return (`self.Health`)))