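; BP_Mine is a mine that explodes when any Character overlaps its Box component.
; It launches that Character upward and opposite to player 0's horizontal velocity, scaled up, regardless of which Character triggered it.
; It then applies fixed damage, sets IsExploded, spawns a Niagara explosion with sound and destroys itself.
; The PlayerExploded function is an empty stub.
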(event `self.Box.OnComponentBeginOverlap`
  (params (OverlappedComponent :type "PrimitiveComponent Object Reference") (OtherActor :type "Actor Object Reference") (OtherComp :type "PrimitiveComponent Object Reference") (OtherBodyIndex :type Integer) (bFromSweep :type Boolean) (SweepResult :type "HitResult Structure (by ref)"))
  (bind _returnvalue (`self.K2_GetActorLocation`))
  (bind _output_get (set `self.Explosion` (`KismetMathLibrary.MakeVector` (.x (`self.GetVelocity` (`GameplayStatics.GetPlayerCharacter` 0))) (.y (`self.GetVelocity` (`GameplayStatics.GetPlayerCharacter` 0))) 1000.0)))
  (bind _ascharacter (cast `Character` OtherActor))
  (`Character.LaunchCharacter` _ascharacter (* _output_get (-3.0 -3.0 1.0)) false false)
  (`GameplayStatics.ApplyDamage` _ascharacter 25.0)
  (set `self.IsExploded` true)
  (`NiagaraFunctionLibrary.SpawnSystemAtLocation` "/Game/VFX/NS_Explosion.NS_Explosion" _returnvalue)
  (`GameplayStatics.PlaySoundAtLocation` "/Game/SFX/Cues/Explode_Cue.Explode_Cue" _returnvalue (struct) 1.0 1.0 0.0 null null null null)
  (`self.K2_DestroyActor`))

(fn `PlayerExploded`)

(fn `UserConstructionScript`)