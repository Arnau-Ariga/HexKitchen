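; BPC_Armor is an actor component that works out the player's armor value from equipped chestplate and leggings.
; On BeginPlay it logs an error if its owner is not BP_FirstPersonCharacter.
; GetPlayerArmor takes an inventory component, looks up the item names in the fixed chestplate and leggings slots against a hard-coded map of cloth, leather and metal values, and returns their sum.
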(event `self.ReceiveBeginPlay`
  (bind _asbp_first_person_character (cast `/Game/FirstPerson/Blueprints/BP_FirstPersonCharacter` (`self.GetOwner`))
    (:`CastFailed`
      (`KismetSystemLibrary.LogString` "[BPC_Armor]: This component MUST be attached to Player. User MUST NOT attach this component to another component."))))

(fn `GetPlayerArmor`
  (params (InventoryComponent :type "/Game/FirstPerson/Blueprints/InventoryComponent Object Reference"))
  (returns (Armor :type "Float (double-precision)"))
  (locals (NewLocalVar :type "Map of String to Float (single-precision)"))
  (bind _inventory_slots (`/Game/FirstPerson/Blueprints/InventoryComponent.Inventory Slots` InventoryComponent))
  (bind _output_name (break `/Game/UserInterface/Inventory_Structure` (`|GetArrayItem` _inventory_slots 9)))
  (bind _output_name_2 (break `/Game/UserInterface/Inventory_Structure` (`|GetArrayItem` _inventory_slots 8)))
  (bind _output_get (set `local.NewLocalVar` (`|MakeMap` "ClothChestplate" 0.06 "LeatherChestplate" 0.18 "MetalChestplate" 0.3 "ClothLeggings" 0.04 "LeatherLeggings" 0.12 "MetalLeggings" 0.2 :!valuetype "Float (single-precision)")))
  (bind (_value _returnvalue) (`BlueprintMapLibrary.Map_Find` _output_get _output_name_2))
  (bind (_value_2 _returnvalue_2) (`BlueprintMapLibrary.Map_Find` _output_get _output_name))
  (return (+ (select `bool` _returnvalue :`true` _value) (select `bool` _returnvalue_2 :`true` _value_2))))