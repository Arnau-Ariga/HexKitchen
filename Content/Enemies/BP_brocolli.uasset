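; Broccoli enemy that chases the player and, within range, stops to rain projectiles down from above them.
; Tick runs a shooting timer that gates both the range check and firing, spacing shots into fixed-count barrages separated by a cooldown scaled by AttackSpeed.
; Each shot spawns a downward-pitched projectile at a random offset over the player with random speed and a sound.
; Each barrage's first shot also briefly activates a Niagara effect.
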(event `self.ReceiveBeginPlay`
  (`parent.ReceiveBeginPlay`)
  (set `self.ShootingTimer` 0.0)
  (set `self.attackSpeed` 1.0))

(event `self.ReceiveTick`
  (params (DeltaSeconds :type "Float (single-precision)"))
  (`parent.ReceiveTick` DeltaSeconds)
  (if (<= (`self.ShootingTimer`) 0.0)
    (if (<= (`KismetMathLibrary.Vector_Distance` (`self.K2_GetActorLocation` (`GameplayStatics.GetPlayerPawn` 0)) (`self.K2_GetActorLocation` self)) 1000.0)
      (`self.stop`)
      (set `self.ShootingTimer` (+ (`self.ShootingTimer`) 0.1))
      (set `self.RainAmount` (+ (`self.RainAmount`) 1))
      (`|ExecutionSequence`
        (:`then_0`
          ; Start Barrage
          (if (>= (`self.RainAmount`) 20)
            (set `self.RainAmount` 0)
            (set `self.ShootingTimer` (+ (`self.ShootingTimer`) (/ 3.0 (`self.attackSpeed`))))
            (elif (== (`self.RainAmount`) 1)
              (`ActorComponent.Activate` (`self.Niagara`) false)
              (`GameplayStatics.PlaySoundAtLocation` "/Game/SFX/Cues/Enemies+Characters/Broccoli_Cue.Broccoli_Cue" (`self.K2_GetActorLocation`) (struct) 1.0 1.0 0.0 null null null null)
              (`KismetSystemLibrary.Delay` 2.0)
              (`ActorComponent.Deactivate` (`self.Niagara`)))))
        (:`then_1`
          ; Fire Bullet
          (set `self.RandAng` (`KismetMathLibrary.Conv_Int64ToDouble` (`KismetMathLibrary.RandomInteger64InRange` 0 360)))
          (set `self.RandDist` (`KismetMathLibrary.Conv_Int64ToDouble` (`KismetMathLibrary.RandomInteger64InRange` 0 300)))
          (bind _returnvalue (`|SpawnActorFromClass` "/Game/Enemies/Enemy_Projectiles/Projectile.Projectile_C" (`KismetMathLibrary.MakeTransform` (`KismetMathLibrary.MakeVector` (+ (* (`KismetMathLibrary.DegCos` (`self.RandAng`)) (`self.RandDist`)) (.x (`SceneComponent.K2_GetComponentLocation` (`Actor.RootComponent` (`GameplayStatics.GetPlayerPawn` 0))))) (+ (* (`KismetMathLibrary.DegSin` (`self.RandAng`)) (`self.RandDist`)) (.y (`SceneComponent.K2_GetComponentLocation` (`Actor.RootComponent` (`GameplayStatics.GetPlayerPawn` 0))))) (+ (.z (`SceneComponent.K2_GetComponentLocation` (`Actor.RootComponent` (`GameplayStatics.GetPlayerPawn` 0)))) 1000.0)) (`KismetMathLibrary.MakeRotator` 0.0 -90.0) (.scale (`self.GetTransform`))) "Undefined" "MultiplyWithRoot" null (`KismetMathLibrary.Conv_Int64ToDouble` (`KismetMathLibrary.RandomInteger64InRange` 1000 2000)) (`self.K2_GetActorRotation` self) null))
          (`GameplayStatics.PlaySoundAtLocation` "/Game/SFX/Cues/Enemies+Characters/Broccoli_Cue.Broccoli_Cue" (`self.K2_GetActorLocation` _returnvalue) (struct) 1.0 1.0 0.0 null null null null)))
      (else
        (set `self.AIActive` true)
        (set `self.seeingPlayer` true)
        (`self.chase`)))
    (else
      (set `self.ShootingTimer` (- (`self.ShootingTimer`) DeltaSeconds)))))

(fn `UserConstructionScript`
  (`parent.UserConstructionScript`))