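; Ghost pepper enemy that starts attacking once the player comes within range, then circles and shoots at them.
; While attacking, Tick places it on an orbit relative to the player's yaw, advancing the angle over time and turning it toward the player.
; It fires rapid projectiles after an initial delay, only while a camera line trace hits it and the player roughly faces it.
; BeginPlay also sets its health component's weakness.
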(event `self.ReceiveBeginPlay`
  (`parent.ReceiveBeginPlay`)
  (set `self.ShootingTimer` 0.0)
  (set `self.attackSpeed` 1.0)
  (set `self.ChargeDistance` 9999.0)
  (set `/Game/Blueprints/BPC_Health.Weakness` "NewEnumerator0" (`self.BPC_Health`)))

(event `self.ReceiveTick`
  (params (DeltaSeconds :type "Float (single-precision)"))
  (bind _returnvalue (`GameplayStatics.GetPlayerCharacter` 0))
  (bind _returnvalue_2 (+ (.yaw (`self.K2_GetActorRotation` _returnvalue)) (`self.ang`)))
  (bind _returnvalue_3 (`KismetMathLibrary.Abs_Int` (`KismetMathLibrary.FTrunc` (- (mod (`KismetMathLibrary.FTrunc` (+ (.yaw (`self.K2_GetActorRotation` (`GameplayStatics.GetPlayerPawn` 0))) 180.0)) 360) (mod (+ (`KismetMathLibrary.FTrunc` (`KismetMathLibrary.DegAtan2` (- (.y (`self.K2_GetActorLocation` (`GameplayStatics.GetPlayerCharacter` 0))) (.y (`self.K2_GetActorLocation`))) (- (.x (`self.K2_GetActorLocation` (`GameplayStatics.GetPlayerCharacter` 0))) (.x (`self.K2_GetActorLocation`))))) 360) 360)))))
  (`parent.ReceiveTick` DeltaSeconds)
  (set `self.Delta Seconds` DeltaSeconds)
  (if (`self.Attacking`)
    (`|ExecutionSequence`
      (:`then_0`
        (if (<= (`self.ShootingTimer`) 0.0)
          (bind _isonscreen (`self.isOnScreenByTraces`))
          (`KismetSystemLibrary.PrintString` (`KismetStringLibrary.Conv_BoolToString` _isonscreen))
          (if _isonscreen
            (if (< (`KismetMathLibrary.Min` _returnvalue_3 (- 360 _returnvalue_3)) 40)
              (set `self.ShootingTimer` 0.1)
              (bind _returnvalue_4 (`|SpawnActorFromClass` "/Game/Enemies/Enemy_Projectiles/Projectile.Projectile_C" (`KismetMathLibrary.MakeTransform` (`SceneComponent.K2_GetComponentLocation` (`self.Shoot`)) (`SceneComponent.K2_GetComponentRotation` (`self.Shoot`)) (.scale (`self.GetTransform`))) "Undefined" "MultiplyWithRoot" null 1000.0 (`self.K2_GetActorRotation` self) null))
              (`GameplayStatics.PlaySoundAtLocation` "/Game/SFX/Cues/Enemies+Characters/BigProjectile_Cue.BigProjectile_Cue" (`self.K2_GetActorLocation` _returnvalue_4) (struct) 1.0 1.0 0.0 null null null null)))
          (else
            (set `self.ShootingTimer` (- (`self.ShootingTimer`) DeltaSeconds)))))
      (:`then_1`
        (`self.K2_SetActorLocationAndRotation` (`KismetMathLibrary.MakeVector` (+ (.x (`self.K2_GetActorLocation` _returnvalue)) (* 700.0 (`KismetMathLibrary.DegCos` _returnvalue_2))) (+ (.y (`self.K2_GetActorLocation` _returnvalue)) (* 700.0 (`KismetMathLibrary.DegSin` _returnvalue_2))) (.z (`self.K2_GetActorLocation` _returnvalue))) (`KismetMathLibrary.MakeRotator` 0.0 0.0 (`KismetMathLibrary.DegAtan2` (- (.y (`self.K2_GetActorLocation` (`GameplayStatics.GetPlayerCharacter` 0))) (.y (`self.K2_GetActorLocation`))) (- (.x (`self.K2_GetActorLocation` (`GameplayStatics.GetPlayerCharacter` 0))) (.x (`self.K2_GetActorLocation`))))))
        (set `self.ang` (+ (`self.ang`) (* 90.0 (`self.Delta Seconds`))))))
    (elif (<= (`KismetMathLibrary.Vector_Distance` (`self.K2_GetActorLocation` (`GameplayStatics.GetPlayerPawn` 0)) (`self.K2_GetActorLocation` self)) 500.0)
      (set `self.Attacking` true)
      (set `self.ShootingTimer` 2.0))))

(fn `isOnScreenByTraces`
  (returns (isOnScreen :type Boolean))
  (bind _outhit (`KismetSystemLibrary.LineTraceSingle` (`PlayerCameraManager.GetCameraLocation` (`PlayerController.PlayerCameraManager` (`GameplayStatics.GetPlayerController` 0))) (`self.K2_GetActorLocation`) "TraceTypeQuery2" false (`|MakeArray` (`GameplayStatics.GetPlayerPawn` 0) :!type "Actor Object Reference") "None" false))
  (return (== (`.HitActor` (`GameplayStatics.BreakHitResult` _outhit)) self)))

(fn `UserConstructionScript`
  (`parent.UserConstructionScript`))