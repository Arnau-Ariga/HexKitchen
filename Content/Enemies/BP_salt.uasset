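; Salt enemy that acts as a support unit, buffing nearby enemies' attack speed when close to the player.
; When its cooldown is up, Tick either chases a distant player or stops within range and restarts the cooldown.
; Each pulse scans all BP_enemy_base actors, permanently raising AttackSpeed on non-salt ones in radius.
; Buff particles use a Delay inside the loop, so deactivation does not run per enemy.
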(event `self.ReceiveBeginPlay`
  (`parent.ReceiveBeginPlay`)
  (set `self.ShootingTimer` 0.0)
  (set `self.isSalt` true))

(event `self.ReceiveTick`
  (params (DeltaSeconds :type "Float (single-precision)"))
  (`parent.ReceiveTick` DeltaSeconds)
  (if (<= (`self.ShootingTimer`) 0.0)
    (if (<= (`KismetMathLibrary.Vector_Distance` (`self.K2_GetActorLocation` (`GameplayStatics.GetPlayerPawn` 0)) (`self.K2_GetActorLocation` self)) 400.0)
      (`self.stop`)
      (set `self.ShootingTimer` (+ (`self.ShootingTimer`) 5.0))
      (`|ExecutionSequence`
        (:`then_0`
          (bind _outactors (`GameplayStatics.GetAllActorsOfClass` "/Game/Enemies/AI_bases/BP_enemy_base.BP_enemy_base_C"))
          (for _array_element _outactors
            (if (`/Game/Enemies/AI_bases/BP_enemy_base.isSalt` _array_element)
              _
              (elif (<= (`KismetMathLibrary.Vector_Distance` (`SceneComponent.K2_GetComponentLocation` (`Character.Mesh` _array_element)) (`SceneComponent.K2_GetComponentLocation` (`self.Mesh`))) 400.0)
                (set `/Game/Enemies/AI_bases/BP_enemy_base.attackSpeed` (+ (`/Game/Enemies/AI_bases/BP_enemy_base.attackSpeed` _array_element) 1.0) _array_element)
                (bind _buffparticle (`/Game/Enemies/AI_bases/BP_enemy_base.BuffParticle` _array_element))
                (`ActorComponent.Activate` _buffparticle false)
                (`KismetSystemLibrary.Delay` 1.0)
                (`ActorComponent.Deactivate` _buffparticle)))))
        (:`then_1`
          (`ActorComponent.Activate` (`self.buffCircle`) false)
          (`KismetSystemLibrary.Delay` 1.0)
          (`ActorComponent.Deactivate` (`self.buffCircle`))))
      (else
        (set `self.AIActive` true)
        (set `self.seeingPlayer` true)
        (`self.chase`)))
    (else
      (set `self.ShootingTimer` (- (`self.ShootingTimer`) DeltaSeconds)))))

(fn `UserConstructionScript`
  (`parent.UserConstructionScript`))