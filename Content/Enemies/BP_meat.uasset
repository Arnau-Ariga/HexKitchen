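; Enemy character that chases the player and performs a leaping ground-slam attack, building on a parent enemy Blueprint's chase logic.
; Tick runs a cooldown timer, then either resumes the chase or, at close range, boosts walk speed, moves toward the player and launches itself upward.
; Box overlaps during the descent damage and stun the player once per slam.
; Landing halts movement, plays impact effects and re-arms the hit after a delay.
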(event `self.ReceiveBeginPlay`
  (`parent.ReceiveBeginPlay`)
  (set `self.ShootingTimer` 0.0)
  (set `self.Slamming` false)
  (set `self.DefaultWalkSpeed` (`CharacterMovementComponent.MaxWalkSpeed` (`self.CharacterMovement`)))
  (set `self.attackSpeed` 1.0)
  (set `/Game/Blueprints/BPC_Health.Weakness` "NewEnumerator0" (`self.BPC_Health`))
  (add `PrimitiveComponent.OnComponentBeginOverlap` (`self.Box`) (delegate `OnComponentBeginOverlap_Event`)))

(event `OnComponentBeginOverlap_Event`
  (params (OverlappedComponent :type "PrimitiveComponent Object Reference") (OtherActor :type "Actor Object Reference") (OtherComp :type "PrimitiveComponent Object Reference") (OtherBodyIndex :type Integer) (bFromSweep :type Boolean) (SweepResult :type "HitResult Structure (by ref)"))
  (bind (_returnvalue_x _returnvalue_y _returnvalue_z) (`KismetMathLibrary.BreakVector` (`CharacterMovementComponent.GetLastUpdateVelocity` (`self.CharacterMovement`))))
  (bind _asbp_first_person_character (cast `/Game/FirstPerson/Blueprints/BP_FirstPersonCharacter` OtherActor))
  (if (and (`self.Slamming`) (not (`self.Attacked`)) (< _returnvalue_z 0.0))
    (`GameplayStatics.ApplyDamage` _asbp_first_person_character 3.0 null self)
    (set `/Game/FirstPerson/Blueprints/BP_FirstPersonCharacter.StunTimerSec` 2.0 _asbp_first_person_character)
    (set `self.Attacked` true)))

(event `self.ReceiveTick`
  (params (DeltaSeconds :type "Float (single-precision)"))
  (`parent.ReceiveTick` DeltaSeconds)
  (if (<= (`self.ShootingTimer`) 0.0)
    (if (<= (`KismetMathLibrary.Vector_Distance` (`self.K2_GetActorLocation` (`GameplayStatics.GetPlayerPawn` 0)) (`self.K2_GetActorLocation` self)) 500.0)
      (`self.stop`)
      (set `CharacterMovementComponent.MaxWalkSpeed` (* (`self.DefaultWalkSpeed`) (/ 5.0 (`self.attackSpeed`))) (`self.CharacterMovement`))
      (set `self.ShootingTimer` (+ (`self.ShootingTimer`) 3.0))
      (`|AIMoveTo` self (0.0 0.0 0.0) (`GameplayStatics.GetPlayerPawn` 0)
        (:`then`
          ; Jump Start
          (`KismetSystemLibrary.Delay` 0.1)
          (`self.LaunchCharacter` (0.0 0.0 1000.0))
          (set `self.Slamming` true)))
      (elif (not (`self.AIActive`))
        (set `CharacterMovementComponent.MaxWalkSpeed` (`self.DefaultWalkSpeed`) (`self.CharacterMovement`))
        (set `self.AIActive` true)
        (set `self.seeingPlayer` true)
        (`self.chase`)))
    (else
      (set `self.ShootingTimer` (- (`self.ShootingTimer`) DeltaSeconds)))))

(event `self.OnLanded`
  (params (Hit :type "HitResult Structure (by ref)"))
  ; Jump End
  (if (`self.Slamming`)
    (`MovementComponent.StopMovementImmediately` (`self.CharacterMovement`))
    (set `self.Slamming` false)
    (`ActorComponent.Activate` (`self.GroundPound`) false)
    (`GameplayStatics.PlaySoundAtLocation` "/Game/SFX/Cues/Enemies+Characters/EnemyAttack_Cue.EnemyAttack_Cue" (`self.K2_GetActorLocation`) (struct) 1.0 1.0 0.0 null null null null)
    (`KismetSystemLibrary.Delay` 1.0)
    (`ActorComponent.Deactivate` (`self.GroundPound`))
    (set `self.Attacked` false)))

(fn `UserConstructionScript`
  (`parent.UserConstructionScript`))