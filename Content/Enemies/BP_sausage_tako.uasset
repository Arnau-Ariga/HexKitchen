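; Sausage octopus enemy that chases the player and performs a spinning projectile attack at close range.
; Tick calls Chase until the player is within range, then calls Stop and sets a timer scaled by AttackSpeed.
; While that timer is high, SpinAttack rapidly rotates the capsule and repeatedly spawns projectiles from the Shoot component.
; The rest of the countdown serves as a cooldown before it re-checks distance.
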(event `self.ReceiveBeginPlay`
  (`parent.ReceiveBeginPlay`)
  (set `self.ShootingTimer` 0.0)
  (set `self.attackSpeed` 1.0))

(event `self.ReceiveTick`
  (params (DeltaSeconds :type "Float (single-precision)"))
  (`parent.ReceiveTick` DeltaSeconds)
  (set `self.DS` DeltaSeconds)
  (`self.SpinAttack`)
  (if (<= (`self.ShootingTimer`) 0.0)
    (if (<= (`KismetMathLibrary.Vector_Distance` (`self.K2_GetActorLocation` (`GameplayStatics.GetPlayerPawn` 0)) (`self.K2_GetActorLocation` self)) 500.0)
      (set `self.ShootingTimer` (+ (+ (`self.ShootingTimer`) (/ 3.0 (`self.attackSpeed`))) 2.0))
      (`self.stop`)
      (else
        (set `self.AIActive` true)
        (set `self.seeingPlayer` true)
        (`self.chase`)))
    (else
      (set `self.ShootingTimer` (- (`self.ShootingTimer`) DeltaSeconds)))))

(event `SpinAttack`
  (bind _capsulecomponent (`self.CapsuleComponent`))
  (if (>= (`self.ShootingTimer`) 3.0)
    (`|ExecutionSequence`
      (:`then_0`
        (if (< (`self.AttackDelay`) 0.0)
          (set `self.AttackDelay` 0.1)
          (`|SpawnActorFromClass` "/Game/Enemies/Enemy_Projectiles/Projectile.Projectile_C" (`KismetMathLibrary.MakeTransform` (`SceneComponent.K2_GetComponentLocation` (`self.Shoot`)) (`SceneComponent.K2_GetComponentRotation` (`self.Shoot`)) (.scale (`self.GetTransform`))) "Undefined" "MultiplyWithRoot" null 1000.0 (`self.K2_GetActorRotation` self) null)
          (else
            (set `self.AttackDelay` (- (`self.AttackDelay`) (`self.DS`))))))
      (:`then_1`
        (`SceneComponent.K2_SetWorldRotation` _capsulecomponent (`KismetMathLibrary.MakeRotator` (.roll (`SceneComponent.K2_GetComponentRotation` _capsulecomponent)) (.pitch (`SceneComponent.K2_GetComponentRotation` _capsulecomponent)) (+ (.yaw (`SceneComponent.K2_GetComponentRotation` _capsulecomponent)) (* 720.0 (`self.DS`)))) false false)))))

(fn `UserConstructionScript`
  (`parent.UserConstructionScript`))