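; Ice pillar actor for the Frozen Chef enemy assets that rises when the player comes near and sinks when they move away.
; Every tick it measures horizontal distance to the player and ramps a clamped build timer up within range or down outside it.
; That timer, multiplied by the Height variable, sets the actor's Z scale, so the pillar grows and shrinks smoothly over a quarter second.
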(event `self.ReceiveBeginPlay`)

(event `self.ReceiveTick`
  (params (DeltaSeconds :type "Float (single-precision)"))
  (set `self.Delta Seconds` DeltaSeconds)
  (`|ExecutionSequence`
    (:`then_0`
      (`self.SetActorScale3D` (`KismetMathLibrary.MakeVector` 1.0 1.0 (* (`self.BuildTimer`) (`self.Height`)))))
    (:`then_1`
      (if (< (`KismetMathLibrary.Distance2D` (`KismetMathLibrary.MakeVector2D` (.x (`self.K2_GetActorLocation` (`GameplayStatics.GetPlayerCharacter` 0))) (.y (`self.K2_GetActorLocation` (`GameplayStatics.GetPlayerCharacter` 0)))) (`KismetMathLibrary.MakeVector2D` (.x (`self.K2_GetActorLocation`)) (.y (`self.K2_GetActorLocation`)))) 750.0)
        (set `self.BuildTimer` (`KismetMathLibrary.FMin` (+ (`self.BuildTimer`) (* 4.0 (`self.Delta Seconds`))) 1.0))
        (else
          (set `self.BuildTimer` (`KismetMathLibrary.FMax` (- (`self.BuildTimer`) (* 4.0 (`self.Delta Seconds`))))))))))

(fn `UserConstructionScript`)