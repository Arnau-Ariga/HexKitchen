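; Popsicle enemy that chases the player and, within range, performs a straight charge that leaves puddles behind.
; Tick runs the attack cooldown, briefly uses AIMoveTo before halting, then resets ChargeDistance to start the dash.
; The dash offsets the capsule along the mesh's facing without sweep, spawning Puddle_standin1 actors underneath.
; ChargeHitbox launches the player upward during most of the charge; the freeze effect is unconnected.
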(event `self.ReceiveBeginPlay`
  (`parent.ReceiveBeginPlay`)
  (set `self.ShootingTimer` 0.0)
  (set `self.attackSpeed` 1.0)
  (set `self.ChargeDistance` 9999.0)
  (set `/Game/Blueprints/BPC_Health.Weakness` "NewEnumerator2" (`self.BPC_Health`)))

(event `self.ReceiveTick`
  (params (DeltaSeconds :type "Float (single-precision)"))
  (bind _returnvalue (* 1000.0 DeltaSeconds))
  (bind _returnvalue_2 (+ (.yaw (`SceneComponent.K2_GetComponentRotation` (`self.Mesh`))) 90.0))
  (`parent.ReceiveTick` DeltaSeconds)
  (`|ExecutionSequence`
    (:`then_0`
      (if (<= (`self.ShootingTimer`) 0.0)
        (if (<= (`KismetMathLibrary.Vector_Distance` (`self.K2_GetActorLocation` (`GameplayStatics.GetPlayerPawn` 0)) (`self.K2_GetActorLocation` self)) 750.0)
          (`self.stop`)
          (set `self.ShootingTimer` (+ (`self.ShootingTimer`) (/ 2.0 (`self.attackSpeed`))))
          (`|AIMoveTo` self (0.0 0.0 0.0) (`GameplayStatics.GetPlayerPawn` 0)
            (:`then`
              ; Popsicle sounds
              (`GameplayStatics.PlaySoundAtLocation` "/Game/SFX/Cues/Enemies+Characters/Popsicle_Cue.Popsicle_Cue" (`self.K2_GetActorLocation`) (struct) 1.0 1.0 0.0 null null null null)
              (`KismetSystemLibrary.Delay` 0.1)
              (`MovementComponent.StopMovementImmediately` (`self.CharacterMovement`))
              (set `self.ChargeDistance` 0.0)))
          (else
            (set `self.AIActive` true)
            (set `self.seeingPlayer` true)
            (`self.chase`)))
        (else
          (set `self.ShootingTimer` (- (`self.ShootingTimer`) DeltaSeconds)))))
    (:`then_1`
      (if (<= (`self.ChargeDistance`) 1000.0)
        (set `self.ChargeDistance` (+ _returnvalue (`self.ChargeDistance`)))
        (`SceneComponent.K2_AddWorldOffset` (`self.CapsuleComponent`) (`KismetMathLibrary.MakeVector` (* (`KismetMathLibrary.DegCos` _returnvalue_2) _returnvalue) (* (`KismetMathLibrary.DegSin` _returnvalue_2) _returnvalue)) false false)
        (if (<= (`self.SpawnIce`) 0.0)
          (set `self.ShootingTimer` (+ 0.0 (/ 0.2 (`self.attackSpeed`))))
          (`|SpawnActorFromClass` "/Game/Enemies/Enemy_Projectiles/puddle_standin1.puddle_standin1_C" (`KismetMathLibrary.MakeTransform` (`KismetMathLibrary.MakeVector` (.x (`SceneComponent.K2_GetComponentLocation` (`self.CapsuleComponent`))) (.y (`SceneComponent.K2_GetComponentLocation` (`self.CapsuleComponent`))) (- (.z (`SceneComponent.K2_GetComponentLocation` (`self.CapsuleComponent`))) 100.0))) "Undefined" "MultiplyWithRoot" null null)
          (else
            (set `self.SpawnIce` (- (`self.SpawnIce`) DeltaSeconds))))))))

(event `self.Charge Hitbox.OnComponentBeginOverlap`
  (params (OverlappedComponent :type "PrimitiveComponent Object Reference") (OtherActor :type "Actor Object Reference") (OtherComp :type "PrimitiveComponent Object Reference") (OtherBodyIndex :type Integer) (bFromSweep :type Boolean) (SweepResult :type "HitResult Structure (by ref)"))
  (if (`GameplayStatics.ObjectIsA` OtherActor (`GameplayStatics.GetObjectClass` (`GameplayStatics.GetPlayerCharacter` 0)))
    (if (<= (`self.ChargeDistance`) 750.0)
      (`self.LaunchCharacter` (`GameplayStatics.GetPlayerCharacter` 0) (0.0 0.0 750.0) false false))))

(fn `UserConstructionScript`
  (`parent.UserConstructionScript`))