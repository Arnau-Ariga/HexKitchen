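; Rat wizard enemy that faces the player every tick and casts a random attack whenever its shoot timer runs out.
; Attacks are a wall prison boxing in the player, a rock tornado, a repeated dive, a vortex storm and a rat swarm.
; Each adds its own delay; a prison on cooldown becomes a rock tornado.
; The dive interpolates location by timer, alternating slams that spawn shockwave rings with climbs back up.
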(event `self.ReceiveTick`
  (params (DeltaSeconds :type "Float (single-precision)"))
  (`parent.ReceiveTick` DeltaSeconds)
  (set `self.Delta Seconds` DeltaSeconds)
  (`self.FollowPlayer`)
  (`self.Attack`)
  (`self.diveTick`))

(event `FollowPlayer`
  (bind _returnvalue (- (`self.K2_GetActorLocation` (`GameplayStatics.GetPlayerCharacter` 0)) (`self.K2_GetActorLocation`)))
  (`self.K2_SetActorRotation` (`KismetMathLibrary.MakeRotFromXZ` _returnvalue _returnvalue)))

(event `Attack`
  (if (<= (`self.shootTimer`) 0.0)
    (bind _output_get (set `self.choice` (`KismetMathLibrary.RandomIntegerInRange` 0 4)))
    (if (== _output_get 0) :!label _label
      (if (<= (`self.wallTimer`) 0.0)
        (`self.Imprison`)
        (else
          (set `self.choice` (`KismetMathLibrary.RandomIntegerInRange` 1 1))
          (goto _label)))
      (elif (== _output_get 1)
        (`self.RockTornado`)
        (elif (== _output_get 2)
          (`self.Dive`)
          (elif (== _output_get 3)
            (`self.vortexStorm`)
            (elif (== _output_get 4)
              (`self.ratSwarm`))))))
    (else
      (set `self.shootTimer` (- (`self.shootTimer`) (`self.Delta Seconds`)))
      (set `self.wallTimer` (- (`self.wallTimer`) (`self.Delta Seconds`)))
      (set `self.dashTimer` (- (`self.dashTimer`) (`self.Delta Seconds`))))))

(event `Dive`
  ; Dash Attack
  (set `self.playerPos` (`self.K2_GetActorLocation` (`GameplayStatics.GetPlayerCharacter` 0)))
  (set `self.dashTimer` 1.0)
  (set `self.shootTimer` (+ (* 7.0 1.0) (`self.shootTimer`)))
  (set `self.fromPos` (`self.K2_GetActorLocation` self))
  (set `self.isDiving` true)
  (set `self.diveCount` 0))

(event `RockTornado`
  ; Rock Tornado
  (set `self.shootTimer` (+ (* 5.0 1.0) (`self.shootTimer`)))
  (for _ (range 11)
    (`|SpawnActorFromClass` "/Game/Enemies/Amalgamation_Data/Rat_Rock.Rat_Rock_C" (`KismetMathLibrary.MakeTransform` (`self.K2_GetActorLocation`)) "Undefined" "MultiplyWithRoot" null self 0.0 (struct) null)))

(event `diveTick`
  (bind _returnvalue (- 1.0 (`self.dashTimer`)))
  ; Dash Attack
  (if (`self.isDiving`)
    (`self.K2_SetActorLocation` (+ (`self.fromPos`) (* (- (`self.playerPos`) (`self.fromPos`)) (`KismetMathLibrary.MakeVector` _returnvalue _returnvalue _returnvalue))))
    (if (< (`self.dashTimer`) 0.0)
      (if (< (.z (`self.K2_GetActorLocation`)) 1000.0)
        (set `self.fromPos` (`self.playerPos`))
        (set `self.playerPos` (`KismetMathLibrary.MakeVector` (.x (`self.fromPos`)) (.y (`self.fromPos`)) 1028.0))
        (set `self.dashTimer` 1.0)
        (for _index (range 10)
          (`|SpawnActorFromClass` "/Game/Enemies/Enemy_Projectiles/Shockwave.Shockwave_C" (`KismetMathLibrary.MakeTransform` (`self.K2_GetActorLocation`) (`KismetMathLibrary.MakeRotator` 0.0 0.0 (* 36.0 _index)) (3.0 3.0 2.0)) "Undefined" "MultiplyWithRoot" null 0.0 (struct) null))
        (elif (< (`self.diveCount`) 2)
          (set `self.diveCount` (+ 1 (`self.diveCount`)))
          (set `self.playerPos` (`self.K2_GetActorLocation` (`GameplayStatics.GetPlayerCharacter` 0)))
          (set `self.dashTimer` 1.0)
          (set `self.fromPos` (`self.K2_GetActorLocation` self))
          (else
            (set `self.isDiving` false)))))))

(event `Imprison`
  ; Prison Wall
  (set `self.shootTimer` (+ (* 1.0 1.0) (`self.shootTimer`)))
  (set `self.wallTimer` 8.0)
  (`self.SpawnWallVert` 1000)
  (`self.SpawnWallVert` -1000)
  (`self.SpawnWallHorz` 1000)
  (`self.SpawnWallHorz` -1000))

(event `SpawnWallVert`
  (params (Xoff :type Integer))
  ; Prison Wall
  (for _index (range 10)
    (`|SpawnActorFromClass` "/Game/Enemies/Enemy_Projectiles/BP_Rat_Wall.BP_Rat_Wall_C" (`KismetMathLibrary.MakeTransform` (`KismetMathLibrary.MakeVector` (+ Xoff (.x (`self.K2_GetActorLocation` (`GameplayStatics.GetPlayerCharacter` 0)))) (+ (.y (`self.K2_GetActorLocation` (`GameplayStatics.GetPlayerCharacter` 0))) (`KismetMathLibrary.Conv_IntToDouble` (* (- _index 5) 200))) (`KismetMathLibrary.RandomFloatInRange` -550.0 -450.0)) (`KismetMathLibrary.MakeRotator` 0.0 0.0 (`KismetMathLibrary.RandomFloatInRange` 0.0 360.0)) (2.0 2.0 2.0)) "AlwaysSpawn" "MultiplyWithRoot" null null)))

(event `vortexStorm`
  ; VortexAttack
  (set `self.shootTimer` (+ (* 1.0 1.0) (`self.shootTimer`)))
  (`|SpawnActorFromClass` "/Game/Enemies/Enemy_Projectiles/VortexSpawner.VortexSpawner_C" (`KismetMathLibrary.MakeTransform` (`self.K2_GetActorLocation` (`GameplayStatics.GetPlayerCharacter` 0))) "Undefined" "MultiplyWithRoot" null null))

(event `ratSwarm`
  ; ratSwarm
  (set `self.shootTimer` (+ (* 6.0 1.0) (`self.shootTimer`)))
  (`|SpawnActorFromClass` "/Game/Enemies/Enemy_Projectiles/ratSwarmSpawner.ratSwarmSpawner_C" (`KismetMathLibrary.MakeTransform` (`self.K2_GetActorLocation` (`GameplayStatics.GetPlayerCharacter` 0))) "Undefined" "MultiplyWithRoot" null null))

(event `SpawnWallHorz`
  (params (Yoff :type Integer))
  ; Prison Wall
  (for _index (range 10)
    (`|SpawnActorFromClass` "/Game/Enemies/Enemy_Projectiles/BP_Rat_Wall.BP_Rat_Wall_C" (`KismetMathLibrary.MakeTransform` (`KismetMathLibrary.MakeVector` (+ (.x (`self.K2_GetActorLocation` (`GameplayStatics.GetPlayerCharacter` 0))) (`KismetMathLibrary.Conv_IntToDouble` (* (- _index 5) 200))) (+ Yoff (.y (`self.K2_GetActorLocation` (`GameplayStatics.GetPlayerCharacter` 0)))) (`KismetMathLibrary.RandomFloatInRange` -550.0 -450.0)) (`KismetMathLibrary.MakeRotator` 0.0 0.0 (`KismetMathLibrary.RandomFloatInRange` 0.0 360.0)) (2.0 2.0 2.0)) "AlwaysSpawn" "MultiplyWithRoot" null null)))

(fn `UserConstructionScript`
  (`parent.UserConstructionScript`))