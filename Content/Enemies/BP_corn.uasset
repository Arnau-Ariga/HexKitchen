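; BP_corn is an enemy that chases the player and fires a shotgun-style burst of corn projectiles at close range.
; When its Tick-driven cooldown expires, it checks player distance and either chases or stops and resets the timer, scaled by attack speed.
; To attack, it issues a brief AI move toward the player, halts, then spawns projectiles from the Shoot component with randomized rotation spread and speed.
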(event `self.ReceiveBeginPlay`
  (`parent.ReceiveBeginPlay`)
  (set `self.ShootingTimer` 0.0)
  (set `self.attackSpeed` 1.0))

(event `self.ReceiveTick`
  (params (DeltaSeconds :type "Float (single-precision)"))
  (`parent.ReceiveTick` DeltaSeconds)
  (if (<= (`self.ShootingTimer`) 0.0)
    (if (<= (`KismetMathLibrary.Vector_Distance` (`self.K2_GetActorLocation` (`GameplayStatics.GetPlayerPawn` 0)) (`self.K2_GetActorLocation` self)) 250.0)
      (`self.stop`)
      (set `self.ShootingTimer` (+ (`self.ShootingTimer`) (/ 2.0 (`self.attackSpeed`))))
      (`|AIMoveTo` self (0.0 0.0 0.0) (`GameplayStatics.GetPlayerPawn` 0)
        (:`then`
          (`KismetSystemLibrary.Delay` 0.1)
          (`MovementComponent.StopMovementImmediately` (`self.CharacterMovement`))
          (for _ (range 11)
            (`|SpawnActorFromClass` "/Game/Enemies/Enemy_Projectiles/Corn_Projectile.Corn_Projectile_C" (`KismetMathLibrary.MakeTransform` (`SceneComponent.K2_GetComponentLocation` (`self.Shoot`)) (`KismetMathLibrary.MakeRotator` (+ (.roll (`SceneComponent.K2_GetComponentRotation` (`self.Shoot`))) (`KismetMathLibrary.RandomInteger64InRange` -20 20)) (+ (.pitch (`SceneComponent.K2_GetComponentRotation` (`self.Shoot`))) (`KismetMathLibrary.RandomInteger64InRange` -20 20)) (+ (.yaw (`SceneComponent.K2_GetComponentRotation` (`self.Shoot`))) (`KismetMathLibrary.RandomInteger64InRange` -20 20))) (.scale (`self.GetTransform`))) "Undefined" "MultiplyWithRoot" null (`KismetMathLibrary.Conv_Int64ToDouble` (`KismetMathLibrary.RandomInteger64InRange` 1000 2000)) (`self.K2_GetActorRotation` self) null))))
      (else
        (set `self.AIActive` true)
        (set `self.seeingPlayer` true)
        (`self.chase`)))
    (else
      (set `self.ShootingTimer` (- (`self.ShootingTimer`) DeltaSeconds)))))

(fn `UserConstructionScript`
  (`parent.UserConstructionScript`))