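; BP_Rat_Wall is an enemy projectile actor, named as a rat wall, that rises after spawning and later removes itself.
; BeginPlay starts a short rise timer and sets a fixed lifespan.
; Tick counts the timer down and moves the actor straight up at a constant, frame-rate-independent speed without sweeping, then holds it in place until the lifespan expires.
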(event `self.ReceiveBeginPlay`
  (set `self.moveUpTimer` 1.0)
  (`self.SetLifeSpan` 8.0))

(event `self.ReceiveTick`
  (params (DeltaSeconds :type "Float (single-precision)"))
  (set `self.Delta Seconds` DeltaSeconds)
  (bind _output_get (set `self.moveUpTimer` (- (`self.moveUpTimer`) (`self.Delta Seconds`))))
  (if (> _output_get 0.0)
    (`self.K2_SetActorLocation` (+ (`self.K2_GetActorLocation`) (`KismetMathLibrary.MakeVector` 0.0 0.0 (* 500.0 (`self.Delta Seconds`)))))))

(fn `UserConstructionScript`)