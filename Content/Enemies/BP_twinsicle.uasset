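; BP_twinsicle is a ranged enemy that splits into two BP_popsicle actors when killed.
; Whenever its shooting timer runs out, Tick either chases a player beyond 1000 units or attacks one within range.
; An attack issues a brief AIMoveTo toward the player, halts movement, then fires Icicles from two shoot points along the actor's rotation, with AttackSpeed scaling the cooldown.
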(event `self.ReceiveBeginPlay`
  (`parent.ReceiveBeginPlay`)
  (set `self.ShootingTimer` 0.0)
  (set `self.attackSpeed` 1.0)
  (set `self.destroyEffect` true))

(event `self.ReceiveTick`
  (params (DeltaSeconds :type "Float (single-precision)"))
  (`parent.ReceiveTick` DeltaSeconds)
  (if (`self.shouldKill`)
    (`self.onKill`)
    (elif (<= (`self.ShootingTimer`) 0.0)
      (if (<= (`KismetMathLibrary.Vector_Distance` (`self.K2_GetActorLocation` (`GameplayStatics.GetPlayerPawn` 0)) (`self.K2_GetActorLocation` self)) 1000.0)
        (`self.stop`)
        (set `self.ShootingTimer` (+ (`self.ShootingTimer`) (/ 1.5 (`self.attackSpeed`))))
        (`|AIMoveTo` self (0.0 0.0 0.0) (`GameplayStatics.GetPlayerPawn` 0)
          (:`then`
            (`KismetSystemLibrary.Delay` 0.1)
            (`MovementComponent.StopMovementImmediately` (`self.CharacterMovement`))
            (`|SpawnActorFromClass` "/Game/Enemies/Enemy_Projectiles/Icicle.Icicle_C" (`KismetMathLibrary.MakeTransform` (`SceneComponent.K2_GetComponentLocation` (`self.Shoot`)) (`SceneComponent.K2_GetComponentRotation` (`self.Shoot`)) (.scale (`self.GetTransform`))) "Undefined" "MultiplyWithRoot" null 1000.0 (`self.K2_GetActorRotation` self) null)
            (`|SpawnActorFromClass` "/Game/Enemies/Enemy_Projectiles/Icicle.Icicle_C" (`KismetMathLibrary.MakeTransform` (`SceneComponent.K2_GetComponentLocation` (`self.Shoot1`)) (`SceneComponent.K2_GetComponentRotation` (`self.Shoot1`)) (.scale (`self.GetTransform`))) "Undefined" "MultiplyWithRoot" null 1000.0 (`self.K2_GetActorRotation` self) null)))
        (else
          (set `self.AIActive` true)
          (set `self.seeingPlayer` true)
          (`self.chase`)))
      (else
        (set `self.ShootingTimer` (- (`self.ShootingTimer`) DeltaSeconds))))))

(event `onKill`
  (`|SpawnActorFromClass` "/Game/Enemies/BP_popsicle.BP_popsicle_C" (`self.GetTransform` self) "Undefined" "MultiplyWithRoot" null null)
  (`|SpawnActorFromClass` "/Game/Enemies/BP_popsicle.BP_popsicle_C" (`self.GetTransform` self) "Undefined" "MultiplyWithRoot" null null)
  (`self.K2_DestroyActor`))

(fn `UserConstructionScript`
  (`parent.UserConstructionScript`))