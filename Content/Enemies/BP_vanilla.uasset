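; Vanilla enemy that picks between chasing, fireball attacks and an evasive probe based on distance to the player.
; Tick runs a cooldown scaled by AttackSpeed, then chases beyond 1300 units.
; At mid range it briefly moves toward the player, halts and fires a Vanilla_Fireball from Shoot.
; Within 700 units it spawns a Tele_Check at a random point on a raised ring around itself, apparently for teleporting.
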(event `self.ReceiveBeginPlay`
  (`parent.ReceiveBeginPlay`)
  (set `self.ShootingTimer` 0.0)
  (set `self.attackSpeed` 1.0))

(event `self.ReceiveTick`
  (params (DeltaSeconds :type "Float (single-precision)"))
  (`parent.ReceiveTick` DeltaSeconds)
  (if (<= (`self.ShootingTimer`) 0.0)
    (if (<= (`KismetMathLibrary.Vector_Distance` (`self.K2_GetActorLocation` (`GameplayStatics.GetPlayerPawn` 0)) (`self.K2_GetActorLocation` self)) 1300.0)
      (if (<= (`KismetMathLibrary.Vector_Distance` (`self.K2_GetActorLocation` (`GameplayStatics.GetPlayerPawn` 0)) (`self.K2_GetActorLocation` self)) 700.0)
        (set `self.ShootingTimer` (+ (`self.ShootingTimer`) (/ 1.0 (`self.attackSpeed`))))
        (set `self.randAng` (`KismetMathLibrary.RandomInteger` 360))
        (bind _returnvalue (`|SpawnActorFromClass` "/Game/Enemies/Enemy_Projectiles/Tele_Check.Tele_Check_C" (`KismetMathLibrary.MakeTransform` (`KismetMathLibrary.MakeVector` (+ (* (`KismetMathLibrary.DegCos` (`KismetMathLibrary.Conv_IntToDouble` (`self.randAng`))) 750.0) (.x (`SceneComponent.K2_GetComponentLocation` (`self.Shoot`)))) (+ (* (`KismetMathLibrary.DegSin` (`KismetMathLibrary.Conv_IntToDouble` (`self.randAng`))) 750.0) (.y (`SceneComponent.K2_GetComponentLocation` (`self.Shoot`)))) (+ (.z (`SceneComponent.K2_GetComponentLocation` (`self.Shoot`))) 200.0)) (struct :`Pitch` -90.0) (.scale (`self.GetTransform`))) "Undefined" "MultiplyWithRoot" null self 1000.0 (`self.K2_GetActorRotation` self) null))
        (`GameplayStatics.PlaySoundAtLocation` "/Game/SFX/Cues/Enemies+Characters/EnemyPoof_Cue.EnemyPoof_Cue" (`self.K2_GetActorLocation` _returnvalue) (struct) 1.0 1.0 0.0 null null null null)
        (else
          (`self.stop`)
          (set `self.ShootingTimer` (+ (`self.ShootingTimer`) (/ 3.0 (`self.attackSpeed`))))
          (`|AIMoveTo` self (0.0 0.0 0.0) (`GameplayStatics.GetPlayerPawn` 0)
            (:`then`
              (`KismetSystemLibrary.Delay` 0.1)
              (`MovementComponent.StopMovementImmediately` (`self.CharacterMovement`))
              (bind _returnvalue_2 (`|SpawnActorFromClass` "/Game/Enemies/Enemy_Projectiles/Vanilla_Fireball.Vanilla_Fireball_C" (`KismetMathLibrary.MakeTransform` (`SceneComponent.K2_GetComponentLocation` (`self.Shoot`)) (`SceneComponent.K2_GetComponentRotation` (`self.Shoot`)) (.scale (`self.GetTransform`))) "Undefined" "MultiplyWithRoot" null 1000.0 (`self.K2_GetActorRotation` self) null))
              (`GameplayStatics.PlaySoundAtLocation` "/Game/SFX/Cues/Enemies+Characters/Fireball_Cue.Fireball_Cue" (`self.K2_GetActorLocation` _returnvalue_2) (struct) 1.0 1.0 0.0 "/Game/SFX/AttenuationConcurrency/WorldAttenuation.WorldAttenuation" null null null)))))
      (else
        (set `self.AIActive` true)
        (set `self.seeingPlayer` true)
        (`self.chase`)))
    (else
      (set `self.ShootingTimer` (- (`self.ShootingTimer`) DeltaSeconds)))))

(fn `UserConstructionScript`
  (`parent.UserConstructionScript`))