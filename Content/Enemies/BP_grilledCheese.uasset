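; Grilled cheese enemy that picks one of three random attacks whenever its Tick-driven cooldown expires.
; It stops to spray projectiles at random angles, moves briefly toward the player to launch a spatula, or rings the player with randomly placed enemy spawn indicators.
; Each attack adds its own cooldown, scaled by AttackSpeed.
; The chase fallback sits behind an always-true branch and never runs, and ChooseMove is an empty stub.
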(event `self.ReceiveBeginPlay`
  (`parent.ReceiveBeginPlay`)
  (set `self.ShootingTimer` 0.0)
  (set `self.attackSpeed` 1.0))

(event `self.ReceiveTick`
  (params (DeltaSeconds :type "Float (single-precision)"))
  (`parent.ReceiveTick` DeltaSeconds)
  (if (<= (`self.ShootingTimer`) 0.0)
    (if true
      (bind _output_get (set `self.Choice` (`KismetMathLibrary.RandomIntegerInRange` 1 3)))
      (if (== 1 _output_get)
        (`self.stop`)
        (set `self.ShootingTimer` (+ (`self.ShootingTimer`) (/ 3.0 (`self.attackSpeed`))))
        (for _ (range 31)
          (`|SpawnActorFromClass` "/Game/Enemies/Enemy_Projectiles/Grilled_Cheese_Projectile.Grilled_Cheese_Projectile_C" (`KismetMathLibrary.MakeTransform` (`SceneComponent.K2_GetComponentLocation` (`self.Shoot`)) (`KismetMathLibrary.MakeRotator` 0.0 (`KismetMathLibrary.Conv_Int64ToDouble` (`KismetMathLibrary.RandomInteger64InRange` 45 85)) (`KismetMathLibrary.Conv_Int64ToDouble` (`KismetMathLibrary.RandomInteger64InRange` 0 360))) (.scale (`self.GetTransform`))) "Undefined" "MultiplyWithRoot" null 1000.0 (`self.K2_GetActorRotation` self) null))
        (elif (== 2 _output_get)
          (set `self.ShootingTimer` (+ (`self.ShootingTimer`) (/ 1.0 (`self.attackSpeed`))))
          (`|AIMoveTo` self (0.0 0.0 0.0) (`GameplayStatics.GetPlayerPawn` 0)
            (:`then`
              (`KismetSystemLibrary.Delay` 0.1)
              (`MovementComponent.StopMovementImmediately` (`self.CharacterMovement`))
              (bind _returnvalue (`|SpawnActorFromClass` "/Game/Enemies/Enemy_Projectiles/Spatula.Spatula_C" (`KismetMathLibrary.MakeTransform` (`KismetMathLibrary.MakeVector` (.x (`SceneComponent.K2_GetComponentLocation` (`self.Shoot`))) (.y (`SceneComponent.K2_GetComponentLocation` (`self.Shoot`))) (- (.z (`SceneComponent.K2_GetComponentLocation` (`self.Shoot`))) 110.0)) (`KismetMathLibrary.MakeRotator` 0.0 0.0 (+ (.yaw (`SceneComponent.K2_GetComponentRotation` (`self.Mesh`))) -90.0)) (4.0 4.0 4.0)) "Undefined" "MultiplyWithRoot" null 1000.0 (`self.K2_GetActorRotation` self) null))
              (`GameplayStatics.PlaySoundAtLocation` "/Game/SFX/Cues/Enemies+Characters/Whoosh_Cue.Whoosh_Cue" (`self.K2_GetActorLocation` _returnvalue) (struct) 1.0 1.0 0.0 null null null null)))
          (else
            (set `self.ShootingTimer` (+ (`self.ShootingTimer`) (/ 10.0 (`self.attackSpeed`))))
            (for _ (range 4)
              (set `self.randAngle` (`KismetMathLibrary.RandomInteger64InRange` 0 360))
              (`|SpawnActorFromClass` "/Game/Enemies/Enemy_Projectiles/EnemySpawnIndicator.EnemySpawnIndicator_C" (`KismetMathLibrary.MakeTransform` (`KismetMathLibrary.MakeVector` (+ (.x (`SceneComponent.K2_GetComponentLocation` (`Actor.RootComponent` (`GameplayStatics.GetPlayerPawn` 0)))) (* 600.0 (`KismetMathLibrary.DegCos` (`KismetMathLibrary.Conv_Int64ToDouble` (`self.randAngle`))))) (+ (.y (`SceneComponent.K2_GetComponentLocation` (`Actor.RootComponent` (`GameplayStatics.GetPlayerPawn` 0)))) (* 600.0 (`KismetMathLibrary.DegSin` (`KismetMathLibrary.Conv_Int64ToDouble` (`self.randAngle`))))) (.z (`SceneComponent.K2_GetComponentLocation` (`Actor.RootComponent` (`GameplayStatics.GetPlayerPawn` 0)))))) "Undefined" "MultiplyWithRoot" null null)))))
      (else
        (set `self.AIActive` true)
        (set `self.seeingPlayer` true)
        (`self.chase`)))
    (else
      (set `self.ShootingTimer` (- (`self.ShootingTimer`) DeltaSeconds)))))

(fn `chooseMove`
  (params (NewParam :type Integer)))

(fn `UserConstructionScript`
  (`parent.UserConstructionScript`))