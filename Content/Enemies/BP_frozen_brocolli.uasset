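; Frozen broccoli enemy that turns toward the player and fires Frozen_Broccoli_Projectile at close range.
; Every tick it rotates to face the player character, and a countdown scaled by AttackSpeed gates projectile spawns while the player is within range.
; When the countdown is ready but the player is out of range, it sets AIActive and SeeingPlayer instead.
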(event `self.ReceiveBeginPlay`
  (`parent.ReceiveBeginPlay`)
  (set `self.ShootingTimer` 0.0)
  (set `self.attackSpeed` 1.0))

(event `self.ReceiveTick`
  (params (DeltaSeconds :type "Float (single-precision)"))
  (bind _returnvalue (- (`self.K2_GetActorLocation` (`GameplayStatics.GetPlayerCharacter` 0)) (`self.K2_GetActorLocation`)))
  (`parent.ReceiveTick` DeltaSeconds)
  (`self.K2_SetActorRotation` (`KismetMathLibrary.MakeRotFromXZ` _returnvalue _returnvalue))
  (if (<= (`self.ShootingTimer`) 0.0)
    (if (<= (`KismetMathLibrary.Vector_Distance` (`self.K2_GetActorLocation` (`GameplayStatics.GetPlayerPawn` 0)) (`self.K2_GetActorLocation` self)) 1000.0)
      (set `self.ShootingTimer` (+ (`self.ShootingTimer`) (/ 3.0 (`self.attackSpeed`))))
      (`|SpawnActorFromClass` "/Game/Enemies/Enemy_Projectiles/Frozen_Broccoli_Projectile.Frozen_Broccoli_Projectile_C" (`KismetMathLibrary.MakeTransform` (`self.K2_GetActorLocation`) (`self.K2_GetActorRotation`)) "Undefined" "MultiplyWithRoot" null 0.0 (struct) null)
      (else
        (set `self.AIActive` true)
        (set `self.seeingPlayer` true)))
    (else
      (set `self.ShootingTimer` (- (`self.ShootingTimer`) DeltaSeconds)))))

(fn `UserConstructionScript`
  (`parent.UserConstructionScript`))