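; Grape bunch enemy that chases the player and periodically spawns BP_grape actors, built on a parent class with a weakness set at BeginPlay.
; Once its cooldown expires, Tick checks player distance: out of range it chases, within range it stops and resets the timer, scaled by AttackSpeed.
; It then plays a spawn sound and, after a short delay, spawns four grapes in a world-axis cross around its Shoot component.
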(event `self.ReceiveBeginPlay`
  (`parent.ReceiveBeginPlay`)
  (set `self.ShootingTimer` 0.0)
  (set `self.SpawnDistance` 200.0)
  (set `self.attackSpeed` 1.0)
  (set `/Game/Blueprints/BPC_Health.Weakness` "NewEnumerator0" (`self.BPC_Health`)))

(event `self.ReceiveTick`
  (params (DeltaSeconds :type "Float (single-precision)"))
  (`parent.ReceiveTick` DeltaSeconds)
  (if (<= (`self.ShootingTimer`) 0.0)
    (if (<= (`KismetMathLibrary.Vector_Distance` (`self.K2_GetActorLocation` (`GameplayStatics.GetPlayerPawn` 0)) (`self.K2_GetActorLocation` self)) 750.0)
      (`self.stop`)
      (set `self.ShootingTimer` (+ (`self.ShootingTimer`) (/ 7.0 (`self.attackSpeed`))))
      ; Sound Effect
      (`GameplayStatics.PlaySoundAtLocation` "/Game/SFX/Cues/Enemies+Characters/EnemySpawn_Cue.EnemySpawn_Cue" (`self.K2_GetActorLocation`) (struct) 1.0 1.0 0.0 null null null null)
      (`KismetSystemLibrary.Delay` 2.0)
      ; Spawn Grapes
      (`|SpawnActorFromClass` "/Game/Enemies/BP_grape.BP_grape_C" (`KismetMathLibrary.MakeTransform` (`KismetMathLibrary.MakeVector` (+ (.x (`SceneComponent.K2_GetComponentLocation` (`self.Shoot`))) (`self.SpawnDistance`)) (.y (`SceneComponent.K2_GetComponentLocation` (`self.Shoot`))) (.z (`SceneComponent.K2_GetComponentLocation` (`self.Shoot`)))) (`SceneComponent.K2_GetComponentRotation` (`self.Shoot`)) (.scale (`SceneComponent.K2_GetComponentToWorld` (`self.Shoot`)))) "Undefined" "MultiplyWithRoot" null null)
      (`|SpawnActorFromClass` "/Game/Enemies/BP_grape.BP_grape_C" (`KismetMathLibrary.MakeTransform` (`KismetMathLibrary.MakeVector` (- (.x (`SceneComponent.K2_GetComponentLocation` (`self.Shoot`))) (`self.SpawnDistance`)) (.y (`SceneComponent.K2_GetComponentLocation` (`self.Shoot`))) (.z (`SceneComponent.K2_GetComponentLocation` (`self.Shoot`)))) (`SceneComponent.K2_GetComponentRotation` (`self.Shoot`)) (.scale (`SceneComponent.K2_GetComponentToWorld` (`self.Shoot`)))) "Undefined" "MultiplyWithRoot" null null)
      (`|SpawnActorFromClass` "/Game/Enemies/BP_grape.BP_grape_C" (`KismetMathLibrary.MakeTransform` (`KismetMathLibrary.MakeVector` (.x (`SceneComponent.K2_GetComponentLocation` (`self.Shoot`))) (+ (.y (`SceneComponent.K2_GetComponentLocation` (`self.Shoot`))) (`self.SpawnDistance`)) (.z (`SceneComponent.K2_GetComponentLocation` (`self.Shoot`)))) (`SceneComponent.K2_GetComponentRotation` (`self.Shoot`)) (.scale (`SceneComponent.K2_GetComponentToWorld` (`self.Shoot`)))) "Undefined" "MultiplyWithRoot" null null)
      (`|SpawnActorFromClass` "/Game/Enemies/BP_grape.BP_grape_C" (`KismetMathLibrary.MakeTransform` (`KismetMathLibrary.MakeVector` (.x (`SceneComponent.K2_GetComponentLocation` (`self.Shoot`))) (- (.y (`SceneComponent.K2_GetComponentLocation` (`self.Shoot`))) (`self.SpawnDistance`)) (.z (`SceneComponent.K2_GetComponentLocation` (`self.Shoot`)))) (`SceneComponent.K2_GetComponentRotation` (`self.Shoot`)) (.scale (`SceneComponent.K2_GetComponentToWorld` (`self.Shoot`)))) "Undefined" "MultiplyWithRoot" null null)
      (else
        (set `self.AIActive` true)
        (set `self.seeingPlayer` true)
        (`self.chase`)))
    (else
      (set `self.ShootingTimer` (- (`self.ShootingTimer`) DeltaSeconds)))))

(fn `UserConstructionScript`
  (`parent.UserConstructionScript`))