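; BP_enemy_base is a base enemy Blueprint that displays health and damage weakness and handles removal.
; Each Tick it pushes BPCHealth's health ratio, rounded-up value and weakness to the W_EnemyHealth widget, which it rotates toward the player with pitch zeroed.
; Tick also picks the Slash, Stab or Blunt billboard sprite from the weakness.
; The kill event either sets ShouldKill when DestroyEffect is set, or destroys the actor immediately.
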(event `self.ReceiveBeginPlay`
  (set `self.attackSpeed` 1.0))

(event `self.ReceiveTick`
  (params (DeltaSeconds :type "Float (single-precision)"))
  (bind _bpc_health (`self.BPC_Health`))
  (bind _health (`/Game/Blueprints/BPC_Health.Health` _bpc_health))
  (bind _weakness (`/Game/Blueprints/BPC_Health.Weakness` (`self.BPC_Health`)))
  (bind _returnvalue (- (`self.K2_GetActorLocation` (`GameplayStatics.GetPlayerCharacter` 0)) (`self.K2_GetActorLocation`)))
  (bind _asw_enemy_health (cast `/Game/UI/W_EnemyHealth` (`WidgetComponent.GetUserWidgetObject` (`self.Widget`))))
  (`/Game/UI/W_EnemyHealth.SetPercentBar` _asw_enemy_health (/ _health (`/Game/Blueprints/BPC_Health.MaxHealth` _bpc_health)) (`KismetStringLibrary.Conv_Int64ToString` (`KismetMathLibrary.FCeil64` _health)) _weakness)
  (`SceneComponent.K2_SetWorldRotation` (`self.Widget`) (`KismetMathLibrary.MakeRotator` (.roll (`KismetMathLibrary.MakeRotFromXZ` _returnvalue _returnvalue)) 0.0 (.yaw (`KismetMathLibrary.MakeRotFromXZ` _returnvalue _returnvalue))) false false)
  (`BillboardComponent.SetSprite` (`self.Billboard`) (select `/Game/Items/Weapons/Enum_DamageType` _weakness :`NewEnumerator0` "/Game/Bright-Condiments/UI/slash.slash" :`NewEnumerator1` "/Game/Bright-Condiments/UI/stab.stab" :`NewEnumerator2` "/Game/Bright-Condiments/UI/blunt.blunt" :!type "Texture2D Object Reference")))

(event `kill`
  (if (`self.destroyEffect`)
    (set `self.shouldKill` true)
    (else
      (`self.K2_DestroyActor`))))

(fn `UserConstructionScript`)