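; Enemy stats component that tracks health, starting it at MaxHealth and exposing it through a getter.
; It binds to the owner's OnTakeAnyDamage and subtracts damage scaled by a CompareDamageTypes multiplier.
; That function holds unconnected weakness-based critical-hit logic, and its type input comes from the empty TakeDamage event rather than the damage delegate.
; At zero health or below it flags death and destroys the owning actor.
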(event `self.ReceiveBeginPlay`
  (set `self.Health` (`self.MaxHealth`))
  (add `Actor.OnTakeAnyDamage` (`self.GetOwner`) (delegate `CustomEvent`)))

(event `CustomEvent`
  (params (DamagedActor :type "Actor Object Reference") (Damage :type "Float (single-precision)") (DamageType :type "DamageType Object Reference") (InstigatedBy :type "Controller Object Reference") (DamageCauser :type "Actor Object Reference"))
  (bind _output_get (set `self.Health` (- (`self.Health`) (* Damage (select `bool` (and (!= (stale `Event Take Damage` Type) 0) (== (stale `Event Take Damage` Type) (`KismetSystemLibrary.MakeLiteralByte` (`self.Weakness`)))) :`false` 1.0 :`true` 2.0)))))
  (if (<= _output_get 0.0)
    (set `self.Is Dead` true)
    (`Actor.K2_DestroyActor` (`self.GetOwner`)) ; If the enemy is dead then delete it from the world
  ))

(event `Event Take Damage`
  (params (Damage :type "Float (double-precision)") (Type :type Byte :default 0)))

(fn `Get Health`
  (returns (Health :type "Float (double-precision)"))
  (return (`self.Health`)))