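; BP_rat_wizard is an enemy Blueprint for a rat wizard that turns toward the player and picks attacks on a timer.
; Each Tick rotates it along the direction to the player character, then counts ShootTimer down or triggers a randomly selected attack once it expires.
; The only attack, RockTornado, is a stub: its 20-step loop is empty and its timer increment evaluates to zero.
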(event `self.ReceiveTick`
  (params (DeltaSeconds :type "Float (single-precision)"))
  (`parent.ReceiveTick` DeltaSeconds)
  (set `self.Delta Seconds` DeltaSeconds)
  (`self.FollowPlayer`)
  (`self.Attack`))

(event `FollowPlayer`
  (bind _returnvalue (- (`self.K2_GetActorLocation` (`GameplayStatics.GetPlayerCharacter` 0)) (`self.K2_GetActorLocation`)))
  (`self.K2_SetActorRotation` (`KismetMathLibrary.MakeRotFromXZ` _returnvalue _returnvalue)))

(event `Attack`
  (if (<= (`self.shootTimer`) 0.0)
    (bind _output_get (set `self.choice` (`KismetMathLibrary.RandomIntegerInRange` 0)))
    (if (== _output_get 0)
      (`self.RockTornado`))
    (else
      (set `self.shootTimer` (- (`self.shootTimer`) (`self.Delta Seconds`))))))

(event `RockTornado`
  ; Rock Tornado
  (set `self.shootTimer` (+ (* 0.0 0.0) (`self.shootTimer`)))
  (for _ (range 20)
    _))

(fn `UserConstructionScript`
  (`parent.UserConstructionScript`))