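; BP_grape is an enemy actor that launches the player upward and destroys itself on close proximity.
; Tick compares its distance to the player pawn against a small radius instead of using overlap events, then calls LaunchCharacter followed by DestroyActor.
; A shooting timer is reset at BeginPlay but otherwise unused, and the nodes setting the player-sighted shooting flag and calling Stop are unconnected.
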(event `self.ReceiveBeginPlay`
  (`parent.ReceiveBeginPlay`)
  (set `self.ShootingTimer` 0.0))

(event `self.ReceiveTick`
  (params (DeltaSeconds :type "Float (single-precision)"))
  (`parent.ReceiveTick` DeltaSeconds)
  (if (<= (`KismetMathLibrary.Vector_Distance` (`self.K2_GetActorLocation` (`GameplayStatics.GetPlayerPawn` 0)) (`self.K2_GetActorLocation` self)) 100.0)
    (`self.LaunchCharacter` (`GameplayStatics.GetPlayerCharacter` 0) (0.0 0.0 250.0) false false)
    (`self.K2_DestroyActor`)))

(fn `UserConstructionScript`
  (`parent.UserConstructionScript`))