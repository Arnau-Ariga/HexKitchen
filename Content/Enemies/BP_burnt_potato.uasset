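; Burnt potato enemy that chases the player on sight and has a preset weakness on its health component.
; PawnSensing sightings set SeeingPlayer and trigger an AI MoveTo toward player 0, which clears that flag on success.
; A stop event disables the AI, clears the sighting and halts character movement immediately.
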(event `self.ReceiveBeginPlay`
  (`parent.ReceiveBeginPlay`)
  (set `self.AIActive` true)
  (set `/Game/Blueprints/BPC_Health.Weakness` "NewEnumerator2" (`self.BPC_Health`)))

(event `self.PawnSensing.OnSeePawn`
  (params (Pawn :type "Pawn Object Reference"))
  (if (`self.AIActive`)
    (set `self.seeingPlayer` true)
    (`self.chase`)))

(event `chase`
  (if (`self.seeingPlayer`)
    (`|AIMoveTo` self (0.0 0.0 0.0) (`GameplayStatics.GetPlayerPawn` 0)
      (:`OnSuccess`
        (set `self.seeingPlayer` false)))))

(event `stop`
  (set `self.AIActive` false)
  (set `self.seeingPlayer` false)
  (`MovementComponent.StopMovementImmediately` (`self.CharacterMovement`)))

(fn `UserConstructionScript`
  (`parent.UserConstructionScript`))