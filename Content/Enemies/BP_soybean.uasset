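; BP_soybean is a ninja-style enemy that chases the player and, within 500 units, randomly picks one of two attacks on a cooldown timer.
; One spawns three shurikens from separate arrow components.
; The other flashes a smoke bomb, then starts a charge that Tick drives with unswept capsule offsets along the mesh's facing.
; During the charge, ChargeHitbox overlaps launch the player upward; Chase and Stop handle movement between attacks.
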(event `self.ReceiveBeginPlay`
  (`parent.ReceiveBeginPlay`)
  (set `self.ShootingTimer` 0.0)
  (set `self.attackSpeed` 1.0)
  (set `self.ChargeDistance` 9999.0))

(event `self.ReceiveTick`
  (params (DeltaSeconds :type "Float (single-precision)"))
  (bind _returnvalue (* 2000.0 DeltaSeconds))
  (bind _returnvalue_2 (+ (.yaw (`SceneComponent.K2_GetComponentRotation` (`self.Mesh`))) 90.0))
  (`parent.ReceiveTick` DeltaSeconds)
  (`|ExecutionSequence`
    (:`then_0`
      (if (<= (`self.ShootingTimer`) 0.0)
        (if (<= (`KismetMathLibrary.Vector_Distance` (`self.K2_GetActorLocation` (`GameplayStatics.GetPlayerPawn` 0)) (`self.K2_GetActorLocation` self)) 500.0)
          (`self.stop`)
          (if (== (`KismetMathLibrary.RandomInteger64InRange` 0 1) 0)
            (set `self.ShootingTimer` (+ (`self.ShootingTimer`) (/ 2.0 (`self.attackSpeed`))))
            (`|AIMoveTo` self (0.0 0.0 0.0) (`GameplayStatics.GetPlayerPawn` 0)
              (:`then`
                (`KismetSystemLibrary.Delay` 0.1)
                (`MovementComponent.StopMovementImmediately` (`self.CharacterMovement`))
                (`ActorComponent.Activate` (`self.smokeBomb`) false)
                (`KismetSystemLibrary.Delay` 0.5)
                (`ActorComponent.Deactivate` (`self.smokeBomb`))
                (set `self.ChargeDistance` 0.0)))
            (else
              (set `self.ShootingTimer` (+ (`self.ShootingTimer`) (/ 1.0 (`self.attackSpeed`))))
              (`|AIMoveTo` self (0.0 0.0 0.0) (`GameplayStatics.GetPlayerPawn` 0)
                (:`then`
                  (`KismetSystemLibrary.Delay` 0.1)
                  (`MovementComponent.StopMovementImmediately` (`self.CharacterMovement`))
                  (`|ExecutionSequence`
                    (:`then_0`
                      (set `self.currArrow` (`self.Shoot`)))
                    (:`then_1`
                      (set `self.currArrow` (`self.Shoot1`)))
                    (:`then_2`
                      (set `self.currArrow` (`self.Shoot2`))))
                  (`|SpawnActorFromClass` "/Game/Enemies/Enemy_Projectiles/Suriken.Suriken_C" (`KismetMathLibrary.MakeTransform` (`SceneComponent.K2_GetComponentLocation` (`self.currArrow`)) (`SceneComponent.K2_GetComponentRotation` (`self.currArrow`)) (.scale (`self.GetTransform`))) "Undefined" "MultiplyWithRoot" null 1000.0 (`self.K2_GetActorRotation` self) null)))))
          (else
            (set `self.AIActive` true)
            (set `self.seeingPlayer` true)
            (`self.chase`)))
        (else
          (set `self.ShootingTimer` (- (`self.ShootingTimer`) DeltaSeconds)))))
    (:`then_1`
      (if (<= (`self.ChargeDistance`) 750.0)
        (set `self.ChargeDistance` (+ _returnvalue (`self.ChargeDistance`)))
        (`SceneComponent.K2_AddWorldOffset` (`self.CapsuleComponent`) (`KismetMathLibrary.MakeVector` (* (`KismetMathLibrary.DegCos` _returnvalue_2) _returnvalue) (* (`KismetMathLibrary.DegSin` _returnvalue_2) _returnvalue)) false false)))))

(event `self.Charge Hitbox.OnComponentBeginOverlap`
  (params (OverlappedComponent :type "PrimitiveComponent Object Reference") (OtherActor :type "Actor Object Reference") (OtherComp :type "PrimitiveComponent Object Reference") (OtherBodyIndex :type Integer) (bFromSweep :type Boolean) (SweepResult :type "HitResult Structure (by ref)"))
  (if (`GameplayStatics.ObjectIsA` OtherActor (`GameplayStatics.GetObjectClass` (`GameplayStatics.GetPlayerCharacter` 0)))
    (if (<= (`self.ChargeDistance`) 750.0)
      (`self.LaunchCharacter` (`GameplayStatics.GetPlayerCharacter` 0) (0.0 0.0 750.0) false false))))

(fn `UserConstructionScript`
  (`parent.UserConstructionScript`))