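; BP_icecube is an ice cube enemy that continually leaves puddles beneath itself.
; BeginPlay runs the parent logic, resets the shooting timer and attack speed, and sets AIActive to false.
; Tick counts the timer down and spawns a stand-in puddle actor below the capsule at intervals scaled by AttackSpeed, without checking AI state.
; Leftover player-sighting and Shoot-component transform nodes are unused.
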(event `self.ReceiveBeginPlay`
  (`parent.ReceiveBeginPlay`)
  (set `self.ShootingTimer` 0.0)
  (set `self.attackSpeed` 1.0)
  (set `self.AIActive` false))

(event `self.ReceiveTick`
  (params (DeltaSeconds :type "Float (single-precision)"))
  (`parent.ReceiveTick` DeltaSeconds)
  (if (<= (`self.ShootingTimer`) 0.0)
    (set `self.ShootingTimer` (+ (`self.ShootingTimer`) (/ 0.1 (`self.attackSpeed`))))
    (`|SpawnActorFromClass` "/Game/Enemies/Enemy_Projectiles/puddle_standin2.puddle_standin2_C" (`KismetMathLibrary.MakeTransform` (`KismetMathLibrary.MakeVector` (.x (`SceneComponent.K2_GetComponentLocation` (`self.CapsuleComponent`))) (.y (`SceneComponent.K2_GetComponentLocation` (`self.CapsuleComponent`))) (- (.z (`SceneComponent.K2_GetComponentLocation` (`self.CapsuleComponent`))) 100.0))) "Undefined" "MultiplyWithRoot" null null)
    (else
      (set `self.ShootingTimer` (- (`self.ShootingTimer`) DeltaSeconds)))))

(fn `UserConstructionScript`
  (`parent.UserConstructionScript`))