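; BP_onion_volcano is an enemy Blueprint that periodically fires onion projectiles while the player is nearby.
; BeginPlay gives it a random yaw and a random initial shot delay.
; Tick counts the timer down only while the player is within a horizontal radius, ignoring height.
; Each shot spawns an Onion_Projectile at the Shoot component with the actor's scale and rotation, then adds a random delay scaled by AttackSpeed.
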(event `self.ReceiveBeginPlay`
  (`parent.ReceiveBeginPlay`)
  (set `self.ShootingTimer` 0.0)
  (set `self.attackSpeed` 1.0)
  (`self.stop`)
  (set `self.ShootingTimer` (`KismetMathLibrary.RandomFloatInRange` 1.0 4.0))
  (`self.K2_SetActorRotation` (`KismetMathLibrary.MakeRotator` 0.0 0.0 (`KismetMathLibrary.RandomFloatInRange` 0.0 360.0))))

(event `self.ReceiveTick`
  (params (DeltaSeconds :type "Float (single-precision)"))
  (`parent.ReceiveTick` DeltaSeconds)
  (if (<= (`KismetMathLibrary.Distance2D` (`KismetMathLibrary.MakeVector2D` (.x (`self.K2_GetActorLocation` (`GameplayStatics.GetPlayerCharacter` 0))) (.y (`self.K2_GetActorLocation` (`GameplayStatics.GetPlayerCharacter` 0)))) (`KismetMathLibrary.MakeVector2D` (.x (`self.K2_GetActorLocation`)) (.y (`self.K2_GetActorLocation`)))) 5000.0)
    (if (<= (`self.ShootingTimer`) 0.0)
      (set `self.ShootingTimer` (+ (`self.ShootingTimer`) (/ (`KismetMathLibrary.RandomFloatInRange` 1.0 4.0) (`self.attackSpeed`))))
      (`|SpawnActorFromClass` "/Game/Enemies/Amalgamation_Data/Onion_Projectile.Onion_Projectile_C" (`KismetMathLibrary.MakeTransform` (`SceneComponent.K2_GetComponentLocation` (`self.Shoot`)) (`SceneComponent.K2_GetComponentRotation` (`self.Shoot`)) (.scale (`self.GetTransform`))) "Undefined" "MultiplyWithRoot" null 1000.0 (`self.K2_GetActorRotation` self) null)
      (else
        (set `self.ShootingTimer` (- (`self.ShootingTimer`) DeltaSeconds))))))

(fn `UserConstructionScript`
  (`parent.UserConstructionScript`))