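; Amalgamation enemy that chases the player, attacks at close range and splits into BP_Gation and BP_Malg when killed.
; Tick runs a cooldown, then randomly picks a charge that leaves puddles, a dig, or a ring of onion volcanoes.
; Dig spawns a teleport-check actor near the player; timer-driven mesh offsets animate burrowing, and surfacing ends in a rock-chunk burst.
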(event `self.ReceiveBeginPlay`
  (`parent.ReceiveBeginPlay`)
  (set `self.ShootingTimer` 0.0)
  (set `self.attackSpeed` 1.0)
  (set `self.ChargeDistance` 9999.0)
  (set `self.destroyEffect` true))

(event `onKill`
  (`|SpawnActorFromClass` "/Game/Enemies/Amalgamation_Data/BP_Gation.BP_Gation_C" (`self.GetTransform` self) "Undefined" "MultiplyWithRoot" null null)
  (`|SpawnActorFromClass` "/Game/Enemies/Amalgamation_Data/BP_Malg.BP_Malg_C" (`self.GetTransform` self) "Undefined" "MultiplyWithRoot" null null)
  (`self.K2_DestroyActor`))

(event `self.ReceiveTick`
  (params (DeltaSeconds :type "Float (single-precision)"))
  (`parent.ReceiveTick` DeltaSeconds)
  (if (`self.shouldKill`)
    (`self.onKill`)
    (else
      (`self.AnimationTick` DeltaSeconds)
      (`self.tickCharge` DeltaSeconds)
      (if (<= (`self.ShootingTimer`) 0.0)
        (if (<= (`KismetMathLibrary.Vector_Distance` (`self.K2_GetActorLocation` (`GameplayStatics.GetPlayerPawn` 0)) (`self.K2_GetActorLocation` self)) 1000.0)
          (bind _output_get (set `self.Choice` (`KismetMathLibrary.Conv_Int64ToInt` (`KismetMathLibrary.RandomInteger64InRange` 1 3))))
          (if (== _output_get 1)
            (`MovementComponent.StopMovementImmediately` (`self.CharacterMovement`))
            (`KismetSystemLibrary.Delay` 1.0)
            (`self.Charge`)
            (elif (== _output_get 2)
              (`self.Dig`)
              (else
                (`self.SpawnVolcano`))))
          (else
            (set `self.AIActive` true)
            (set `self.seeingPlayer` true)
            (`self.chase`)))
        (else
          (set `self.ShootingTimer` (- (`self.ShootingTimer`) DeltaSeconds)))))))

(event `Charge`
  ; Attack 1 - Charge
  (set `self.ShootingTimer` (+ (`self.ShootingTimer`) (/ 4.0 (`self.attackSpeed`))))
  (`|AIMoveTo` self (0.0 0.0 0.0) (`GameplayStatics.GetPlayerPawn` 0)
    (:`then`
      (`KismetSystemLibrary.Delay` 0.1)
      (`MovementComponent.StopMovementImmediately` (`self.CharacterMovement`))
      (set `self.ChargeDistance` 0.0))))

(event `tickCharge`
  (params (DeltaSeconds :type "Float (double-precision)"))
  (bind _returnvalue (* 1000.0 DeltaSeconds))
  (bind _returnvalue_2 (+ (.yaw (`SceneComponent.K2_GetComponentRotation` (`self.Mesh`))) 90.0))
  ; Attack 1 - Charge
  (`|ExecutionSequence`
    (:`then_1`
      (if (<= (`self.ChargeDistance`) 2000.0)
        (set `self.ChargeDistance` (+ _returnvalue (`self.ChargeDistance`)))
        (`SceneComponent.K2_AddWorldOffset` (`self.CapsuleComponent`) (`KismetMathLibrary.MakeVector` (* (`KismetMathLibrary.DegCos` _returnvalue_2) _returnvalue) (* (`KismetMathLibrary.DegSin` _returnvalue_2) _returnvalue)) false false)
        (if (<= (`self.SpawnCharPuddle`) 0.0)
          (set `self.SpawnCharPuddle` (+ 0.05 (/ 0.2 (`self.attackSpeed`))))
          (`|SpawnActorFromClass` "/Game/Enemies/Amalgamation_Data/char_puddle.char_puddle_C" (`KismetMathLibrary.MakeTransform` (`KismetMathLibrary.MakeVector` (.x (`SceneComponent.K2_GetComponentLocation` (`self.CapsuleComponent`))) (.y (`SceneComponent.K2_GetComponentLocation` (`self.CapsuleComponent`))) (- (.z (`SceneComponent.K2_GetComponentLocation` (`self.CapsuleComponent`))) 100.0))) "Undefined" "MultiplyWithRoot" null null)
          (else
            (set `self.SpawnCharPuddle` (- (`self.SpawnCharPuddle`) DeltaSeconds))))))))

(event `Dig`
  ; Dig
  (`MovementComponent.StopMovementImmediately` (`self.CharacterMovement`))
  (set `self.ShootingTimer` (+ (`self.ShootingTimer`) (/ 3.0 (`self.attackSpeed`))))
  (set `self.randAng` (`KismetMathLibrary.RandomInteger` 360))
  (`|SpawnActorFromClass` "/Game/Enemies/Amalgamation_Data/Tele_Check_amalg.Tele_Check_amalg_C" (`KismetMathLibrary.MakeTransform` (`KismetMathLibrary.MakeVector` (+ (* (`KismetMathLibrary.DegCos` (`KismetMathLibrary.Conv_IntToDouble` (`self.randAng`))) 750.0) (.x (`self.K2_GetActorLocation` (`GameplayStatics.GetPlayerPawn` 0)))) (+ (* (`KismetMathLibrary.DegSin` (`KismetMathLibrary.Conv_IntToDouble` (`self.randAng`))) 750.0) (.y (`self.K2_GetActorLocation` (`GameplayStatics.GetPlayerPawn` 0)))) (+ (.z (`self.K2_GetActorLocation` (`GameplayStatics.GetPlayerPawn` 0))) 100.0)) (struct :`Pitch` -90.0) (.scale (`self.GetTransform`))) "Undefined" "MultiplyWithRoot" null self 1000.0 (`self.K2_GetActorRotation` self) null))

(event `DigDown`
  ; Dig
  (set `self.animTimer` 1.0)
  (set `self.animPlay` "DigDown"))

(event `DigUp`
  ; Dig
  (set `self.animTimer` 0.25)
  (set `self.animPlay` "DigUp"))

(event `AnimationTick`
  (params (DeltaSeconds :type "Float (double-precision)"))
  ; Dig
  (if (> (`self.animTimer`) 0.0)
    (set `self.animTimer` (- (`self.animTimer`) DeltaSeconds))
    (if (== (`self.animPlay`) "DigDown")
      (`self.DigDownTick` DeltaSeconds)
      (elif (== (`self.animPlay`) "DigUp")
        (`self.DigUpTick` DeltaSeconds)))
    (else
      (set `self.animTimer` 0.0)
      (`|ExecutionSequence`
        (:`then_0`
          (if (== (`self.animPlay`) "DigUp")
            (`SceneComponent.K2_SetRelativeLocation` (`self.Mesh`) (0.0 0.0 -90.0) false false)
            (`|AIMoveTo` self (0.0 0.0 0.0) (`GameplayStatics.GetPlayerPawn` 0)
              (:`then`
                (`KismetSystemLibrary.Delay` 0.1)
                (`MovementComponent.StopMovementImmediately` (`self.CharacterMovement`))
                (for _ (range 31)
                  (`|SpawnActorFromClass` "/Game/Enemies/Amalgamation_Data/Amalg_Rock_Chunk.Amalg_Rock_Chunk_C" (`KismetMathLibrary.MakeTransform` (`SceneComponent.K2_GetComponentLocation` (`self.Shoot`)) (`KismetMathLibrary.MakeRotator` 0.0 (`KismetMathLibrary.Conv_Int64ToDouble` (`KismetMathLibrary.RandomInteger64InRange` 45 65)) (`KismetMathLibrary.Conv_Int64ToDouble` (`KismetMathLibrary.RandomInteger64InRange` 0 360))) (.scale (`self.GetTransform`))) "Undefined" "MultiplyWithRoot" null 1000.0 (`self.K2_GetActorRotation` self) null))))))
        (:`then_1`
          (set `self.animPlay` "None"))))))

(event `DigDownTick`
  (params (DeltaSeconds :type "Float (double-precision)"))
  ; Dig
  (`SceneComponent.K2_AddLocalOffset` (`self.Mesh`) (`KismetMathLibrary.MakeVector` 0.0 0.0 (* DeltaSeconds -800.0)) false false))

(event `DigUpTick`
  (params (DeltaSeconds :type "Float (double-precision)"))
  ; Dig
  (`SceneComponent.K2_AddLocalOffset` (`self.Mesh`) (`KismetMathLibrary.MakeVector` 0.0 0.0 (* DeltaSeconds 3200.0)) false false))

(event `SpawnVolcano`
  ; Spawn Volcano
  (set `self.ShootingTimer` (+ (`self.ShootingTimer`) (/ 5.0 (`self.attackSpeed`))))
  (`MovementComponent.StopMovementImmediately` (`self.CharacterMovement`))
  (for _index (range 3)
    (set `self.Index` _index)
    (`|SpawnActorFromClass` "/Game/Enemies/Amalgamation_Data/BP_onion_volcano.BP_onion_volcano_C" (`KismetMathLibrary.MakeTransform` (`KismetMathLibrary.MakeVector` (+ (.x (`self.K2_GetActorLocation` self)) (* 200.0 (`KismetMathLibrary.DegCos` (* (`self.Index`) 120.0)))) (+ (.y (`self.K2_GetActorLocation` self)) (* 200.0 (`KismetMathLibrary.DegSin` (* (`self.Index`) 120.0)))) (.z (`self.K2_GetActorLocation` self)))) "Undefined" "MultiplyWithRoot" null null)))

(fn `UserConstructionScript`
  (`parent.UserConstructionScript`))