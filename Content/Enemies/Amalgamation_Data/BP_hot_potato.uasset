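; Hot potato enemy character that rushes the player and leaps in a suicide slam, with a health weakness set at BeginPlay.
; Tick uses a cooldown timer: within range it boosts walk speed, starts AIMoveTo and launches upward shortly after; otherwise it chases if AI is active.
; Getting close mid-slam launches and damages the player, then destroys the enemy.
; Landing ends the slam and resets speed.
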(event `self.ReceiveBeginPlay`
  (`parent.ReceiveBeginPlay`)
  (set `self.ShootingTimer` 0.0)
  (set `/Game/Blueprints/BPC_Health.Weakness` "NewEnumerator1" (`self.BPC_Health`)))

(event `self.ReceiveTick`
  (params (DeltaSeconds :type "Float (single-precision)"))
  (bind _returnvalue (`GameplayStatics.GetPlayerCharacter` 0))
  (`parent.ReceiveTick` DeltaSeconds)
  (if (and (<= (`KismetMathLibrary.Vector_Distance` (`self.K2_GetActorLocation` (`GameplayStatics.GetPlayerPawn` 0)) (`self.K2_GetActorLocation` self)) 150.0) (`self.Slamming`))
    (`self.LaunchCharacter` _returnvalue (0.0 0.0 250.0) false false)
    (`GameplayStatics.ApplyDamage` _returnvalue 5.0)
    (`self.K2_DestroyActor`)
    (elif (<= (`self.ShootingTimer`) 0.0)
      (if (<= (`KismetMathLibrary.Vector_Distance` (`self.K2_GetActorLocation` (`GameplayStatics.GetPlayerPawn` 0)) (`self.K2_GetActorLocation` self)) 600.0)
        (set `CharacterMovementComponent.MaxWalkSpeed` 2000.0 (`self.CharacterMovement`))
        (set `self.ShootingTimer` (+ (`self.ShootingTimer`) 4.0))
        (`|AIMoveTo` self (0.0 0.0 0.0) (`GameplayStatics.GetPlayerPawn` 0)
          (:`then`
            (`KismetSystemLibrary.Delay` 0.1)
            (`self.LaunchCharacter` (0.0 0.0 500.0))
            (set `self.Slamming` true)))
        (elif (`self.AIActive`)
          (set `self.AIActive` true)
          (set `self.seeingPlayer` true)
          (`self.chase`)))
      (else
        (set `self.ShootingTimer` (- (`self.ShootingTimer`) DeltaSeconds))))))

(event `self.OnLanded`
  (params (Hit :type "HitResult Structure (by ref)"))
  (if (`self.Slamming`)
    (`MovementComponent.StopMovementImmediately` (`self.CharacterMovement`))
    (set `self.Slamming` false)
    (set `CharacterMovementComponent.MaxWalkSpeed` 400.0 (`self.CharacterMovement`))))

(fn `UserConstructionScript`
  (`parent.UserConstructionScript`))