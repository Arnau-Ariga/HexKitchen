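; Amalgamation enemy that chases the player and, once in range and off cooldown, randomly picks a charge or a jump slam.
; Charge slides the capsule along its facing each Tick without sweeping, then drops a puddle and a ring of hot potatoes.
; Jump slam boosts walk speed and launches upward; landing restores speed, resumes the chase, flashes GroundPound and spawns eight radial lines of FaultlineSpawners with staggered delays rippling outward.
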(event `self.ReceiveBeginPlay`
  (`parent.ReceiveBeginPlay`)
  (set `self.ShootingTimer` 0.0)
  (set `self.attackSpeed` 1.0)
  (set `self.ChargeDistance` 9999.0)
  (set `self.DefaultWalkSpeed` (`CharacterMovementComponent.MaxWalkSpeed` (`self.CharacterMovement`))))

(event `self.ReceiveTick`
  (params (DeltaSeconds :type "Float (single-precision)"))
  (`parent.ReceiveTick` DeltaSeconds)
  (`self.tickCharge` DeltaSeconds)
  (if (<= (`self.ShootingTimer`) 0.0)
    (if (<= (`KismetMathLibrary.Vector_Distance` (`self.K2_GetActorLocation` (`GameplayStatics.GetPlayerPawn` 0)) (`self.K2_GetActorLocation` self)) 1000.0)
      (bind _returnvalue (`KismetMathLibrary.RandomBool`))
      (if _returnvalue
        (`self.Charge`)
        (else
          (`self.Jumpy`)))
      (else
        (set `self.AIActive` true)
        (set `self.seeingPlayer` true)
        (`self.chase`)))
    (else
      (set `self.ShootingTimer` (- (`self.ShootingTimer`) DeltaSeconds)))))

(event `Charge`
  ; Attack 1 - Charge
  (set `self.ShootingTimer` (+ (`self.ShootingTimer`) (/ 4.0 (`self.attackSpeed`))))
  (`|AIMoveTo` self (0.0 0.0 0.0) (`GameplayStatics.GetPlayerPawn` 0)
    (:`then`
      (`KismetSystemLibrary.Delay` 0.1)
      (`MovementComponent.StopMovementImmediately` (`self.CharacterMovement`))
      (set `self.ChargeDistance` 0.0)
      (set `self.charging` true))))

(event `tickCharge`
  (params (DeltaSeconds :type "Float (double-precision)"))
  (bind _returnvalue (* 1000.0 DeltaSeconds))
  (bind _returnvalue_2 (+ (.yaw (`SceneComponent.K2_GetComponentRotation` (`self.Mesh`))) 90.0))
  ; Attack 1 - Charge
  (`|ExecutionSequence`
    (:`then_0`
      (if (> (`self.ChargeDistance`) 1000.0)
        (if (`self.charging`)
          (set `self.charging` false)
          (`|SpawnActorFromClass` "/Game/Enemies/Amalgamation_Data/char_puddle.char_puddle_C" (`KismetMathLibrary.MakeTransform` (`KismetMathLibrary.MakeVector` (.x (`SceneComponent.K2_GetComponentLocation` (`self.CapsuleComponent`))) (.y (`SceneComponent.K2_GetComponentLocation` (`self.CapsuleComponent`))) (- (.z (`SceneComponent.K2_GetComponentLocation` (`self.CapsuleComponent`))) 100.0))) "Undefined" "MultiplyWithRoot" null null)
          (for _index (range 3)
            (set `self.Index` _index)
            (`|SpawnActorFromClass` "/Game/Enemies/Amalgamation_Data/BP_hot_potato.BP_hot_potato_C" (`KismetMathLibrary.MakeTransform` (`KismetMathLibrary.MakeVector` (+ (.x (`self.K2_GetActorLocation` self)) (* 200.0 (`KismetMathLibrary.DegCos` (* (`self.Index`) 120.0)))) (+ (.y (`self.K2_GetActorLocation` self)) (* 200.0 (`KismetMathLibrary.DegSin` (* (`self.Index`) 120.0)))) (.z (`self.K2_GetActorLocation` self)))) "Undefined" "MultiplyWithRoot" null null)))))
    (:`then_1`
      (if (<= (`self.ChargeDistance`) 1000.0)
        (set `self.ChargeDistance` (+ _returnvalue (`self.ChargeDistance`)))
        (`SceneComponent.K2_AddWorldOffset` (`self.CapsuleComponent`) (`KismetMathLibrary.MakeVector` (* (`KismetMathLibrary.DegCos` _returnvalue_2) _returnvalue) (* (`KismetMathLibrary.DegSin` _returnvalue_2) _returnvalue)) false false)))))

(event `Jumpy`
  ; Dig
  (if (and (not (`self.Slamming`)) (<= (`self.ShootingTimer`) 0.0))
    (`self.stop`)
    (set `CharacterMovementComponent.MaxWalkSpeed` (* (`self.DefaultWalkSpeed`) 300.0) (`self.CharacterMovement`))
    (set `self.ShootingTimer` (+ (`self.ShootingTimer`) 3.0))
    (`|AIMoveTo` self (0.0 0.0 0.0) (`GameplayStatics.GetPlayerPawn` 0)
      (:`then`
        (`KismetSystemLibrary.Delay` 0.1)
        (`self.LaunchCharacter` (0.0 0.0 1000.0))
        (set `self.Slamming` true)))
    (else
      (`KismetSystemLibrary.PrintString` "Hello"))))

(event `self.OnLanded`
  (params (Hit :type "HitResult Structure (by ref)"))
  ; Dig
  (if (`self.Slamming`)
    (`MovementComponent.StopMovementImmediately` (`self.CharacterMovement`))
    (set `self.Slamming` false)
    (`|ExecutionSequence`
      (:`then_0`
        (set `CharacterMovementComponent.MaxWalkSpeed` (`self.DefaultWalkSpeed`) (`self.CharacterMovement`))
        (set `self.AIActive` true)
        (set `self.seeingPlayer` true)
        (`self.chase`)
        (for _index (range 8)
          (set `self.Index_0` _index)
          (for _index_2 (range 1 11)
            (set `self.Index_1` _index_2)
            (`|SpawnActorFromClass` "/Game/Enemies/Amalgamation_Data/faultlineSpawner.faultlineSpawner_C" (`KismetMathLibrary.MakeTransform` (+ (`self.K2_GetActorLocation` self) (`KismetMathLibrary.MakeVector` (* (* 200 (`self.Index_1`)) (`KismetMathLibrary.DegSin` (`KismetMathLibrary.Conv_IntToDouble` (* (`self.Index_0`) 45)))) (* (* 200 (`self.Index_1`)) (`KismetMathLibrary.DegCos` (`KismetMathLibrary.Conv_IntToDouble` (* (`self.Index_0`) 45)))))) (`KismetMathLibrary.MakeRotator` (`KismetMathLibrary.Conv_IntToDouble` (* (`self.Index_0`) 60)) -90.0)) "Undefined" "MultiplyWithRoot" null (* 0.05 (`self.Index_1`)) 0.0 (struct) null))))
      (:`then_1`
        (`ActorComponent.Activate` (`self.GroundPound`) false)
        (`KismetSystemLibrary.Delay` 1.0)
        (`ActorComponent.Deactivate` (`self.GroundPound`))))))

(fn `UserConstructionScript`
  (`parent.UserConstructionScript`))