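; BP_Gation is an enemy that picks its attack by distance to the player whenever its shooting timer expires.
; Beyond 2000 units it chases; at mid range it stops and fires a fan of fireballs.
; Within 1000 it fires rapid bursts of randomly scattered grilled cheese projectiles, with every fourth triggering a long cooldown and a chase.
; Each attack starts an AI move toward the player, then halts movement before spawning projectiles.
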(event `self.ReceiveBeginPlay`
  (`parent.ReceiveBeginPlay`)
  (set `self.ShootingTimer` 0.0)
  (set `self.attackSpeed` 1.0))

(event `self.ReceiveTick`
  (params (DeltaSeconds :type "Float (single-precision)"))
  (`parent.ReceiveTick` DeltaSeconds)
  (if (<= (`self.ShootingTimer`) 0.0)
    (if (<= (`KismetMathLibrary.Vector_Distance` (`self.K2_GetActorLocation` (`GameplayStatics.GetPlayerPawn` 0)) (`self.K2_GetActorLocation` self)) 2000.0)
      (if (<= (`KismetMathLibrary.Vector_Distance` (`self.K2_GetActorLocation` (`GameplayStatics.GetPlayerPawn` 0)) (`self.K2_GetActorLocation` self)) 1000.0)
        (bind _output_get (set `self.MilkCount` (+ (`self.MilkCount`) 1)))
        (if (> _output_get 3)
          (set `self.MilkCount` 0)
          (set `self.ShootingTimer` (+ (`self.ShootingTimer`) (/ 8.0 (`self.attackSpeed`))))
          (`|ExecutionSequence`
            (:`then_0`
              (`|AIMoveTo` self (0.0 0.0 0.0) (`GameplayStatics.GetPlayerPawn` 0) :!label _label
                (:`then`
                  (`KismetSystemLibrary.Delay` 0.1)
                  (`MovementComponent.StopMovementImmediately` (`self.CharacterMovement`))
                  (for _ (range 3)
                    (`|SpawnActorFromClass` "/Game/Enemies/Amalgamation_Data/Grilled_Cheese_Projectile2.Grilled_Cheese_Projectile2_C" (`KismetMathLibrary.MakeTransform` (`SceneComponent.K2_GetComponentLocation` (`self.Shoot`)) (`KismetMathLibrary.MakeRotator` (.roll (`SceneComponent.K2_GetComponentRotation` (`self.Shoot`))) (+ (.pitch (`SceneComponent.K2_GetComponentRotation` (`self.Shoot`))) (`KismetMathLibrary.RandomIntegerInRange` -30 10)) (+ (.yaw (`SceneComponent.K2_GetComponentRotation` (`self.Shoot`))) (`KismetMathLibrary.RandomIntegerInRange` -20 20))) (.scale (`self.GetTransform`))) "Undefined" "MultiplyWithRoot" null 1000.0 (`self.K2_GetActorRotation` self) null)))))
            (:`then_1`
              (set `self.AIActive` true)
              (set `self.seeingPlayer` true)
              (`self.chase`)))
          (else
            (set `self.ShootingTimer` (+ (`self.ShootingTimer`) (/ 0.2 (`self.attackSpeed`))))
            (goto _label)))
        (else
          (`self.stop`)
          (set `self.ShootingTimer` (+ (`self.ShootingTimer`) (/ 3.0 (`self.attackSpeed`))))
          (`|AIMoveTo` self (0.0 0.0 0.0) (`GameplayStatics.GetPlayerPawn` 0)
            (:`then`
              (`KismetSystemLibrary.Delay` 0.1)
              (`MovementComponent.StopMovementImmediately` (`self.CharacterMovement`))
              (for _index (range 4)
                (`|SpawnActorFromClass` "/Game/Enemies/Amalgamation_Data/Gation_fireball.Gation_fireball_C" (`KismetMathLibrary.MakeTransform` (`SceneComponent.K2_GetComponentLocation` (`self.Shoot`)) (`KismetMathLibrary.MakeRotator` (.roll (`SceneComponent.K2_GetComponentRotation` (`self.Shoot`))) (.pitch (`SceneComponent.K2_GetComponentRotation` (`self.Shoot`))) (+ (.yaw (`SceneComponent.K2_GetComponentRotation` (`self.Shoot`))) (* 20.0 _index) -30.0)) (.scale (`self.GetTransform`))) "Undefined" "MultiplyWithRoot" null 1000.0 (`self.K2_GetActorRotation` self) null))))))
      (else
        (set `self.AIActive` true)
        (set `self.seeingPlayer` true)
        (`self.chase`)))
    (else
      (set `self.ShootingTimer` (- (`self.ShootingTimer`) DeltaSeconds)))))

(fn `UserConstructionScript`
  (`parent.UserConstructionScript`))