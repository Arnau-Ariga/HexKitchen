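; Crafting component that checks recipes against the player character's inventory and crafts their output items.
; TryCraftAll runs CraftItem on every CraftingRecipes data table row, printing a warning when materials are missing.
; CraftItem matches ingredients by name and quantity, updates the matching slots, then spawns Item_Bp actors into the inventory via FillSlot.
; The E key only toggles an InteractPressed flag; nothing in this graph calls TryCraftAll.
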(event `self.ReceiveBeginPlay`)

(event `self.ReceiveTick`
  (params (DeltaSeconds :type "Float (single-precision)")))

(event `Key|E`
  (params (Key :type "Key Structure"))
  (:`Pressed`
    (bind _output_get (set `self.Interact Pressed` (not (stale _output_get))))))

(fn `Add Item`
  (params (`Item Class` :type String) (Amount :type Integer :default 1))
  (for _ (range 1 (+ Amount 1))
    (bind _returnvalue (`|SpawnActorFromClass` "/Game/Items/Blueprints/Item_Bp.Item_Bp_C" (`KismetMathLibrary.MakeTransform` (0.0 0.0 0.0)) "Undefined" "MultiplyWithRoot" null null))
    (`/Game/FirstPerson/Blueprints/InventoryComponent.Fill Slot` (`/Game/FirstPerson/Blueprints/BP_FirstPersonCharacter.InventoryComponent` (cast `/Game/FirstPerson/Blueprints/BP_FirstPersonCharacter` (`GameplayStatics.GetPlayerCharacter` 0) :!pure true)) _returnvalue)))

(fn `CraftItem`
  (params (Recipe :type "/Game/Crafting/Blueprints/ST_CraftingRecipe1 Structure"))
  (bind _outputitem (break `/Game/Crafting/Blueprints/ST_CraftingRecipe1` Recipe))
  (bind _has_all (`self.Has All Ingredients` Recipe))
  (if _has_all
    (`self.Remove Ingredients` Recipe)
    (`self.Add Item` (break `/Game/Crafting/Blueprints/ST_Ingredient1` _outputitem) (`.Amount_5_F663FC734BFF729D47FC6B928F18121C` (break `/Game/Crafting/Blueprints/ST_Ingredient1` _outputitem)))
    (else
      (`KismetSystemLibrary.PrintString` "MISSING MATERIALS"))))

(fn `Has All Ingredients`
  (params (Recipe :type "/Game/Crafting/Blueprints/ST_CraftingRecipe1 Structure"))
  (returns (`Has All` :type Boolean))
  (locals (`Number of Ingredients` :type Integer :default 1) (`Collected # of Ingredients` :type Integer))
  ; I might have fixed the error
  (for _array_element Recipe_Ingredients_14_91B163DB4BB943018611B8B825C40E4C
    (for _array_element_2 (`/Game/FirstPerson/Blueprints/InventoryComponent.Inventory Slots` (`/Game/FirstPerson/Blueprints/BP_FirstPersonCharacter.InventoryComponent` (cast `/Game/FirstPerson/Blueprints/BP_FirstPersonCharacter` (`GameplayStatics.GetPlayerCharacter` 0) :!pure true)))
      (bind (_item _amount) (break `/Game/Crafting/Blueprints/ST_Ingredient1` _array_element))
      (if (and (`KismetStringLibrary.EqualEqual_StrStr` (break `/Game/UserInterface/Inventory_Structure` _array_element_2) _item) (>= (`.Quantity_7_4E0F2A2049AC4851C66FC8BB431F874B` (break `/Game/UserInterface/Inventory_Structure` _array_element_2)) _amount))
        (bind _output_get (set `local.Collected # of Ingredients` (+ (stale _output_get) 1))))))
  (return (== (`KismetArrayLibrary.Array_Length` Recipe_Ingredients_14_91B163DB4BB943018611B8B825C40E4C) (`local.Collected # of Ingredients`))))

(fn `Remove Ingredients`
  (params (Recipe :type "/Game/Crafting/Blueprints/ST_CraftingRecipe1 Structure"))
  (bind _inventory_slots (`/Game/FirstPerson/Blueprints/InventoryComponent.Inventory Slots` (`/Game/FirstPerson/Blueprints/BP_FirstPersonCharacter.InventoryComponent` (cast `/Game/FirstPerson/Blueprints/BP_FirstPersonCharacter` (`GameplayStatics.GetPlayerCharacter` 0) :!pure true))))
  (for _array_element Recipe_Ingredients_14_91B163DB4BB943018611B8B825C40E4C
    (for (_array_element_2 _array_index) _inventory_slots
      (if (`KismetStringLibrary.EqualEqual_StrStr` (break `/Game/UserInterface/Inventory_Structure` _array_element_2) (break `/Game/Crafting/Blueprints/ST_Ingredient1` _array_element))
        (bind _returnvalue (`KismetMathLibrary.Max` (- (`.Amount_5_F663FC734BFF729D47FC6B928F18121C` (break `/Game/Crafting/Blueprints/ST_Ingredient1` _array_element)) (`.Quantity_7_4E0F2A2049AC4851C66FC8BB431F874B` (break `/Game/UserInterface/Inventory_Structure` _array_element_2)))))
        (setmembers `/Game/UserInterface/Inventory_Structure` :`StructRef` (`|GetArrayItem` _inventory_slots _array_index) :`Quantity` _returnvalue :`Empty?` (== _returnvalue 0))))))

(fn `TryCraftAll`
  (bind _craftingrecipes (`self.CraftingRecipes`))
  (bind _outrownames (`DataTableFunctionLibrary.GetDataTableRowNames` _craftingrecipes))
  (for _array_element _outrownames
    (bind _returnvalue (`|GetDataTableRow` _craftingrecipes _array_element)
      (:`then`
        (`self.CraftItem` _returnvalue)))))