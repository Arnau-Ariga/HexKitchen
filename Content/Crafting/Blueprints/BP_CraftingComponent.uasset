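; Crafting component that turns recipe ingredients from the player's inventory into output items.
; CraftItem checks ingredients against the GameInstanceColson inventory, removes them, adds the output, then calls Crafted.
; The check counts individual stacks meeting each amount, requiring the count to equal the ingredient total.
; Removal empties matching slots through the first-person character's InventoryComponent, gated by UI slot quantity text, while output items are spawned as actors to fill slots.
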(fn `Add Item`
  (params (`Item Class` :type "/Game/Items/Blueprints/Item_Bp Class Reference") (Amount :type Integer :default 1))
  (bind _asbp_first_person_character (cast `/Game/FirstPerson/Blueprints/BP_FirstPersonCharacter` (`GameplayStatics.GetPlayerCharacter` 0)))
  (for _ (range 1 (+ Amount 1))
    (bind _returnvalue (`|SpawnActorFromClass` `Item Class` (`KismetMathLibrary.MakeTransform` (0.0 0.0 0.0)) "Undefined" "MultiplyWithRoot" null null))
    (`/Game/FirstPerson/Blueprints/InventoryComponent.fill slot (but better)` (`/Game/FirstPerson/Blueprints/BP_FirstPersonCharacter.InventoryComponent` _asbp_first_person_character) _returnvalue)))

(fn `CraftItem`
  (params (Recipe :type "/Game/Crafting/Blueprints/ST_CraftingRecipe Structure"))
  (bind (_outputitemclass _outputamount) (break `/Game/Crafting/Blueprints/ST_CraftingRecipe` Recipe))
  (bind _has_all (`self.Has All Ingredients` Recipe))
  (if _has_all
    (`self.Remove Ingredients` Recipe)
    (`self.Add Item` _outputitemclass _outputamount)
    (`self.Crafted`)
    (else
      (`KismetSystemLibrary.PrintString` "MISSING MATERIALS"))))

(fn `Has All Ingredients`
  (params (Recipe :type "/Game/Crafting/Blueprints/ST_CraftingRecipe Structure"))
  (returns (`Has All` :type Boolean))
  (locals (`Number of Ingredients` :type Integer :default 1) (`Collected # of Ingredients` :type Integer))
  (bind (_outputitemclass _outputamount _ingredients) (break `/Game/Crafting/Blueprints/ST_CraftingRecipe` Recipe))
  ; ERROR HERE
  (bind _asgame_instance_colson (cast `/Game/colson/GameInstanceColson` (`GameplayStatics.GetGameInstance`)))
  (set `local.Number of Ingredients` (`KismetArrayLibrary.Array_Length` _ingredients))
  (for _array_element _ingredients
    (for _array_element_2 (`/Game/colson/GameInstanceColson.inventory` _asgame_instance_colson)
      (bind (_name _quantity _empty_ _image _class) (break `/Game/UserInterface/Inventory_Structure` _array_element_2))
      (bind (_itemclass _amount) (break `/Game/Crafting/Blueprints/ST_Ingredient` _array_element))
      (if (== _class _itemclass)
        (if (>= _quantity _amount)
          (`/Engine/EditorBlueprintResources/StandardMacros.IncrementInt` (`local.Collected # of Ingredients`))))))
  (if (== (`local.Collected # of Ingredients`) (`local.Number of Ingredients`))
    (return true)
    (else
      (return false))))

(fn `Remove Ingredients`
  (params (Recipe :type "/Game/Crafting/Blueprints/ST_CraftingRecipe Structure"))
  (bind _asgame_instance_colson (cast `/Game/colson/GameInstanceColson` (`GameplayStatics.GetGameInstance`)))
  (bind _asbp_first_person_character (cast `/Game/FirstPerson/Blueprints/BP_FirstPersonCharacter` (`GameplayStatics.GetPlayerCharacter` 0)))
  (for _array_element (`.Ingredients_9_91B163DB4BB943018611B8B825C40E4C` (break `/Game/Crafting/Blueprints/ST_CraftingRecipe` Recipe))
    (for (_array_element_2 _array_index) (`/Game/colson/GameInstanceColson.inventory` _asgame_instance_colson)
      (if (> (`KismetStringLibrary.Conv_StringToInt` (`KismetTextLibrary.Conv_TextToString` (`/Game/UserInterface/Inventory_Button_UI.qauck` (`/Game/colson/Inventory_UI.Get Slot At Index` (`/Game/FirstPerson/Blueprints/InventoryComponent.Inventory UI` (`/Game/FirstPerson/Blueprints/BP_FirstPersonCharacter.InventoryComponent` _asbp_first_person_character)) _array_index)))) 0)
        (bind (_itemclass _amount) (break `/Game/Crafting/Blueprints/ST_Ingredient` _array_element))
        (if (== (`.Class_14_AC7B0F7441F37E615EB1F48087B28887` (break `/Game/UserInterface/Inventory_Structure` _array_element_2)) _itemclass)
          (bind _asbp_first_person_character_2 (cast `/Game/FirstPerson/Blueprints/BP_FirstPersonCharacter` (`GameplayStatics.GetPlayerCharacter` 0)))
          (`KismetSystemLibrary.PrintString` "Hello")
          (for _ (range (+ _amount 1))
            (`/Game/FirstPerson/Blueprints/InventoryComponent.unfill slot but better` (`/Game/FirstPerson/Blueprints/BP_FirstPersonCharacter.InventoryComponent` _asbp_first_person_character_2) _array_index)))
        (else
          (`KismetSystemLibrary.PrintString` "BAD" false))))))