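; Interactable crafting table that shows a "Craft" prompt and toggles the crafting UI for the player.
; The first interaction creates and caches W_CraftingUI; later ones toggle its visibility, switching player movement, input mode and mouse cursor to match.
; Each interaction also refreshes the color of every recipe entry in the UI's scroll box.
; A trigger overlap tracks InInteractRange, which is also cleared while the UI is open.
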(event `self.ReceiveTick`
  (params (DeltaSeconds :type "Float (single-precision)")))

(event `self.Trigger.OnComponentBeginOverlap`
  (params (OverlappedComponent :type "PrimitiveComponent Object Reference") (OtherActor :type "Actor Object Reference") (OtherComp :type "PrimitiveComponent Object Reference") (OtherBodyIndex :type Integer) (bFromSweep :type Boolean) (SweepResult :type "HitResult Structure (by ref)"))
  (set `self.In Interact Range` true))

(event `self.Trigger.OnComponentEndOverlap`
  (params (OverlappedComponent :type "PrimitiveComponent Object Reference") (OtherActor :type "Actor Object Reference") (OtherComp :type "PrimitiveComponent Object Reference") (OtherBodyIndex :type Integer))
  (set `self.In Interact Range` false))

(event `/Game/Blueprints/Interact/BPI_Interactable.Interact`
  (bind _returnvalue (`PlayerState.GetPlayerController` (`GameplayStatics.GetPlayerState` 0)))
  (`/Engine/EditorBlueprintResources/StandardMacros.IsValid` (`self.CraftingUIRef`)
    (:`Is Valid`
      (if (`Widget.IsVisible` (`self.CraftingUIRef`))
        (`Widget.SetVisibility` (`self.CraftingUIRef`) "Collapsed")
        (`CharacterMovementComponent.SetMovementMode` (`Character.CharacterMovement` (`GameplayStatics.GetPlayerCharacter` 0)) "MOVE_Walking" 0)
        (`WidgetBlueprintLibrary.SetInputMode_GameOnly` _returnvalue)
        (set `PlayerController.bShowMouseCursor` false _returnvalue)
        (set `self.In Interact Range` true)
        (else
          (`Widget.SetVisibility` (`self.CraftingUIRef`) "Visible")
          (`CharacterMovementComponent.SetMovementMode` (`Character.CharacterMovement` (`GameplayStatics.GetPlayerCharacter` 0)) "MOVE_None" 0)
          (`WidgetBlueprintLibrary.SetInputMode_GameAndUIEx` _returnvalue (`self.CraftingUIRef`))
          (set `PlayerController.bShowMouseCursor` true _returnvalue)
          (set `self.In Interact Range` false))))
    (:`Is Not Valid`
      (bind _returnvalue_2 (`|CreateWidget` "/Game/Crafting/UI/W_CraftingUI.W_CraftingUI_C" (`PlayerState.GetPlayerController` (`GameplayStatics.GetPlayerState` 0))))
      (bind _output_get (set `self.CraftingUIRef` _returnvalue_2))
      (`UserWidget.AddToViewport` _output_get 0)
      (`Widget.SetVisibility` _output_get "Visible")
      (`CharacterMovementComponent.SetMovementMode` (`Character.CharacterMovement` (`GameplayStatics.GetPlayerCharacter` 0)) "MOVE_None" 0)
      (`WidgetBlueprintLibrary.SetInputMode_GameAndUIEx` (`PlayerState.GetPlayerController` (`GameplayStatics.GetPlayerState` 0)) (`self.CraftingUIRef`))
      (set `PlayerController.bShowMouseCursor` true (`PlayerState.GetPlayerController` (`GameplayStatics.GetPlayerState` 0)))
      (set `self.In Interact Range` false)))
  (cast `/Game/FirstPerson/Blueprints/BP_FirstPersonCharacter` (`GameplayStatics.GetPlayerCharacter` 0))
  (for _array_element (`PanelWidget.GetAllChildren` (`/Game/Crafting/UI/W_CraftingUI.ScrollBox_Recipes` (`self.CraftingUIRef`)))
    (bind _asw_recipe_entry (cast `/Game/Crafting/UI/W_RecipeEntry` _array_element))
    (`/Game/Crafting/UI/W_RecipeEntry.Set Entry Color` _asw_recipe_entry)))

(fn `GetPrompt`
  (returns (Prompt :type String))
  (return "Craft"))

(fn `IsInteractable`
  (returns (IsInteractable :type Boolean))
  (return true))

(fn `UserConstructionScript`)