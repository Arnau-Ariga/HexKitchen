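; Interactable weapon pickup that appears as a knife, fork or spoon, based on the damage type in its Weapon class defaults.
; BeginPlay sets the mesh and the name used in the pickup prompt.
; Interact spawns the matching item actor, passes it to the player's inventory component and destroys the pickup; older direct-equip logic is left disconnected.
; Interaction is only allowed while the player is not holding a sauce.
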(event `self.ReceiveBeginPlay`
  (bind _staticmesh (`self.StaticMesh`))
  (switch `/Game/Items/Weapons/Enum_DamageType` (`.Damage Type` (defaults `Object` (`self.Weapon`)))
    (:`NewEnumerator0`
      (`StaticMeshComponent.SetStaticMesh` (`self.StaticMesh`) "/Game/Items/Meshes/SM_Knife.SM_Knife")
      (set `self.Weapon Name` "Knife"))
    (:`NewEnumerator1`
      (`StaticMeshComponent.SetStaticMesh` _staticmesh "/Game/Items/Meshes/SM_Fork.SM_Fork")
      (set `self.Weapon Name` "Fork"))
    (:`NewEnumerator2`
      (`StaticMeshComponent.SetStaticMesh` _staticmesh "/Game/Items/Meshes/SM_Spoon.SM_Spoon")
      (set `self.Weapon Name` "Spoon"))))

(event `self.ReceiveActorBeginOverlap`
  (params (OtherActor :type "Actor Object Reference")))

(event `/Game/Blueprints/Interact/BPI_Interactable.Interact`
  (bind _asbp_first_person_character (cast `/Game/FirstPerson/Blueprints/BP_FirstPersonCharacter` (`GameplayStatics.GetPlayerCharacter` 0)))
  (bind _returnvalue (`|SpawnActorFromClass` (select `/Game/Items/Weapons/Enum_DamageType` (defaults `Object` (`self.Weapon`)) :`NewEnumerator3` "/Game/Items/Blueprints/Item_Bp.Item_Bp_C" :`NewEnumerator0` "/Game/Items/BP_KnifeBase.BP_KnifeBase_C" :`NewEnumerator1` "/Game/Items/BP_ForkBase.BP_ForkBase_C" :`NewEnumerator2` "/Game/Items/BP_SpoonBase.BP_SpoonBase_C" :!type "Actor Class Reference") (`KismetMathLibrary.MakeTransform` (0.0 0.0 0.0)) "Undefined" "MultiplyWithRoot" null null))
  (bind _asitem_bp (cast `/Game/Items/Blueprints/Item_Bp` _returnvalue))
  (`/Game/FirstPerson/Blueprints/InventoryComponent.fill slot (but better)` (`/Game/FirstPerson/Blueprints/BP_FirstPersonCharacter.InventoryComponent` _asbp_first_person_character) _asitem_bp)
  (`self.K2_DestroyActor`))

(fn `GetPrompt`
  (returns (Prompt :type String))
  (return (`KismetStringLibrary.Concat_StrStr` "Pick Up " (`self.Weapon Name`))))

(fn `IsInteractable`
  (returns (IsInteractable :type Boolean))
  (bind _asbp_first_person_character (cast `/Game/FirstPerson/Blueprints/BP_FirstPersonCharacter` (`GameplayStatics.GetPlayerCharacter` 0)))
  (return (not (`KismetSystemLibrary.IsValid` (`/Game/Bright-Condiments/BPComponents/BPC_PlayerCondiments.Holding Sauce` (`/Game/FirstPerson/Blueprints/BP_FirstPersonCharacter.BPC_PlayerCondiments` _asbp_first_person_character))))))

(fn `UserConstructionScript`)