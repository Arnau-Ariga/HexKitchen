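; BP_WeaponPickupable is an interactable world pickup that gives the player a weapon.
; On BeginPlay it reads the Weapon class defaults' DamageType to choose a knife, fork or spoon mesh and display name for slash, stab or blunt.
; Interacting copies that damage type to the first-person character, equips the weapon class and destroys the pickup.
; GetPrompt builds the "Pick Up" text from the weapon name.
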(event `self.ReceiveBeginPlay`
  (bind _staticmesh (`self.StaticMesh`))
  (switch `/Game/Items/Weapons/Enum_DamageType` (defaults `Object` (`self.Weapon`))
    (:`NewEnumerator0`
      (`StaticMeshComponent.SetStaticMesh` (`self.StaticMesh`) "/Game/Items/Meshes/SM_Knife.SM_Knife")
      (set `self.Weapon Name` "Knife"))
    (:`NewEnumerator1`
      (`StaticMeshComponent.SetStaticMesh` _staticmesh "/Game/Items/Meshes/SM_Fork.SM_Fork")
      (set `self.Weapon Name` "Fork"))
    (:`NewEnumerator2`
      (`StaticMeshComponent.SetStaticMesh` _staticmesh "/Game/Items/Meshes/SM_Spoon.SM_Spoon")
      (set `self.Weapon Name` "Spoon"))))

(event `self.ReceiveActorBeginOverlap`
  (params (OtherActor :type "Actor Object Reference")))

(event `/Game/Blueprints/Interact/BPI_Interactable.Interact`
  (bind _weapon (`self.Weapon`))
  (bind _asbp_first_person_character_ (cast `/Game/FirstPerson/Blueprints/BP_FirstPersonCharacter` (`GameplayStatics.GetPlayerCharacter` 0)))
  (set `/Game/FirstPerson/Blueprints/BP_FirstPersonCharacter.Damage Type` (defaults `Object` _weapon) _asbp_first_person_character_)
  (`/Game/FirstPerson/Blueprints/BP_FirstPersonCharacter.Equip Weapon` _asbp_first_person_character_ _weapon)
  (`self.K2_DestroyActor`))

(fn `GetPrompt`
  (returns (Prompt :type String))
  (return (`KismetStringLibrary.Concat_StrStr` "Pick Up " (`self.Weapon Name`))))

(fn `IsInteractable`
  (returns (IsInteractable :type Boolean))
  (return true))

(fn `UserConstructionScript`)