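; BP_Spork is a spork weapon item that the first-person player can pick up.
; On BeginPlay it registers itself in the item list of the player character's ItemInHand.
; While picked up, it polls ItemInHand every Tick and snaps the Item component between two fixed relative offsets, one for moving and one for standing still.
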(event `self.ReceiveBeginPlay`
  (`parent.ReceiveBeginPlay`)
  (bind _asbp_first_person_character (cast `/Game/FirstPerson/Blueprints/BP_FirstPersonCharacter` (`GameplayStatics.GetPlayerCharacter` 0)))
  (`/Game/FirstPerson/Blueprints/ItemInHandComponent.Add Item to Item List` (`/Game/FirstPerson/Blueprints/BP_FirstPersonCharacter.Item in Hand` _asbp_first_person_character) self))

(event `self.ReceiveTick`
  (params (DeltaSeconds :type "Float (single-precision)"))
  (`parent.ReceiveTick` DeltaSeconds)
  (bind _asbp_first_person_character (cast `/Game/FirstPerson/Blueprints/BP_FirstPersonCharacter` (`GameplayStatics.GetPlayerCharacter` 0)))
  (if (`self.Is Picked Up`)
    (bind _is_moving (`/Game/FirstPerson/Blueprints/ItemInHandComponent.IsPlayerMoving` (`/Game/FirstPerson/Blueprints/BP_FirstPersonCharacter.Item in Hand` _asbp_first_person_character)))
    (if _is_moving
      (`SceneComponent.K2_SetRelativeLocation` (`self.Item`) (0.0 0.0 -10.0) false false)
      (else
        (`SceneComponent.K2_SetRelativeLocation` (`self.Item`) (0.0 -7.0 6.0) false false)))))

(fn `UserConstructionScript`
  (`parent.UserConstructionScript`))