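; BP_Food is a health pickup that heals the first-person character when overlapped.
; It adds HealAmount to the character's BPCHealth component and destroys itself, but only if Health is at least 10 below MaxHealth.
; The heal is not clamped to MaxHealth.
; An eased Timeline for raising the item above its starting height exists but is disconnected, so it never runs.
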(event `self.ReceiveBeginPlay`
  (bind (_returnvalue_x _returnvalue_y _returnvalue_z) (`KismetMathLibrary.BreakVector` (`self.K2_GetActorLocation`)))
  (set `self.Initial Z` _returnvalue_z)
  (set `self.Direction` 1.0))

(event `self.ReceiveActorBeginOverlap`
  (params (OtherActor :type "Actor Object Reference"))
  (bind _asbp_first_person_character (cast `/Game/FirstPerson/Blueprints/BP_FirstPersonCharacter` OtherActor))
  (bind _bpc_health (`/Game/FirstPerson/Blueprints/BP_FirstPersonCharacter.BPC_Health` _asbp_first_person_character))
  (if (<= (`/Game/Blueprints/BPC_Health.Health` _bpc_health) (- (`/Game/Blueprints/BPC_Health.MaxHealth` _bpc_health) 10.0))
    (set `/Game/Blueprints/BPC_Health.Health` (+ (`/Game/Blueprints/BPC_Health.Health` _bpc_health) (`self.HealAmount`)) _bpc_health)
    (`self.K2_DestroyActor`)))

(event `self.ReceiveTick`
  (params (DeltaSeconds :type "Float (single-precision)")))

(fn `UserConstructionScript`)