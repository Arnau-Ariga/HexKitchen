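; BPC_Health is an actor component that tracks health for BP_FirstPersonCharacter and handles player death.
; It creates the health bar widget, binds to the owner's damage event, clamps health, plays a sound and copies the value into GameInstanceColson.
; At zero health, or when Tick finds the player fallen off the map, a one-shot Die shows the death menu, disables input and resets the saved health.
; A debug G key applies test damage.
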(event Custom|Die
  (bind _returnvalue (Game|GetPlayerController 0))
  ;[0.15 0.15 0.15 0.5] If the player dies call this function
  (if (not (Variables|Default|GetIsDead))
    (Variables|Default|SetIsDead true)
    (bind _returnvalue_2 (UserInterface|CreateWidget "/Game/UserInterface/W_DeathMenu.W_DeathMenu_C"))
    (UserInterface|Viewport|AddtoViewport _returnvalue_2 0)
    (Variables|/Script/Engine.PlayerController|SetbShowMouseCursor _returnvalue true)
    (Input|DisableInput (Game|GetPlayerCharacter 0) _returnvalue)
    (Audio|PlaySound2D 0 1.0 1.0 0.0 0 0)
    (bind _asgame_instance_colson (Utilities|Casting|CastToGameInstanceColson (Game|GetGameInstance)))
    (Variables|/Game/UserInterface/GameInstanceColson.GameInstanceColson_C|Sethealth _asgame_instance_colson 1e+02)))

(event Custom|TakeDamage
  (params (DamagedActor :type Actor%20Object%20Reference) (Damage :type Float%20%28single-precision%29) (DamageType :type Damage%20Type%20Object%20Reference) (InstigatedBy :type Controller%20Object%20Reference) (DamageCauser :type Actor%20Object%20Reference))
  ;[0.15 0.15 0.15 0.5] If player is damaged update health
  (bind _output_get (Variables|Default|SetHealth (Math|Float|Clamp(Float) (- (Variables|Default|GetHealth) Damage) 0.0 1e+02)))
  (Development|PrintString (Utilities|String|ToString(Float) _output_get))
  (Audio|PlaySound2D 0 1.0 1.0 0.0 0 0)
  (bind _asgame_instance_colson (Utilities|Casting|CastToGameInstanceColson (Game|GetGameInstance)))
  (Variables|/Game/UserInterface/GameInstanceColson.GameInstanceColson_C|Sethealth _asgame_instance_colson (Variables|Default|GetHealth))
  (if (<= (Variables|Default|GetHealth) 0.0)
    (CallFunction|Die)))

(event EventTick
  (params (DeltaSeconds :type Float%20%28single-precision%29))
  ;[0.15 0.15 0.15 0.5] Checks if player fell off map
  (if (> -1e+02 (.Z (Math|Vector|BreakVector (Transformation|GetActorLocation (Game|GetPlayerCharacter 0)))))
    (CallFunction|Die)))

(event EventBeginPlay
  ;[0.15 0.15 0.15 0.5] If player is damaged update health
  (bind _returnvalue (UserInterface|CreateWidget "/Game/UserInterface/Indicators/W_HealthBar.W_HealthBar_C"))
  (UserInterface|Viewport|AddtoViewport _returnvalue 0)
  (bind _asbp_first_person_character (Utilities|Casting|CastToBP_FirstPersonCharacter (Components|GetOwner)))
  (EventDispatchers|BindEventtoOnTakeAnyDamage _asbp_first_person_character (delegate Custom|TakeDamage)))

(event Input|KeyboardEvents|DebugKeyG
  (params (Key :type Key%20Structure :default "None") (ActionValue :type Input%20Action%20Value%20Structure))
  ;[0.15 0.15 0.15 0.5] Test Damage
  (:Pressed
    (Game|Damage|ApplyDamage (Components|GetOwner) 1e+01 0 0)))